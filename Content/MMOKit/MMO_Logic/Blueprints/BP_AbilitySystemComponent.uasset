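; Actor component for MMOKit characters and mobs that holds their abilities and runs networked activation, with add/remove blocked on clients.
; Client activation checks and fires locally, then the server revalidates, fires, and confirms or denies to the owner and replicates to other clients.
; Each stage delegates to the ability's AbilityLogic object.
; Global and per-ability cooldowns use timestamps with 10% lag leeway and notify the player controller; per-ability end notification is unfinished.
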(event Custom|GlobalCooldownEnd
  ;[0.7865 0.1065 0.7201] Global Cooldown End
  (bind _asbp_player_controller (Utilities|Casting|CastToBP_PlayerController (Pawn|GetController (Variables|Default|GetOwnerCharacter))))
  (Default|CallOnGlobalCooldownEnd _asbp_player_controller))

(event Custom|ActivateAbility_Server
  (params (Ability :type Ability%20Asset%20Object%20Reference) (OptionalVictim :type Character%20Object%20Reference) (OptionalInstigationTransform :type Transform) (OptionalTargetTransform :type Transform))
  ;[0.4452 0.6332 1] Ability execution on server
  (if (CallFunction|CanExecuteAbilityServer Ability)
    (bind (_victimout _stopexecute) (Class|AbilityLogic|FireServer (Variables|/Script/MMOKitCode.AbilityAssetCpp|GetAbilityLogic Ability) (Pawn|GetController (Variables|Default|GetOwnerCharacter)) (Variables|Default|GetOwnerCharacter) OptionalVictim Ability OptionalInstigationTransform OptionalTargetTransform))
    (if _stopexecute
      (Class|MmoUtilities|LogString "Fire Ability on Server cancelled the execution" "Verbosity_SuperVerbose")
      (CallFunction|ActivateAbilityDenyOwningClient Ability _victimout OptionalInstigationTransform OptionalTargetTransform :!label _label)
      (else
        (CallFunction|ActivateGlobalandLocalCooldown Ability)
        (CallFunction|ActivateAbilityConfirmOwningClient Ability _victimout OptionalInstigationTransform OptionalTargetTransform)
        (CallFunction|ActivateAbilityClientsExceptOwner Ability (Variables|Default|GetOwnerCharacter) _victimout OptionalInstigationTransform OptionalTargetTransform)))
    (else
      (Class|MmoUtilities|LogString "CanExecuteAbilityServer: returned false" "Verbosity_DoNotDisplay")
      (goto _label))))

(event Custom|ActivateAbility_ConfirmOwningClient
  (params (Ability :type Ability%20Asset%20Object%20Reference) (VictimChar :type Character%20Object%20Reference) (InstigationTransform :type Transform) (TargetTransform :type Transform))
  ;[1 0.312 0.302] Confirm to Owner Client
  (Networking|CanExecuteCosmeticEvents
    (:True
      (Class|AbilityLogic|FireOwneronConfirm (Variables|/Script/MMOKitCode.AbilityAssetCpp|GetAbilityLogic Ability) (Game|GetPlayerController 0) (Game|GetPlayerCharacter 0) VictimChar Ability InstigationTransform TargetTransform))))

(event Custom|ActivateAbility_ClientsExceptOwner
  (params (Ability :type Ability%20Asset%20Object%20Reference) (Instigator :type Character%20Object%20Reference) (Victim :type Character%20Object%20Reference) (InstigationTransform :type Transform) (TargetTransform :type Transform))
  ;[1 0.312 0.302] Replicate to Clients except Owner
  (Networking|CanExecuteCosmeticEvents
    (:True
      (if (!= (Game|GetPlayerCharacter 0) (Variables|Default|GetOwnerCharacter)) ; NOT OUR CHARACTER
        (Class|AbilityLogic|FireClientsExceptOwner (Variables|/Script/MMOKitCode.AbilityAssetCpp|GetAbilityLogic Ability) Instigator Victim Ability InstigationTransform TargetTransform)))))

(event Custom|ActivateAbility_DenyOwningClient
  (params (Ability :type Ability%20Asset%20Object%20Reference) (VictimChar :type Character%20Object%20Reference) (InstigationTransform :type Transform) (TargetTransform :type Transform))
  ;[1 0.312 0.302] Deny to Owner Client
  (Networking|CanExecuteCosmeticEvents
    (:True
      (Class|AbilityLogic|FireOwneronDeny (Variables|/Script/MMOKitCode.AbilityAssetCpp|GetAbilityLogic Ability) (Game|GetPlayerController 0) (Game|GetPlayerCharacter 0) VictimChar Ability InstigationTransform TargetTransform))))

(event Custom|ActivateAbilityFromClient
  (params (Ability :type Ability%20Asset%20Object%20Reference))
  ;[1 0.312 0.302] Activate Ability From Client - this is the starting point of an ability logic if it's activated from client
  (Utilities|IsValid Ability
    (:Is%20Valid
      (Networking|CanExecuteCosmeticEvents
        (:True
          (if (CallFunction|CanExecuteAbilityClient Ability)
            (bind (_optionalvictim _optionalinstigationtransform _optionaltargettransform _stopexecute) (Class|AbilityLogic|FireLocally (Variables|/Script/MMOKitCode.AbilityAssetCpp|GetAbilityLogic Ability) (Pawn|GetController (Variables|Default|GetOwnerCharacter)) (Variables|Default|GetOwnerCharacter) Ability))
            (if (not _stopexecute)
              (CallFunction|ActivateGlobalandLocalCooldown Ability)
              (CallFunction|ActivateAbilityServer Ability _optionalvictim _optionalinstigationtransform _optionaltargettransform))
            (else
              (Class|MmoUtilities|LogString "CanExecuteAbilityClient: returned false" "Verbosity_DoNotDisplay"))))
        (:False
          (Class|MmoUtilities|LogString "Error in your blueprint code. Can't call \"ActivateAbilityFromClient\" function from server!" "Verbosity_Normal" true true "(R=1.000000,G=0.000000,B=0.024480,A=1.000000)" 5.0))))))

(event Custom|AddAbility
  (params (Ability :type Ability%20Asset%20Object%20Reference))
  ;[0.4452 0.6332 1] Add/Remove ability
  (Utilities|IsValid Ability
    (:Is%20Valid
      (Networking|CanExecuteCosmeticEvents
        (:True
          (Class|MmoUtilities|LogString "Error: can't add/remove abilities on Client!" "Verbosity_SuperVerbose"))
        (:False
          (Utilities|Array|AddUnique (Variables|Default|GetAbilities) Ability))))))

(event Custom|RemoveAbility
  (params (Ability :type Ability%20Asset%20Object%20Reference))
  ;[0.4452 0.6332 1] Add/Remove ability
  (Utilities|IsValid Ability
    (:Is%20Valid
      (Networking|CanExecuteCosmeticEvents
        (:True
          (Class|MmoUtilities|LogString "Error: can't add/remove abilities on Client!" "Verbosity_SuperVerbose"))
        (:False
          (Utilities|Array|RemoveItem (Variables|Default|GetAbilities) Ability))))))

(event Custom|ActivateAbilityFromServer
  (params (Ability :type Ability%20Asset%20Object%20Reference) (OptionalVictim :type Character%20Object%20Reference) (OptionalInstigatorTransform :type Transform))
  ;[0.4452 0.6332 1] Activate Ability from Server - starting point if activated from server
  (Utilities|IsValid Ability
    (:Is%20Valid
      (Networking|CanExecuteCosmeticEvents
        (:True
          (Class|MmoUtilities|LogString "Error in your blueprint code. Can't call \"ActivateAbilityFromServer\" function from client!" "Verbosity_Normal" true true "(R=1.000000,G=0.000000,B=0.024480,A=1.000000)" 5.0))
        (:False
          (CallFunction|ActivateAbilityServer :Ability Ability :OptionalVictim OptionalVictim :OptionalTargetTransform OptionalInstigatorTransform))))))

(event EventBeginPlay
  ;[0.7865 0.1065 0.7201] BeginPlay
  (bind _ascharacter (Utilities|Casting|CastToCharacter (Components|GetOwner)))
  (Variables|Default|SetOwnerCharacter _ascharacter))

(fn CanExecuteAbilityServer
  (params (Ability :type Ability%20Asset%20Object%20Reference))
  ;[0.4452 0.6332 1] mobs tend to spam their default ability, so checking its cooldown will save us
  ; checking anything else for them most of the time
  (if (not (CallFunction|IsAbilityonCooldown Ability))
    (if (CallFunction|DidGlobalCooldownEnd)
      (bind _statscomp (Class|BPIStats|GetStatsComponent(Message) (Variables|Default|GetOwnerCharacter)))
      (return (and (Utilities|Array|ContainsItem (Variables|Default|GetAbilities) Ability) (or (Variables|/Game/MMOKit/MMO_Logic/Blueprints/DataAssetTypes/AbilityAsset.AbilityAsset_C|GetUsableByDead Ability) (Default|IsAlive _statscomp))))
      (else
        (return false)))
    (else
      (return false))))

(fn CanExecuteAbilityClient
  (params (Ability :type Ability%20Asset%20Object%20Reference))
  (bind _statscomp (Class|BPIStats|GetStatsComponent(Message) (Variables|Default|GetOwnerCharacter)))
  (return (Math|Boolean|ANDBoolean (CallFunction|DidGlobalCooldownEnd) (Utilities|Array|ContainsItem (Variables|Default|GetAbilities) Ability) (not (CallFunction|IsAbilityonCooldown Ability)) (or (Variables|/Game/MMOKit/MMO_Logic/Blueprints/DataAssetTypes/AbilityAsset.AbilityAsset_C|GetUsableByDead Ability) (Default|IsAlive _statscomp)))))

(fn DidGlobalCooldownEnd
  (return (>= (Math|Timespan|GetTotalSeconds (- (Math|DateTime|Now) (Variables|Default|GetLastTimeUsedAbility))) (* (Variables|Default|GetGlobalCoolDown) 0.9))))

(fn ActivateGlobalandLocalCooldown
  (params (Ability :type Ability%20Asset%20Object%20Reference))
  (Utilities|FlowControl|Sequence
    (:then_0
      ;[0.7865 0.1065 0.7201] Activate global cooldown
      (Variables|Default|SetLastTimeUsedAbility (Math|DateTime|Now))
      (Utilities|Time|SetTimerbyEvent (EventDispatchers|CreateEvent :!event Custom|GlobalCooldownEnd) (Variables|Default|GetGlobalCoolDown))
      (bind _asbp_player_controller (Utilities|Casting|CastToBP_PlayerController (Pawn|GetController (Variables|Default|GetOwnerCharacter))))
      (Default|CallOnGlobalCooldownStart _asbp_player_controller))
    (:then_1
      (Utilities|Map|Add (Variables|Default|GetCachedCooldowns) Ability (Math|DateTime|Now))
      (bind _asbp_player_controller_2 (Utilities|Casting|CastToBP_PlayerController (Pawn|GetController (Variables|Default|GetOwnerCharacter))))
      (Default|CallOnAbilityCooldownStart _asbp_player_controller_2 Ability))))

(fn IsAbilityonCooldown
  (params (Ability :type Ability%20Asset%20Object%20Reference))
  (bind _cachedcooldowns (Variables|Default|GetCachedCooldowns))
  (bind (_value _returnvalue) (Utilities|Map|Find _cachedcooldowns Ability))
  (if _returnvalue
    (return (not (>= (Math|Timespan|GetTotalSeconds (- (Math|DateTime|Now) _value)) (* (Variables|/Script/MMOKitCode.AbilityAssetCpp|GetCooldown Ability) 0.9))))
    (else
      (return false))))
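; Point-and-click camera component with boom zoom, RMB look with a faked cursor lock, and Path of Exile-style click-to-move.
; LMB raycasts pick non-friendly characters, interactables or ground, then build a navmesh path.
; Tick re-paths to targets, turning and running the character along points.
; On arrival it fires ReachedTarget for attack or interaction, clearing character targets unless LMB is held; it also supplies the attack origin.
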(event Custom|SetPathDestination
  (params (Destination :type Vector))
  (bind _ownercharacter (Variables|Default|GetOwnerCharacter))
  ;[1 0.312 0.302] LMB: Set Path Destination to Attackable Character / Interactable / Ground Point
  (bind _returnvalue (Class|NavigationSystemV1|FindPathtoLocationSynchronously (Transformation|GetActorLocation _ownercharacter) Destination _ownercharacter 0))
  (if (Utilities|Array|IsValidIndex (Variables|/Script/NavigationSystem.NavigationPath|GetPathPoints _returnvalue))
    (Utilities|Array|RemoveIndex (Variables|/Script/NavigationSystem.NavigationPath|GetPathPoints _returnvalue)) ; remove PathStart point
  )
  (Variables|Default|SetPathPoints (Variables|/Script/NavigationSystem.NavigationPath|GetPathPoints _returnvalue))
  (CallFunction|DebugDrawPath))

(event Custom|ZoomUpdate
  ;[1 1 1] (Called on Tick) Zoom In/Out
  (if (< (Variables|Zoom|GetZoomAlpha) 1.0)
    (Variables|/Script/Engine.SpringArmComponent|SetTargetArmLength (Variables|/Game/MMOKit/MMO_Logic/Blueprints/BP_PlayerCharacter.BP_PlayerCharacter_C|GetCameraBoom (Variables|Default|GetOwnerCharacter)) (Math|Interpolation|Ease "EaseInOut" (Variables|Zoom|GetZoomAlpha) (Variables|Zoom|GetZoomFrom) (Variables|Zoom|GetZoomTo) 2.0))
    (Variables|Zoom|SetZoomAlpha (+ (Variables|Zoom|GetZoomAlpha) (Math|Float|SafeDivide (Utilities|Time|GetWorldDeltaSeconds) 0.3))) ; Increase alpha on each tick by\nDeltaTime*(1/ZoomTime)\n1/ZoomTime is ZoomSpeed
  ))

(event Custom|OnDeathResetPath
  ;[1 0.312 0.302] OnDeath - Reset path and stop running
  (Variables|Default|SetTrackTarget 0)
  (Variables|Default|SetLmbDown false)
  (Utilities|Array|Clear (Variables|Default|GetPathPoints)))

(event Custom|AutoRun
  (bind _pathpoints (Variables|Default|GetPathPoints))
  (bind _returnvalue (Utilities|Array|Length _pathpoints))
  (bind _returnvalue_2 (> _returnvalue 0))
  ;[1 0.312 0.302] (Called on Tick) AutoRun towards destination
  (Utilities|FlowControl|Sequence
    (:then_0
      (if (Variables|Default|GetLmbDown)
        (bind _ascharacter (Utilities|Casting|CastToCharacter (Variables|Default|GetTrackTarget))
          (:then
            (bind _alive (Class|BPICharacter|IsAlive(Message) _ascharacter))
            (if _alive
              (CallFunction|GetAnythingUnderCursor false :!label _label) ; If LMB is pressed down, keep getting new targets or path
              (else
                (CallFunction|GetAnythingUnderCursor true) ; If LMB is pressed down, keep getting new targets or path
              )))
          (:CastFailed
            (goto _label)))
        (else
          (Utilities|IsValid (Variables|Default|GetTrackTarget)
            (:Is%20Valid
              (CallFunction|SetPathtoTarget) ; If LMB is not pressed down, but we have a target\nUpdate path to target every frame
            )))))
    (:then_1
      (if _returnvalue_2
        (CallFunction|UpdateNextPoint)
        (if _returnvalue_2 ; it's a new check, after PathPoints potentially became empty
          (CallFunction|TurnTowardsNextPoint)
          (CallFunction|RunTowardsNextPoint))))))

(event Custom|UpdateNextPoint
  (bind _ownercharacter (Variables|Default|GetOwnerCharacter))
  (bind _pathpoints (Variables|Default|GetPathPoints))
  (bind _returnvalue (Transformation|GetActorLocation _ownercharacter))
  (bind _output (Utilities|Array|Get(acopy) _pathpoints))
  (bind (_x _y) (Math|Vector|BreakVector _output))
  (bind (_x_2 _y_2) (Math|Vector|BreakVector _returnvalue))
  ;[1 0.312 0.302] Update Next Path Point: if within 20 cm (@ 400 speed) of the next point, discard this point, so we can start moving towards the next point
  (bind _maxspeed (Default|GetMaxMoveSpeed (Variables|Default|GetOwnerCharacter)))
  (if (< (Class|KismetMathLibrary|VectorDistanceSquared (Math|Vector|MakeVector _x _y 0.0) (Math|Vector|MakeVector _x_2 _y_2 0.0)) (* 5e+02 (Math|Float|Square (/ _maxspeed 4e+02))))
    (Utilities|Array|RemoveIndex (Variables|Default|GetPathPoints))))

(event Custom|TurnTowardsNextPoint
  (bind _returnvalue (Utilities|Time|GetWorldDeltaSeconds))
  (bind _returnvalue_2 (Utilities|Time|GetWorldDeltaSeconds))
  (bind _pathpoints (Variables|Default|GetPathPoints))
  (bind _ownercharacter (Variables|Default|GetOwnerCharacter))
  (bind _ownercharacter_2 (Variables|Default|GetOwnerCharacter))
  (bind _ownercharacter_3 (Variables|Default|GetOwnerCharacter))
  (bind _ownercharacter_4 (Variables|Default|GetOwnerCharacter))
  (bind _turnspeed (Variables|Default|GetTurnSpeed))
  (bind _returnvalue_3 (Transformation|GetActorLocation _ownercharacter_3))
  (bind _returnvalue_4 (Transformation|GetActorRotation _ownercharacter_2))
  (bind _returnvalue_5 (Transformation|GetActorRotation _ownercharacter_4))
  (bind _output (Utilities|Array|Get(acopy) _pathpoints))
  (bind _returnvalue_6 (* _returnvalue_2 6e+01))
  (bind _returnvalue_7 (Math|Rotator|FindLookatRotation _returnvalue_3 _output))
  (bind _yaw (Math|Rotator|BreakRotator _returnvalue_5))
  (bind _yaw_2 (Math|Rotator|BreakRotator _returnvalue_4))
  (bind _returnvalue_8 (* 1e+01 _returnvalue_6))
  (bind _returnvalue_9 (Math|Rotator|NormalizeAxis _yaw))
  (bind _yaw_3 (Math|Rotator|BreakRotator _returnvalue_7))
  (bind _returnvalue_10 (Math|Rotator|MakeRotator 0.0 0.0 _yaw_3))
  (bind _yaw_4 (Math|Rotator|BreakRotator _returnvalue_10))
  (bind _returnvalue_11 (Math|Rotator|NormalizeAxis _yaw_4))
  (bind _returnvalue_12 (- _returnvalue_11 _returnvalue_9))
  (bind _returnvalue_13 (Math|Rotator|NormalizeAxis _returnvalue_12))
  (bind _returnvalue_14 (Math|Float|Sign(Float) _returnvalue_13))
  (bind _returnvalue_15 (Math|Float|Absolute(Float) _returnvalue_13))
  (bind _returnvalue_16 (* _returnvalue _returnvalue_14 _turnspeed))
  (bind _returnvalue_17 (< _returnvalue_15 _returnvalue_8))
  (bind _returnvalue_18 (+ _yaw_2 _returnvalue_16))
  (bind _returnvalue_19 (Math|Float|SelectFloat _yaw_4 _returnvalue_18 _returnvalue_17))
  (bind _returnvalue_20 (Math|Rotator|NormalizeAxis _returnvalue_19))
  (bind _returnvalue_21 (Math|Rotator|MakeRotator 0.0 0.0 _returnvalue_20))
  ;[1 0.312 0.302] This is a simple math formula to turn the character towards its next path point at constant speed
  ; Our target angle is: LookAt(Next Point)
  ; Our current angle is: Character's Yaw
  ; The difference between them is = Normalize(TargetAngle) - Normalize(CurrentAngle)
  ; Then normalize the difference itself and check its sign.
  ; If it's a plus sign, just add a bit of degrees (TurnSpeed * deltaTime) to Character's yaw.
  ; If it's a negative sign, substract the same amount.
  ; If the difference is negligible (<=10 degrees), then just set it to exactly Target Yaw already.
  ; By default it turns at around 12 degrees per frame, so 10 is a good fit.
  ; If you change TurnSpeed, make sure to adjust the "10" in the logic of this function or you might get yaw-jittering after it reaches its rotation goal.
  (if (Utilities|Array|IsNotEmpty (Variables|Default|GetPathPoints))
    (Transformation|SetActorRotation _ownercharacter _returnvalue_21)
    (Default|SetActorRotationonServer _ownercharacter _returnvalue_21)))

(event Custom|RunTowardsNextPoint
  ;[1 0.312 0.302] Run towards the next path point
  (Class|PawnMovementComponent|AddInputVector (Variables|/Script/Engine.Character|GetCharacterMovement (Variables|Default|GetOwnerCharacter)) (Math|Vector|GetForwardVector (Math|Rotator|MakeRotator 0.0 0.0 (.Yaw (Math|Rotator|BreakRotator (Math|Rotator|FindLookatRotation (Transformation|GetActorLocation (Variables|Default|GetOwnerCharacter)) (Utilities|Array|Get(acopy) (Variables|Default|GetPathPoints))))))) false))

(event EventZoominOut
  (params (X :type Float%20%28double-precision%29))
  ;[1 1 1] (Called on Tick) Zoom In/Out
  (Variables|Zoom|SetZoomAlpha (Math|Float|SelectFloat 0.2 (Math|Float|SelectFloat (Variables|Zoom|GetZoomAlpha) 0.0 (< (Variables|Zoom|GetZoomAlpha) 0.2)) (Math|Float|InRange(Float) (Variables|Zoom|GetZoomAlpha) 0.2 1.0 false false)))
  (Variables|Zoom|SetZoomFrom (Variables|/Script/Engine.SpringArmComponent|GetTargetArmLength (Variables|/Game/MMOKit/MMO_Logic/Blueprints/BP_PlayerCharacter.BP_PlayerCharacter_C|GetCameraBoom (Variables|Default|GetOwnerCharacter))))
  (Variables|Zoom|SetZoomTo (Math|Float|Clamp(Float) (+ (* X 1e+02) (Variables|Zoom|GetZoomTo)) 1e+02 1.2e+03)))

(event EventLookAround
  (params (InputVector :type Vector%202D%20Structure))
  (bind (_x _y) (Math|Vector2D|BreakVector2D InputVector))
  (bind _ownercontroller (Variables|Default|GetOwnerController))
  (bind _turnratemousegamepad (Variables|/Game/MMOKit/MMO_Logic/Blueprints/BP_PlayerController.BP_PlayerController_C|GetTurnRateMouseGamepad _ownercontroller))
  ;[1 1 1] LookAround
  ;;[1 1 1 0] Note: gamepad and mouse are polled differently in UE5.  For some reason, the mouse is FPS agnostic,
  ;; while the gamepad requires deltaTime. In this case, I've not fixed the gamepad, because:
  ;; a) this may get fixed in UE5 eventually
  ;; b) most MMO clients don't go beyond 60 fps
  ;; c) most MMOs aren't relient on gamepads
  ;; If you want to fix this, you have to decouple LookAround into two InputActions: MouseLookAround and GamepadLookAround.
  (if (Variables|Default|GetAllowCameraLook)
    (Class|PlayerController|AddYawInput (Variables|Default|GetOwnerController) (* _turnratemousegamepad _x 2.0))
    (Class|PlayerController|AddPitchInput (Variables|Default|GetOwnerController) (* _turnratemousegamepad _y 2.0))))

(event EventOnRMB
  (params (Down :type Boolean))
  (bind _ownercontroller (Variables|Default|GetOwnerController))
  (bind (_locationx _locationy) (Game|Player|GetMousePosition _ownercontroller))
  ;[1 0.312 0.302] RMB. Explanation:
  ; - LMB needs to move around even when it's down to guide the character
  ; - This means cursor positional lock is off during LMB down (we disable it by unchecking Hide Cursor During Capture in the setup)
  ; - But for RMB, we need keep it in place, otherwise it'll get blocked by screen borders during camera rotation. So we imitate it manually.
  (Variables|Default|SetRmbDown Down)
  (Variables|/Script/Engine.PlayerController|SetbShowMouseCursor (Variables|Default|GetOwnerController) (not (Variables|Default|GetRmbDown)))
  (if (Variables|Default|GetRmbDown)
    (Variables|Default|SetCachedMousePos (Math|Vector2D|MakeVector2D _locationx _locationy)) ; Save mouse pos when RMB goes down
    (else
      (Class|PlayerController|SetMouseLocation (Variables|Default|GetOwnerController) (Math|Float|Truncate (.X (Math|Vector2D|BreakVector2D (Variables|Default|GetCachedMousePos)))) (Math|Float|Truncate (.Y (Math|Vector2D|BreakVector2D (Variables|Default|GetCachedMousePos))))) ; Restore mouse pos after RMB is released
    )))

(event EventTick
  (params (DeltaSeconds :type Float%20%28single-precision%29))
  (bind _returnvalue (Viewport|GetViewportSize))
  (bind (_x _y) (Math|Vector2D|BreakVector2D _returnvalue))
  ;[1 1 1] Tick
  (CallFunction|ZoomUpdate)
  (CallFunction|AutoRun)
  (if (Variables|Default|GetRmbDown)
    (Class|PlayerController|SetMouseLocation (Variables|Default|GetOwnerController) (Math|Float|Truncate (/ _x 2.0)) (Math|Float|Truncate (/ _y 2.0))) ; Because we don't lock cursor in Point-n-Click,\nwe imitate lock by setting cursor to the center of the screen\nwhenever RMB is down (= when we're rotating the camera)
  ))

(event EventBeginPlay
  (bind _ownercharacter (Variables|Default|GetOwnerCharacter))
  (bind _ownercharacter_2 (Variables|Default|GetOwnerCharacter))
  (bind _ownercontroller (Variables|Default|GetOwnerController))
  (bind _ownercharacter_3 (Variables|Default|GetOwnerCharacter))
  (bind _followcamera (Variables|/Game/MMOKit/MMO_Logic/Blueprints/BP_PlayerCharacter.BP_PlayerCharacter_C|GetFollowCamera _ownercharacter_2))
  (bind _cameraboom (Variables|/Game/MMOKit/MMO_Logic/Blueprints/BP_PlayerCharacter.BP_PlayerCharacter_C|GetCameraBoom _ownercharacter))
  (bind _charactermovement (Variables|/Script/Engine.Character|GetCharacterMovement _ownercharacter_3))
  ;[1 1 1] BeginPlay: initialize camera and some variables
  (|CallParentFunction)
  (bind _output_get (Variables|/Script/Engine.SpringArmComponent|SetTargetArmLength _cameraboom 6.5e+02))
  (Variables|Zoom|SetZoomTo _output_get)
  (Transformation|SetRelativeLocation _cameraboom "0, 0,75.000000" false false)
  (Transformation|SetRelativeLocation _followcamera "0, 0, 0" false false)
  (Transformation|SetRelativeScale3D _followcamera "1.000000,1.000000,1.000000")
  (Input|SetInputModeGameandUI _ownercontroller 0 "LockOnCapture" false false)
  (Variables|/Script/Engine.PlayerController|SetbShowMouseCursor _ownercontroller true)
  (Variables|/Script/Engine.Pawn|SetbUseControllerRotationYaw _ownercharacter_3 false)
  (Variables|/Script/Engine.CharacterMovementComponent|SetRotationRate _charactermovement "0,500.000000, 0") ; just resetting it to default, not that we use it in thos camera mode
  (bind _output_get_2 (Variables|/Script/Engine.CharacterMovementComponent|SetbUseControllerDesiredRotation _charactermovement false))
  (Default|SetUseControllerRotationonServer (Variables|Default|GetOwnerCharacter) _output_get_2)
  (Variables|/Script/Engine.CharacterMovementComponent|SetRotationRate (Variables|/Script/Engine.Character|GetCharacterMovement (Variables|Default|GetOwnerCharacter)) (Math|Rotator|MakeRotator 0.0 0.0 -1.0))
  (Default|SetRotationRateonServer (Variables|Default|GetOwnerCharacter) -1.0)
  (Rendering|SetVisibility (Variables|/Script/Engine.Character|GetMesh (Variables|Default|GetOwnerCharacter)) true true)
  (Pawn|SetControlRotation (Variables|Default|GetOwnerController) (Math|Rotator|MakeRotator 0.0 -55.0 -135.0)) ; Default camera rotation
  (bind _charactereventbus (Default|GetCharacterEventBus (Variables|Default|GetOwnerCharacter)))
  (EventDispatchers|BindEventtoOnDeath _charactereventbus (EventDispatchers|CreateEvent :!event Custom|OnDeathResetPath)))

(event EventChatLostFocus
  (bind _ownercontroller (Variables|Default|GetOwnerController))
  ;[1 1 1] Chat Lost Focus
  (Input|SetInputModeGameOnly _ownercontroller false)
  (Input|SetInputModeGameandUI _ownercontroller 0 "LockOnCapture" false false)
  (Variables|/Script/Engine.PlayerController|SetbShowMouseCursor _ownercontroller true))

(event EventOnLMB
  (params (Down :type Boolean))
  ;[1 0.312 0.302] LMB: Set Path Destination to Attackable Character / Interactable / Ground Point
  (bind _output_get (Variables|Default|SetLmbDown Down))
  (if _output_get
    (CallFunction|GetAnythingUnderCursor true)))

(fn GetAnythingUnderCursor
  (params (LmbClick :type Boolean))
  (bind _array (Utilities|Array|MakeArray "ObjectTypeQuery1"))
  (bind _array_2 (Utilities|Array|MakeArray "ObjectTypeQuery7" "ObjectTypeQuery1" "ObjectTypeQuery2"))
  (bind _array_3 (Utilities|Array|MakeArray "ObjectTypeQuery3" "ObjectTypeQuery4" "ObjectTypeQuery1" "ObjectTypeQuery2"))
  (bind _ownercontroller (Variables|Default|GetOwnerController))
  (bind _ownercontroller_2 (Variables|Default|GetOwnerController))
  (bind _ownercharacter (Variables|Default|GetOwnerCharacter))
  (bind _ownercontroller_3 (Variables|Default|GetOwnerController))
  (bind _ownercharacter_2 (Variables|Default|GetOwnerCharacter))
  (bind (_hitresult _returnvalue) (Class|PlayerController|GetHitResultUnderCursorforObjects _ownercontroller _array false))
  (bind _array_4 (Utilities|Array|MakeArray _ownercharacter))
  (bind _array_5 (Utilities|Array|MakeArray _ownercharacter_2))
  (bind (_hitresult_2 _returnvalue_2) (Class|PlayerControllerCpp|GetHitResultUnderCursorforObjectswithIgnore _ownercontroller_2 _array_3 true _array_4))
  (bind (_hitresult_3 _returnvalue_3) (Class|PlayerControllerCpp|GetHitResultUnderCursorforObjectswithIgnore _ownercontroller_3 _array_2 true _array_5))
  ;[1 0.312 0.302] Do up to three raycasts:
  ; 1. Get unfriendly character under cursor, if found then pursue it. No more raycasts are performed.
  ; 2. Get interactible under cursor, if found then approach it. No more raycasts are performed.
  ; 3. If nothing else succeeds, find ground under cursor and go there.
  ;
  ; SetPathToTarget handles pursueing or stopping to pursue the target, and issuing a ReachedTarget event
  (if LmbClick
    (Utilities|FlowControl|Sequence
      (:then_0
        (if _returnvalue_2
          (LocalVariables|SetHitResult _hitresult_2)
          (bind _ascharacter (Utilities|Casting|CastToCharacter (.HitActor (Collision|BreakHitResult (LocalVariables|GetHitResult)))))
          (bind _alive (Class|BPICharacter|IsAlive(Message) _ascharacter))
          (if _alive
            (bind _reaction (Class|BPIReaction|GetReaction(Message) _ascharacter))
            (if (not (or (Utilities|Enum|Equal(Enum) _reaction "NewEnumerator0") (Utilities|Enum|Equal(Enum) _reaction "NewEnumerator3"))) ; If friendly character, ignore the click
              (Variables|Default|SetTrackTarget _ascharacter)
              (CallFunction|SetPathtoTarget)
              (return)))))
      (:then_1
        (if _returnvalue_3
          (bind _output_get (LocalVariables|SetHitResult _hitresult_3))
          (bind _can (Class|BPIInteractable|CanInteract(Message) (.HitActor (Collision|BreakHitResult _output_get))))
          (if _can
            (Variables|Default|SetTrackTarget (.HitActor (Collision|BreakHitResult _output_get)))
            (CallFunction|SetPathtoTarget)
            (return))))
      (:then_2
        (Variables|Default|SetTrackTarget 0)
        (if _returnvalue :!label _label
          (bind _output_get_2 (LocalVariables|SetHitResult _hitresult))
          (CallFunction|SetPathDestination (.Location (Collision|BreakHitResult _output_get_2))))))
    (else
      (Utilities|IsValid (Variables|Default|GetTrackTarget)
        (:Is%20Valid
          (CallFunction|SetPathtoTarget))
        (:Is%20Not%20Valid
          (goto _label))))))

(fn DebugDrawPath
  (bind _ownercharacter (Variables|Default|GetOwnerCharacter))
  ;[1 0.312 0.302] Draw Spheres & Lines
  ; Along navmesh path
  (Utilities|FlowControl|Sequence
    (:then_0
      ;[1 0.312 0.302] Draw Spheres
      (for _array_element (Variables|Default|GetPathPoints) ; draw spheres for each point on the navmesh
        (Rendering|Debug|DrawDebugSphere _array_element 35.0 12 "(R=0.000000,G=0.586572,B=1.000000,A=1.000000)" 0.0 1.0)))
    (:then_1
      ;[1 0.312 0.302] Draw lines between path points
      ; The first origin is from the character's feet
      (for (_array_element_2 _array_index) (Variables|Default|GetPathPoints) ; draw lines between character and pathpoints
        (LocalVariables|SetLineTarget _array_element_2)
        (Utilities|FlowControl|Sequence
          (:then_0
            (if (< _array_index 1)
              (LocalVariables|SetLineOrigin (- (Transformation|GetActorLocation _ownercharacter) (Math|Vector|MakeVector 0.0 0.0 (Components|Capsule|GetScaledCapsuleHalfHeight (Variables|/Script/Engine.Character|GetCapsuleComponent _ownercharacter)))))
              (else
                (LocalVariables|SetLineOrigin (Utilities|Array|Get(acopy) (Variables|Default|GetPathPoints) (- _array_index 1))))))
          (:then_1
            (Rendering|Debug|DrawDebugLine (LocalVariables|GetLineOrigin) (LocalVariables|GetLineTarget) "(R=0.000000,G=0.584079,B=1.000000,A=1.000000)" 0.0 1.0)))))))

(fn SetPathtoTarget
  (bind _ownercharacter (Variables|Default|GetOwnerCharacter))
  (bind _returnvalue (Transformation|GetActorLocation _ownercharacter))
  (bind (_x _y) (Math|Vector|BreakVector _returnvalue))
  ;[1 0.312 0.302] If we want to go to a target's location, we raycast from our character to target and hope to hit its colliders. It may work better than simply running towards it center in case it's irregularly-shaped.
  ; If we fail to (e.g. because the target is behind a wall), then let's move towards its general location for now.
  ; If we succeed, we try to move to where the raycast hit.
  ;
  ; It's not a big deal if we failed, because on tick we'll still call this function again and eventually get a clear path.
  ; The only problem would happen if the target has no colliders in its center for our raycast to hit.
  ;
  ; Because this function gets called on Tick, it'll chase moving objects/creatures.
  ;
  ; If we're chasing an interactable object, then once within 100 cm of desired location, stop moving and dispatch ReachedTarget event.
  ; If we're chasing a mob, then once within weapon range (or mob's + player's collider radius in case of FAT mobs), stop chasing and dispatch ReachedTarget event.
  ;
  ; ReachedTarget either triggers an Interact or an Attack in BP_InteractionPointNClick::OnTargetReached event.
  ;
  ; If LMB isn't pressed down, we can set target to nothing and stop attacking. But if LMB is pressed down, attacks will continue, even if the cursor is not over the target.
  ; It's almost the exact same behavior as Path of Exile.
  (bind _range (Default|GetWeaponRange (Variables|Default|GetOwnerCharacter)))
  (LocalVariables|SetWeaponRange _range)
  (LocalVariables|SetProtagCapsuleRadius (Variables|/Script/Engine.CapsuleComponent|GetCapsuleRadius (Variables|/Script/Engine.Character|GetCapsuleComponent (Variables|Default|GetOwnerCharacter))))
  (Utilities|FlowControl|Sequence
    (:then_0
      (bind _ascharacter (Utilities|Casting|CastToCharacter (Variables|Default|GetTrackTarget))
        (:then
          (LocalVariables|SetTargetIsCharacter true)
          (LocalVariables|SetTargetCapsuleRadius (Variables|/Script/Engine.CapsuleComponent|GetCapsuleRadius (Variables|/Script/Engine.Character|GetCapsuleComponent _ascharacter))))
        (:CastFailed
          (LocalVariables|SetTargetIsCharacter false)))
      (bind (_outhit _returnvalue_2) (Collision|LineTraceForObjects (Transformation|GetActorLocation (Variables|Default|GetOwnerCharacter)) (Transformation|GetActorLocation (Variables|Default|GetTrackTarget)) (select (LocalVariables|GetTargetIsCharacter) (Utilities|Array|MakeArray "ObjectTypeQuery3" "ObjectTypeQuery4" "ObjectTypeQuery1" "ObjectTypeQuery2") (Utilities|Array|MakeArray "ObjectTypeQuery7" "ObjectTypeQuery1" "ObjectTypeQuery2")) true (Utilities|Array|MakeArray (Variables|Default|GetOwnerCharacter)) "ForOneFrame" false))
      (if _returnvalue_2
        (bind _output_get (LocalVariables|SetTargetDestination (.ImpactPoint (Collision|BreakHitResult _outhit))))
        (CallFunction|SetPathDestination _output_get)
        (else
          (bind _output_get_2 (LocalVariables|SetTargetDestination (Transformation|GetActorLocation (Variables|Default|GetTrackTarget))))
          (CallFunction|SetPathDestination _output_get_2))))
    (:then_1
      ;;[1 0.312 0.302] When/if target is reached, dispatch ReachedTarget event
      (if (<= (Class|KismetMathLibrary|VectorDistanceSquared (Math|Vector|MakeVector _x _y 0.0) (Math|Vector|MakeVector (.X (Math|Vector|BreakVector (Transformation|GetActorLocation (Variables|Default|GetTrackTarget)))) (.Y (Math|Vector|BreakVector (Transformation|GetActorLocation (Variables|Default|GetTrackTarget)))) 0.0)) (Math|Float|Square (Math|Float|SelectFloat (Math|Float|Max(Float) (+ (LocalVariables|GetProtagCapsuleRadius) (LocalVariables|GetTargetCapsuleRadius)) (LocalVariables|GetWeaponRange)) (+ (LocalVariables|GetProtagCapsuleRadius) 1.4e+02) (LocalVariables|GetTargetIsCharacter)))) ; If we're within N cm of target, stop chasing
        (Variables|Default|SetPathPoints (Utilities|Array|MakeArray (Transformation|GetActorLocation (Variables|Default|GetTrackTarget)))) ; Set point to turn towards (i.e. target actor)
        (CallFunction|TurnTowardsNextPoint)
        (Default|CallReachedTarget (Variables|Default|GetTrackTarget)) ; Will result in an attack, it's listened to in Point-n-Click Interaction Component
        (Utilities|Array|Clear (Variables|Default|GetPathPoints)) ; Stops movement
        ;;[1 0.312 0.302] If we just reached interactable, reset target, as we don't want to interact multiple times with it
        (Utilities|Casting|CastToBPI_Interactable (Variables|Default|GetTrackTarget)
          (:then
            (Variables|Default|SetTrackTarget 0))
          (:CastFailed
            ;;[1 0.312 0.302] LMB pressed down - character will continue to chase and attack target
            ;; LMB not down - character will stop chasing and attacking after performing one attack
            (Utilities|Casting|CastToCharacter (Variables|Default|GetTrackTarget))
            (if (not (Variables|Default|GetLmbDown)) ; After attacking once, don't continue pursueing/attacking if LMB is not pressed down
              (Variables|Default|SetTrackTarget 0))))))))

(fn GetCameraAttackOrigin
  (bind _ownercharacter (Variables|Default|GetOwnerCharacter))
  (bind _tracktarget (Variables|Default|GetTrackTarget))
  (bind _ownercharacter_2 (Variables|Default|GetOwnerCharacter))
  (bind _ownercharacter_3 (Variables|Default|GetOwnerCharacter))
  (bind _returnvalue (Transformation|GetActorLocation _ownercharacter_3))
  (bind _returnvalue_2 (Transformation|GetActorLocation _tracktarget))
  (bind _meleeattackvector (Variables|/Game/MMOKit/MMO_Logic/Blueprints/BP_BaseCharacter.BP_BaseCharacter_C|GetMeleeAttackVector _ownercharacter))
  (bind _meleeattackvector_2 (Variables|/Game/MMOKit/MMO_Logic/Blueprints/BP_BaseCharacter.BP_BaseCharacter_C|GetMeleeAttackVector _ownercharacter_2))
  (bind _returnvalue_3 (Transformation|GetWorldTransform _meleeattackvector))
  (bind _returnvalue_4 (Math|Rotator|FindLookatRotation _returnvalue _returnvalue_2))
  (bind _returnvalue_5 (Transformation|GetWorldTransform _meleeattackvector_2))
  (bind (_location _rotation _scale) (Math|Transform|BreakTransform _returnvalue_3))
  (bind (_location_2 _rotation_2 _scale_2) (Math|Transform|BreakTransform _returnvalue_5))
  (bind _yaw (Math|Rotator|BreakRotator _returnvalue_4))
  (bind _returnvalue_6 (Math|Rotator|MakeRotator 0.0 0.0 _yaw))
  (Utilities|IsValid (Variables|Default|GetTrackTarget)
    (:Is%20Valid
      ;[1 0.312 0.302] If target is valid, look at target and add 40cm to Character's MeleeAttachVector (it's an arrow component)
      (return (Math|Transform|MakeTransform (+ (* (Math|Vector|Normalize (Math|Vector|GetForwardVector _returnvalue_6)) 4e+01) _location) _returnvalue_6 _scale)))
    (:Is%20Not%20Valid
      ;[1 0.312 0.302] If no target, then simply add 40 cm to the same arrow component
      (return (Math|Transform|MakeTransform (+ _location_2 (* (Math|Vector|Normalize (Transformation|GetActorForwardVector _ownercharacter_2)) 4e+01)) _rotation_2 _scale_2)))))
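; Over-the-shoulder camera component for the MMO character, handling look, movement input, eased zoom and menu cursor mode.
; BeginPlay sets up the offset boom; jogging turns the character toward the camera, while swimming and flying follow camera pitch.
; Attack montages snap yaw to the camera and replicate it to the server, restoring turn rate next tick.
; GetCameraAttackOrigin lowers the boom origin, remaps pitch and angles yaw to align attacks with the offset view.
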(event Custom|RotateTowardsAttack
  (bind _ownercharacter (Variables|Default|GetOwnerCharacter))
  (bind _ownercharacter_2 (Variables|Default|GetOwnerCharacter))
  (bind _returnvalue (Transformation|GetActorRotation _ownercharacter_2))
  (bind _followcamera (Variables|/Game/MMOKit/MMO_Logic/Blueprints/BP_PlayerCharacter.BP_PlayerCharacter_C|GetFollowCamera _ownercharacter))
  (bind _returnvalue_2 (Transformation|GetWorldRotation _followcamera))
  (bind (_roll _pitch) (Math|Rotator|BreakRotator _returnvalue))
  (bind _yaw (Math|Rotator|BreakRotator _returnvalue_2))
  (bind _returnvalue_3 (Math|Rotator|MakeRotator _roll _pitch _yaw))
  ;[1 1 1] When character attacks, he must rotate immediately towards his vector of attack
  ; Then he must set his turn rate back to desired one
  (Variables|/Script/Engine.CharacterMovementComponent|SetRotationRate (Variables|/Script/Engine.Character|GetCharacterMovement (Variables|Default|GetOwnerCharacter)) (Math|Rotator|MakeRotator 0.0 0.0 -1.0))
  (Default|SetRotationRateonServer (Variables|Default|GetOwnerCharacter) -1.0)
  (Default|SetActorRotationonServer (Variables|Default|GetOwnerCharacter) _returnvalue_3)
  (Transformation|SetActorRotation (Variables|Default|GetOwnerCharacter) _returnvalue_3)
  (Utilities|FlowControl|DelayUntilNextTick)
  (Variables|/Script/Engine.CharacterMovementComponent|SetRotationRate (Variables|/Script/Engine.Character|GetCharacterMovement (Variables|Default|GetOwnerCharacter)) (Math|Rotator|MakeRotator 0.0 0.0 (Variables|Default|GetCharRotationRateYaw)))
  (Default|SetRotationRateonServer (Variables|Default|GetOwnerCharacter) (Variables|Default|GetCharRotationRateYaw)))

(event Custom|ZoomUpdate
  ;[1 1 1] Zoom In/Out is executed in the Tick event
  (if (< (Variables|Zoom|GetZoomAlpha) 1.0)
    (Variables|/Script/Engine.SpringArmComponent|SetTargetArmLength (Variables|/Game/MMOKit/MMO_Logic/Blueprints/BP_PlayerCharacter.BP_PlayerCharacter_C|GetCameraBoom (Variables|Default|GetOwnerCharacter)) (Math|Interpolation|Ease "EaseInOut" (Variables|Zoom|GetZoomAlpha) (Variables|Zoom|GetZoomFrom) (Variables|Zoom|GetZoomTo) 2.0))
    (Variables|Zoom|SetZoomAlpha (+ (Variables|Zoom|GetZoomAlpha) (Math|Float|SafeDivide (Utilities|Time|GetWorldDeltaSeconds) 0.3))) ; Increase alpha on each tick by\nDeltaTime*(1/ZoomTime)\n1/ZoomTime is ZoomSpeed
  ))

(event EventZoominOut
  (params (X :type Float%20%28double-precision%29))
  ;[1 1 1] Zoom In/Out is executed in the Tick event
  (Variables|Zoom|SetZoomAlpha (Math|Float|SelectFloat 0.2 (Math|Float|SelectFloat (Variables|Zoom|GetZoomAlpha) 0.0 (< (Variables|Zoom|GetZoomAlpha) 0.2)) (Math|Float|InRange(Float) (Variables|Zoom|GetZoomAlpha) 0.2 1.0 false false)))
  (Variables|Zoom|SetZoomFrom (Variables|/Script/Engine.SpringArmComponent|GetTargetArmLength (Variables|/Game/MMOKit/MMO_Logic/Blueprints/BP_PlayerCharacter.BP_PlayerCharacter_C|GetCameraBoom (Variables|Default|GetOwnerCharacter))))
  (Variables|Zoom|SetZoomTo (Math|Float|Clamp(Float) (+ (* X 1e+02) (Variables|Zoom|GetZoomTo)) 2e+02 7e+02)))

(event EventLookAround
  (params (InputVector :type Vector%202D%20Structure))
  (bind (_x _y) (Math|Vector2D|BreakVector2D InputVector))
  (bind _ownercontroller (Variables|Default|GetOwnerController))
  (bind _turnratemousegamepad (Variables|/Game/MMOKit/MMO_Logic/Blueprints/BP_PlayerController.BP_PlayerController_C|GetTurnRateMouseGamepad _ownercontroller))
  ;[1 1 1] LookAround
  ;;[1 1 1 0] Note: gamepad and mouse are polled differently in UE5.  For some reason, the mouse is FPS agnostic,
  ;; while the gamepad requires deltaTime. In this case, I've not fixed the gamepad, because:
  ;; a) this may get fixed in UE5 eventually
  ;; b) most MMO clients don't go beyond 60 fps
  ;; c) most MMOs aren't relient on gamepads
  ;; If you want to fix this, you have to decouple LookAround into two InputActions: MouseLookAround and GamepadLookAround.
  (if (not (Variables|Default|GetMenuMode))
    (Class|PlayerController|AddYawInput (Variables|Default|GetOwnerController) (* _turnratemousegamepad _x))
    (Class|PlayerController|AddPitchInput (Variables|Default|GetOwnerController) (* _turnratemousegamepad _y))))

(event EventJog
  (params (InputVector :type Vector%202D%20Structure))
  (bind (_x _y) (Math|Vector2D|BreakVector2D InputVector))
  (bind (_x_2 _y_2) (Math|Vector2D|BreakVector2D InputVector))
  (bind _ownercharacter (Variables|Default|GetOwnerCharacter))
  (bind _ownercharacter_2 (Variables|Default|GetOwnerCharacter))
  (bind _returnvalue (Transformation|GetActorRotation _ownercharacter_2))
  (bind _followcamera (Variables|/Game/MMOKit/MMO_Logic/Blueprints/BP_PlayerCharacter.BP_PlayerCharacter_C|GetFollowCamera _ownercharacter))
  (bind _yaw (Math|Rotator|BreakRotator _returnvalue))
  (bind _returnvalue_2 (Transformation|GetWorldRotation _followcamera))
  (bind (_roll _pitch _yaw_2) (Math|Rotator|BreakRotator _returnvalue_2))
  (bind _returnvalue_3 (Math|Rotator|MakeRotator 0.0 0.0 _yaw))
  (bind _returnvalue_4 (+ _pitch 1e+01))
  (bind _returnvalue_5 (Math|Rotator|MakeRotator 0.0 _returnvalue_4 _yaw_2))
  ;[1 1 1] Jog: in the direction of the Player Character
  (switch Utilities|FlowControl|Switch|SwitchonEMovementMode (Variables|/Script/Engine.CharacterMovementComponent|GetMovementMode (Variables|/Script/Engine.Character|GetCharacterMovement (Variables|Default|GetOwnerCharacter)))
    (:MOVE_Walking
      (Class|PawnMovementComponent|AddInputVector (Variables|/Script/Engine.Character|GetCharacterMovement (Variables|Default|GetOwnerCharacter)) (+ (* (Math|Vector|GetForwardVector _returnvalue_3) _y_2) (* (Math|Vector|GetRightVector _returnvalue_3) _x_2)) false :!label _label))
    (:MOVE_NavWalking
      (goto _label))
    (:MOVE_Falling
      (goto _label))
    (:MOVE_Swimming
      ;[1 1 1] Fly/Swim: in the direction of the camera + 10 degrees upwards (pitch) to see a bit of the view below
      (Class|PawnMovementComponent|AddInputVector (Variables|/Script/Engine.Character|GetCharacterMovement (Variables|Default|GetOwnerCharacter)) (+ (* (Math|Vector|GetForwardVector _returnvalue_5) _y) (* (Math|Vector|GetRightVector _returnvalue_5) _x)) false :!label _label_2))
    (:MOVE_Flying
      (goto _label_2))))

(event EventJogStart
  ;[1 1 1] On jog start/end: turn towards camera
  (bind _output_get (Variables|/Script/Engine.CharacterMovementComponent|SetbUseControllerDesiredRotation (Variables|/Script/Engine.Character|GetCharacterMovement (Variables|Default|GetOwnerCharacter)) true))
  (Default|SetUseControllerRotationonServer (Variables|Default|GetOwnerCharacter) _output_get))

(event EventBeginPlay
  (bind _ownercharacter (Variables|Default|GetOwnerCharacter))
  (bind _ownercharacter_2 (Variables|Default|GetOwnerCharacter))
  (bind _ownercontroller (Variables|Default|GetOwnerController))
  (bind _cameraboom (Variables|/Game/MMOKit/MMO_Logic/Blueprints/BP_PlayerCharacter.BP_PlayerCharacter_C|GetCameraBoom _ownercharacter))
  (bind _charactermovement (Variables|/Script/Engine.Character|GetCharacterMovement _ownercharacter_2))
  ;[1 1 1] BeginPlay
  (|CallParentFunction)
  (Input|SetInputModeGameOnly _ownercontroller false)
  (Variables|/Script/Engine.PlayerController|SetbShowMouseCursor _ownercontroller false)
  (Variables|/Script/Engine.Pawn|SetbUseControllerRotationYaw _ownercharacter false)
  (Transformation|SetRelativeLocation _cameraboom "0, 0,80.000000" false false)
  (Transformation|SetRelativeScale3D _cameraboom "1.000000,1.000000,1.000000")
  (bind _output_get (Variables|/Script/Engine.SpringArmComponent|SetTargetArmLength _cameraboom 2e+02))
  (Variables|Zoom|SetZoomTo _output_get)
  (Transformation|SetRelativeLocation (Variables|/Game/MMOKit/MMO_Logic/Blueprints/BP_PlayerCharacter.BP_PlayerCharacter_C|GetFollowCamera (Variables|Default|GetOwnerCharacter)) "0,55.000000, 0" false false)
  (Variables|/Script/Engine.CharacterMovementComponent|SetRotationRate _charactermovement "0,700.000000, 0")
  (bind _output_get_2 (Variables|/Script/Engine.CharacterMovementComponent|SetbUseControllerDesiredRotation _charactermovement false))
  (Default|SetUseControllerRotationonServer (Variables|Default|GetOwnerCharacter) _output_get_2)
  (Variables|/Script/Engine.CharacterMovementComponent|SetRotationRate (Variables|/Script/Engine.Character|GetCharacterMovement (Variables|Default|GetOwnerCharacter)) (Math|Rotator|MakeRotator 0.0 0.0 (Variables|Default|GetCharRotationRateYaw)))
  (Default|SetRotationRateonServer (Variables|Default|GetOwnerCharacter) (Variables|Default|GetCharRotationRateYaw))
  (Rendering|SetVisibility (Variables|/Script/Engine.Character|GetMesh (Variables|Default|GetOwnerCharacter)) true true)
  (EventDispatchers|BindEventtoOnAttackMontage (Variables|Default|GetOwnerCharacter) (delegate Custom|RotateTowardsAttack)))

(event EventTick
  (params (DeltaSeconds :type Float%20%28single-precision%29))
  ;[1 1 1] Tick
  (CallFunction|ZoomUpdate))

(event EventJogEnd
  ;[1 1 1] On jog start/end: turn towards camera
  (bind _output_get (Variables|/Script/Engine.CharacterMovementComponent|SetbUseControllerDesiredRotation (Variables|/Script/Engine.Character|GetCharacterMovement (Variables|Default|GetOwnerCharacter)) false))
  (Default|SetUseControllerRotationonServer (Variables|Default|GetOwnerCharacter) _output_get))

(event EventMenuModeToggle
  (params (On :type Boolean))
  (bind _ownercontroller (Variables|Default|GetOwnerController))
  ;[1 1 1] Menu Mode Toggle
  (bind _output_get (Variables|Default|SetMenuMode On))
  (if _output_get
    (Input|SetInputModeGameandUI _ownercontroller 0 "DoNotLock" false false)
    (Variables|/Script/Engine.PlayerController|SetbShowMouseCursor _ownercontroller true)
    (else
      (Input|SetInputModeGameOnly _ownercontroller false)
      (Variables|/Script/Engine.PlayerController|SetbShowMouseCursor _ownercontroller false))))

(event EventChatLostFocus
  (bind _ownercontroller (Variables|Default|GetOwnerController))
  ;[1 1 1] Chat Lost Focus
  (if (Variables|Default|GetMenuMode)
    (Input|SetInputModeGameOnly _ownercontroller false)
    (Input|SetInputModeGameandUI _ownercontroller 0 "DoNotLock" false false)
    (else
      (Input|SetInputModeGameOnly _ownercontroller false))))

(fn GetCameraAttackOrigin
  (bind _ownercharacter (Variables|Default|GetOwnerCharacter))
  (bind _cameraboom (Variables|/Game/MMOKit/MMO_Logic/Blueprints/BP_PlayerCharacter.BP_PlayerCharacter_C|GetCameraBoom _ownercharacter))
  (bind _followcamera (Variables|/Game/MMOKit/MMO_Logic/Blueprints/BP_PlayerCharacter.BP_PlayerCharacter_C|GetFollowCamera _ownercharacter))
  (bind _returnvalue (Transformation|GetWorldTransform _cameraboom))
  (bind _returnvalue_2 (Transformation|GetWorldRotation _followcamera))
  (bind (_location _rotation _scale) (Math|Transform|BreakTransform _returnvalue))
  (bind (_roll _pitch _yaw) (Math|Rotator|BreakRotator _returnvalue_2))
  (bind _pitch_2 (Math|Rotator|BreakRotator _returnvalue_2))
  (bind _returnvalue_3 (Math|Float|InRange(Float) _pitch_2 -2e+01 0.0))
  (bind _returnvalue_4 (Math|Float|MapRangeClamped _pitch_2 -2e+01 -9e+01 2e+01 5.0))
  (bind _returnvalue_5 (< _pitch_2 2e+01))
  (bind _returnvalue_6 (+ _pitch_2 _returnvalue_4))
  (bind _returnvalue_7 (Math|Float|SelectFloat _returnvalue_6 _pitch_2 _returnvalue_5))
  (bind _returnvalue_8 (Math|Float|SelectFloat 0.0 _returnvalue_7 _returnvalue_3))
  (bind _returnvalue_9 (Math|Rotator|MakeRotator _roll _returnvalue_8 _yaw))
  ;[1 1 1] This code:
  ; - lowers the origin point by 40cm from the boom camera
  ; - turns the angle to the right by 20 degrees, because we're in an over the shoulder camera, so in order to hit what's under the cursor, we need to rotate it a little
  ; - uses the Pitch (vertical angle) of the Follow Camera, but modifies it a little "a la New World"
  (return (Math|Transform|MakeTransform (- _location "0,0,40.000000") (Math|Rotator|CombineRotators _returnvalue_9 (Math|Vector|RotatorfromAxisandAngle (Math|Vector|GetUpVector _returnvalue_9) 2e+01)) _scale)))
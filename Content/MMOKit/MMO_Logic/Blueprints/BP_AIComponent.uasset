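; AI component that manages a mob's aggro list and current target.
; Damage from the owner's event bus accumulates per-attacker aggro, and players are notified when aggro changes.
; Target selection prunes invalid entries and takes the last living one, as the highest-value tracker never updates, falling back to in-range characters for one reaction type.
; Target changes go out on the bus, while Tick drops targets with an aggro-blocking effect.
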(event Custom|OnGotHit
  (params (Attacker :type Character%20Object%20Reference) (Damage :type Integer))
  (bind _aggrolist (Variables|Default|GetAggroList))
  (bind (_value _returnvalue) (Utilities|Map|Find _aggrolist Attacker))
  (bind _returnvalue_2 (Math|Integer|SelectInt _value 0 _returnvalue))
  (bind _returnvalue_3 (+ _returnvalue_2 Damage))
  (Utilities|FlowControl|Sequence
    (:then_0
      ;[0.4452 0.6332 1] Adds or removes characters from AgroList depending on the total AggroValue they've contributed
      ; If they've contributed an accumulated negative aggro value they are removed from AggroList
      (Utilities|IsValid Attacker
        (:Is%20Valid
          (if (> _returnvalue_3 0)
            (CallFunction|AddorUpdateAggroList Attacker _returnvalue_3 (not _returnvalue))
            (else
              (CallFunction|RemovefromAggroList Attacker))))))
    (:then_1
      (CallFunction|UpdateTarget))))

(event Custom|OnPlayerEnterAggroRange
  (params (Entrant :type Character%20Object%20Reference))
  ;[0.4452 0.6332 1] On Player Enter Aggro Range
  (if (CallFunction|IsCharacterValidforAggro Entrant)
    (Utilities|Array|AddUnique (Variables|Default|GetCharsInAggroRange) Entrant)
    (CallFunction|UpdateTarget) ; will attack if not otherwise engaged
  ))

(event Custom|OnPlayerLeaveAggroRange
  (params (Leaver :type Character%20Object%20Reference))
  ;[0.4452 0.6332 1] BeginPlay
)

(event Custom|UpdateTarget
  (bind _ownereventbus (Variables|Default|GetOwnerEventBus))
  ;[0.4452 0.6332 1] Update target if necessary
  (bind _newtarget (CallFunction|FindBestTarget))
  (if (!= _newtarget (Variables|Default|GetTargetCharacter))
    (bind _output_get (Variables|Default|SetTargetCharacter _newtarget))
    ;;[0.4452 0.6332 1] if mob spawns on top of a player, AiController is not ready yet, and so the bus isn't ready either. Wait a frame.
    (if (Variables|/Game/MMOKit/MMO_Logic/Blueprints/EventBuses/BP_CharacterEventBus.BP_CharacterEventBus_C|GetIsBusReady _ownereventbus) :!label _label
      (Default|CallOnTargetChanged _ownereventbus _output_get)
      (else
        (Utilities|FlowControl|DelayUntilNextTick)
        (goto _label)))))

(event Custom|AddOrUpdateAggroList
  (params (Char :type Character%20Object%20Reference) (AggroValue :type Integer) (FreshlyAdded :type Boolean))
  ;[0.4452 0.6332 1] Will add a target to aggro list
  ; If target is player, we'll send them a notification that this mob is now aggro
  (Utilities|FlowControl|Sequence
    (:then_0
      (if FreshlyAdded
        (Class|BPIPlayerCharacterSpecific|ChangeReactiontoCreature(Message) Char true (.AsCharacter (Utilities|Casting|CastToCharacter (Components|GetOwner))))))
    (:then_1
      (Utilities|Map|Add (Variables|Default|GetAggroList) Char AggroValue))))

(event Custom|RemoveFromAggroList
  (params (Char :type Character%20Object%20Reference))
  ;[0.4452 0.6332 1] Will remove a target from aggro list
  ; If target is player, we'll send them a notification that this mob is no longer aggro
  ; Does not reset the target, if Char is current target!
  (bind _returnvalue (Utilities|Map|Remove (Variables|Default|GetAggroList) Char))
  (if (and (Utilities|IsValid Char) _returnvalue)
    (Class|BPIPlayerCharacterSpecific|ChangeReactiontoCreature(Message) Char false (.AsCharacter (Utilities|Casting|CastToCharacter (Components|GetOwner))))))

(event Custom|DropCurrentTarget
  ;[0.4452 0.6332 1] Drop Current Target
  (CallFunction|RemovefromAggroList (Variables|Default|GetTargetCharacter))
  (Variables|Default|SetTargetCharacter 0)
  (Default|CallOnTargetChanged (Variables|Default|GetOwnerEventBus))
  (CallFunction|FindBestTarget))

(event EventBeginPlay
  ;[0.4452 0.6332 1] BeginPlay
  (bind _eventbus (Class|BPIMobSpecific|GetMobEventBus(Message) (Components|GetOwner)))
  (bind _output_get (Variables|Default|SetOwnerEventBus _eventbus))
  (EventDispatchers|AssignOnGotHit _output_get (EventDispatchers|CreateEvent :!event Custom|OnGotHit))
  (EventDispatchers|BindEventtoOnPlayerEnterAggroRange (Variables|Default|GetOwnerEventBus) (delegate Custom|OnPlayerEnterAggroRange))
  (EventDispatchers|BindEventtoOnPlayerLeftAggroRange (Variables|Default|GetOwnerEventBus) (delegate Custom|OnPlayerLeaveAggroRange)))

(event EventTick
  (params (DeltaSeconds :type Float%20%28single-precision%29))
  (bind _targetcharacter (Variables|Default|GetTargetCharacter))
  ;[0.4452 0.6332 1] OnTick is a bit lazy way of doing it. We check if current target has become invalid for aggro and drop it if it has.
  ; Feel free to optimize it by dispatching events.
  (Utilities|IsValid _targetcharacter
    (:Is%20Valid
      (if (not (CallFunction|IsCharacterValidforAggro _targetcharacter))
        (CallFunction|DropCurrentTarget)))))

(fn FindBestTarget
  ;[0.4452 0.6332 1] Returns a character with the highest aggro value
  ; - if a character is no longer valid (e.g. got destroyed), it's removed from the aggro list
  ; - if a character with a negative aggro value is encountered, it's removed from aggro list
  ;
  ; If we run out of aggro list, but we're a hostile mob, try finding someone in aggro range
  (LocalVariables|SetHighestAggroValue 0)
  (LocalVariables|SetHighestAggroCharacter 0)
  (bind _keys (Utilities|Map|Keys (Variables|Default|GetAggroList)))
  (for _array_element _keys
    (Utilities|IsValid _array_element
      (:Is%20Valid
        (if (> (.Value (Utilities|Map|Find (Variables|Default|GetAggroList) _array_element)) 0)
          (bind _alive (Class|BPICharacter|IsAlive(Message) _array_element))
          (if _alive
            (if (> (.Value (Utilities|Map|Find (Variables|Default|GetAggroList) _array_element)) (LocalVariables|GetHighestAggroValue))
              (LocalVariables|SetHighestAggroCharacter _array_element))
            (else
              (Utilities|Array|Add (LocalVariables|GetKeysToRemove) _array_element :!label _label)))
          (else
            (goto _label))))
      (:Is%20Not%20Valid
        (goto _label))))
  (for _array_element_2 (LocalVariables|GetKeysToRemove)
    (CallFunction|RemovefromAggroList _array_element_2))
  (Utilities|IsValid (LocalVariables|GetHighestAggroCharacter)
    (:Is%20Valid
      (return (LocalVariables|GetHighestAggroCharacter)))
    (:Is%20Not%20Valid
      ;;[0.4452 0.6332 1] if we ran out of aggro list, but we're a hostile mob, try getting a random player from aggro range
      (bind _reaction (Class|BPIMobSpecific|GetMobInitialReaction(Message) (Components|GetOwner)))
      (if (and (Utilities|Enum|Equal(Enum) _reaction "NewEnumerator2") (> (Utilities|Array|Length (Variables|Default|GetCharsInAggroRange)) 0))
        (for _array_element_3 (Variables|Default|GetCharsInAggroRange)
          (bind _alive_2 (Class|BPICharacter|IsAlive(Message) _array_element_3))
          (if _alive_2
            (return _array_element_3))))
      (return 0))))

(fn IsCharacterValidforAggro
  (params (Char :type Character%20Object%20Reference))
  (bind _found (Class|BPIBuffs|CharacterHasEffect(Message) Char "NewEnumerator1"))
  (return (not _found)))
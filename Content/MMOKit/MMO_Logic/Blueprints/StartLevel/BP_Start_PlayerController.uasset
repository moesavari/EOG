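; Player controller for the MMO start level, driving the login HUD, character selection and character creation screens.
; On BeginPlay it spawns the WebSockets actor, connects to the persistence server, logs the Steam ticket and warns in PIE if the connection fails.
; It swaps widgets per screen, returns to the start HUD on disconnect, and spawns or restyles a preview character dummy at a BP_EmptyActor's location.
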(event Custom|OnDisconnectResetEverything
  ;[1 0.312 0.302] On Disconnect, go back to WBP_Start_Hud
  (CallFunction|RemoveAllWidgets)
  (CallFunction|HideDummy)
  (bind _returnvalue (UserInterface|CreateWidget "/Game/MMOKit/MMO_Logic/Widgets/StartLevel/WBP_Start_HUD.WBP_Start_HUD_C" self))
  (bind _output_get (Variables|Default|SetStartHUD _returnvalue))
  (UserInterface|Viewport|AddtoViewport _output_get 0))

(event Custom|DisplayStartWarning
  ;[0.7865 0.1065 0.7201] If launching PIE in incorrect net mode, display a warning
  (CallFunction|DisplayStartWarningClient))

(event Custom|PrintSteamTicket
  ;[1 0.312 0.302] Print Steam Ticket
  (Class|MmoUtilities|LogString (Utilities|String|Append "Steam id: " (Class|MmoUtilities|GetSteamUserId)) "Verbosity_SuperVerbose")
  (Class|MmoUtilities|LogString (Utilities|String|Append "Steam ticket: " (Class|MmoUtilities|GetSteamSessionTicket)) "Verbosity_SuperVerbose"))

(event Custom|DisplayStartWarningClient
  ;[0.7865 0.1065 0.7201] If launching PIE in incorrect net mode, display a warning
  (bind _returnvalue (UserInterface|CreateWidget "/Game/MMOKit/MMO_Logic/Widgets/WBP_EditorWarning3.WBP_EditorWarning3_C"))
  (UserInterface|Viewport|AddtoViewport _returnvalue 0))

(event Custom|RemoveAllWidgets
  ;[1 0.312 0.302] Remove All Widgets (call before transitioning to another widget)
  (Viewport|RemoveAllWidgets)
  (Variables|Default|SetStartHUD 0)
  (Variables|Default|SetCharSelectionMenu 0)
  (Variables|Default|SetCharCreationMenu 0))

(event EventBeginPlay
  ;[1 1 1] BeginPlay
  (Networking|CanExecuteCosmeticEvents
    (:True
      (bind _returnvalue (Game|SpawnActorfromClass "/Game/MMOKit/MMO_Logic/Blueprints/WebSockets/BP_WebSockets.BP_WebSockets_C" (Math|Transform|MakeTransform "0, 0, 0" "0, 0, 0" "1.000000,1.000000,1.000000") "Undefined" "OverrideRootScale" 0 0))
      (Variables|Default|SetStartTcpConnectionClient _returnvalue)
      (bind _returnvalue_2 (UserInterface|CreateWidget "/Game/MMOKit/MMO_Logic/Widgets/StartLevel/WBP_Start_HUD.WBP_Start_HUD_C" self))
      (bind _output_get (Variables|Default|SetStartHUD _returnvalue_2))
      (UserInterface|Viewport|AddtoViewport _output_get 0)
      (Input|SetInputModeUIOnly self 0 "DoNotLock" false)
      (Variables|Default|SetbShowMouseCursor self true)
      (Default|ConnecttoPersistenceServer (Variables|Default|GetStartTcpConnectionClient))
      (CallFunction|PrintSteamTicket)
      (EventDispatchers|BindEventtoOnGotDisconnected (Variables|Default|GetBP_Start_EventBus) (EventDispatchers|CreateEvent :!event Custom|OnDisconnectResetEverything))
      ;[1 0.312 0.302] If not connected to persistent server in PIE, display a warning
      (bind _returnvalue_3 (Class|MmoUtilities|InPieWorld))
      (if _returnvalue_3
        (Utilities|FlowControl|Delay 1.0)
        (if (not (Class|WebSocketConn|IsConnected (Variables|Default|GetStartTcpConnectionClient)))
          (bind _returnvalue_4 (UserInterface|CreateWidget "/Game/MMOKit/MMO_Logic/Widgets/WBP_EditorWarning1.WBP_EditorWarning1_C"))
          (UserInterface|Viewport|AddtoViewport _returnvalue_4 0))))))

(event EventGotoCharacterSelection
  ;[1 0.312 0.302] Go to Char Selection (from WBP_Start_Hud)
  (CallFunction|RemoveAllWidgets)
  (bind _returnvalue (UserInterface|CreateWidget "/Game/MMOKit/MMO_Logic/Widgets/StartLevel/WBP_CharSelection.WBP_CharSelection_C"))
  (bind _output_get (Variables|Default|SetCharSelectionMenu _returnvalue))
  (UserInterface|Viewport|AddtoViewport _output_get 0))

(event EventGotoCharacterCreation
  ;[1 0.312 0.302] Go to Char Creation (from WBP_CharSelection)
  (CallFunction|RemoveAllWidgets)
  (bind _returnvalue (UserInterface|CreateWidget "/Game/MMOKit/MMO_Logic/Widgets/StartLevel/WBP_CharCreation.WBP_CharCreation_C"))
  (bind _output_get (Variables|Default|SetCharCreationMenu _returnvalue))
  (UserInterface|Viewport|AddtoViewport _output_get 0))

(event EventSpawnDummy
  (params (Appearance :type F%20Appearance%20Full%20Structure))
  ;[1 0.312 0.302] Spawn or update dummy
  (Utilities|IsValid (Variables|Default|GetDummy)
    (:Is%20Valid
      (Default|SetNewLook (Variables|Default|GetDummy) Appearance)
      (Rendering|SetActorHiddenInGame (Variables|Default|GetDummy) false))
    (:Is%20Not%20Valid
      (bind _outactors (Actor|GetAllActorsOfClass "/Game/MMOKit/MMO_Logic/Blueprints/StartLevel/BP_EmptyActor.BP_EmptyActor_C"))
      (if (> (Utilities|Array|Length _outactors) 0)
        (bind _returnvalue (Game|SpawnActorfromClass "/Game/MMOKit/MMO_Logic/Blueprints/StartLevel/BP_CharacterCreationDummy.BP_CharacterCreationDummy_C" (Transformation|GetActorTransform (Utilities|Array|Get(acopy) _outactors)) "Undefined" "MultiplyWithRoot" 0 Appearance 0))
        (Variables|Default|SetDummy _returnvalue)))))

(event EventChangeDummyAppearance
  (params (NewLook :type F%20Appearance%20Full%20Structure))
  (bind _dummy (Variables|Default|GetDummy))
  ;[1 0.312 0.302] Change Dummy's Appearance
  (Utilities|IsValid _dummy
    (:Is%20Valid
      (Default|SetNewLook _dummy NewLook))))

(event EventHideDummy
  ;[1 0.312 0.302] Hide Dummy
  (Utilities|IsValid (Variables|Default|GetDummy)
    (:Is%20Valid
      (Rendering|SetActorHiddenInGame (Variables|Default|GetDummy) true))))

(fn ConstructionScript)

(fn GetPlayerTcp
  (return (Variables|Default|GetStartTcpConnectionClient)))

(fn GetStartEventBus
  (return (Variables|Default|GetBP_Start_EventBus)))
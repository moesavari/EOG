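; BP_HttpManager sends the MMO's HTTP requests to the address and port cached in the game state, from clients and game servers.
; TreatRequest receives request objects from C++ CreateRequest, builds URL and JSON header, then calls ProcessRequest.
; It references each request until OnReadyForDeletion fires, protecting it from garbage collection.
; Clients authenticate by cookie and character ID, plus account ID in PIE; servers by password and GUID.
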(event Custom|OnRequestComplete
  (params (ThisObject :type BP%20Http%20Request%20Object%20Reference))
  ;[0.7865 0.1065 0.7201] On request completion, stop referencing the object, so it's grabbed by GC
  (Utilities|Set|Remove (Variables|Default|GetRequestObjects) ThisObject))

(event EventTreatRequest
  (params (BodyJson :type Json%20Object%20Wrapper%20Structure%20%28by%20ref%29) (Verb :type EHttpVerbs%20Enum :default "Post") (Path :type String) (CreatedRequest :type Http%20Request%20Cpp%20Object%20Reference))
  ;[0.7865 0.1065 0.7201] Treat Request. How it works:
  ; 1. Anywhere in the code you call BP_HttpManager::CreateRequest, which is a C++ function
  ; 2. The C++ function handles delegates and creates a Request object
  ; 3. Then we arrive into TreatRequest, which saves a reference to the request object, so it's protected from garbage collection
  ; 4. Then the code goes into BP_HttpRequest::ProcessRequest, where it handles the details
  ; 5. After getting a response, it tells the manager that it finished its job, so we stop referencing the request object
  (bind _asbp_http_request (Utilities|Casting|CastToBP_HttpRequest CreatedRequest))
  (Utilities|Set|Add (Variables|Default|GetRequestObjects) _asbp_http_request)
  (EventDispatchers|BindEventtoOnReadyforDeletion _asbp_http_request (delegate Custom|OnRequestComplete))
  (Default|ProcessRequest _asbp_http_request Verb (CallFunction|GetRequestUrl Path) (CallFunction|CreateHeader) BodyJson self))

(fn ConstructionScript)

(fn GetRequestUrl
  (params (Path :type String))
  (bind _tcpconn (Class|BPIGameState|GetTcpConnection(Message) (Game|GetGameState)))
  (return (Utilities|String|ToString(Text) (Utilities|Text|FormatText "http://{ip}:{port}/{path}" (Variables|/Game/MMOKit/MMO_Logic/Blueprints/WebSockets/BP_WebSockets.BP_WebSockets_C|GetCachedServerAddress _tcpconn) (Utilities|String|ToString(Integer) (Variables|/Game/MMOKit/MMO_Logic/Blueprints/WebSockets/BP_WebSockets.BP_WebSockets_C|GetServerPort _tcpconn)) Path))))

(fn CreateHeader
  ;[0.7865 0.1065 0.7201] This function generates an authentication header wheen sending http requests
  (LocalVariables|SetHeaderTemp (|MakeRequestHeader "Json"))
  (Networking|CanExecuteCosmeticEvents
    (:True
      ;[1 0.312 0.302] the player identifies himself by cookie + char id
      (bind _cookie (Class|BPIGameInstance|GetCookie(Message) (Game|GetGameInstance)))
      (Class|HttpBlueprintFunctionLibrary|AddHeader (LocalVariables|GetHeaderTemp) "Cookie" _cookie)
      (bind _chrid (Class|BPIPlayerController|GetCharId(Message) (Game|GetPlayerController 0)))
      (Class|HttpBlueprintFunctionLibrary|AddHeader (LocalVariables|GetHeaderTemp) "CharId" (Utilities|String|ToString(Integer) _chrid))
      ;[1 0.312 0.302] In PIE, it's a special case
      ; Because the login works differently, PS doesn't keep a map of <cookie, account>, so in Debug the PS will
      ; trust your supplied Account ID instead of getting it from cookie
      (bind _returnvalue (Class|MmoUtilities|InPieWorld))
      (if _returnvalue
        (bind _accountid (Class|BPIPlayerController|GetAccountId(Message) (Game|GetPlayerController 0)))
        (Class|HttpBlueprintFunctionLibrary|AddHeader (LocalVariables|GetHeaderTemp) "Account" (Utilities|String|ToString(Integer) _accountid))))
    (:False
      ;[0.4452 0.6332 1] the server identifies itself by password (to prove it's a server) + providing its guid
      (bind _password (Class|BPIGameMode|GetServerPassword(Message) (Game|GetGameMode)))
      (Class|HttpBlueprintFunctionLibrary|AddHeader (LocalVariables|GetHeaderTemp) "ServerPassword" _password)
      (bind _serverguid (Class|BPIGameState|GetServerGuid(Message) (Game|GetGameState)))
      (Class|HttpBlueprintFunctionLibrary|AddHeader (LocalVariables|GetHeaderTemp) "ServerGuid" _serverguid)))
  (return (LocalVariables|GetHeaderTemp)))
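; BP_HttpRequest wraps a single HTTP request in MMOKit, reporting success and body through a response delegate, then signaling ready for deletion.
; ProcessRequest serializes the JSON body and switches on verb, because the HttpRequest node cannot take it as a parameter; GET sends no body.
; As Unreal hides status codes, success handling treats a JSON "status" field of 400 or above as failure.
; Debug flags print headers and bodies.
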(event Custom|ProcessRequest
  (params (Verb :type EHttpVerbs%20Enum :default "Post") (Url :type String) (Header :type Http%20Header%20Structure) (JsonObject :type Json%20Object%20Wrapper%20Structure) (WorldContextObject :type Object%20Object%20Reference))
  (Variables|Default|SetRequestVerb Verb)
  (Variables|Default|SetRequestUrl Url)
  (Variables|Default|SetHeader Header)
  (bind _output_get (Variables|Default|SetRequestBodyJson JsonObject))
  (bind (_outjsonstring _returnvalue) (Class|JsonBlueprintFunctionLibrary|ToString _output_get))
  (Variables|Default|SetValidRequestBody _returnvalue)
  (Variables|Default|SetRequestBody _outjsonstring)
  (Variables|Default|SetWorld%20Context%20Object WorldContextObject)
  (switch Utilities|FlowControl|Switch|SwitchonEHttpVerbs (Variables|Default|GetRequestVerb)
    (:Post
      ;[0.7865 0.1065 0.7201] The reason for the ugly switch is because of how Unreal currently exposes Http Requests to blueprints.
      ; You can't pass the verb as a parameter, because it's a custom UK2Node that changes itself on Verb switch.
      (if (Variables|Default|GetValidRequestBody)
        (bind (_outheader _result_body) (|HttpRequest (Variables|Default|GetRequestUrl) "Post" (Variables|Default|GetHeader) (Variables|Default|GetRequestBody))
          (:then
            (CallFunction|OnRequestProcessing))
          (:On%20Success
            (CallFunction|OnRequestSuccessful _outheader _result_body))
          (:On%20Error
            (CallFunction|OnRequestFailed)))
        (else
          (Class|MmoUtilities|LogString (Variables|Default|GetWorld%20Context%20Object) "HttpRequest: JSON couldn't be turned into string! Request not sent." "Verbosity_Normal" true true "(R=1.000000,G=0.000000,B=0.027179,A=1.000000)" 5.0))))
    (:Put
      (if (Variables|Default|GetValidRequestBody)
        (bind (_outheader_2 _result_body_2) (|HttpRequest (Variables|Default|GetRequestUrl) "Put" (Variables|Default|GetHeader) (Variables|Default|GetRequestBody))
          (:then
            (CallFunction|OnRequestProcessing))
          (:On%20Success
            (CallFunction|OnRequestSuccessful _outheader_2 _result_body_2))
          (:On%20Error
            (CallFunction|OnRequestFailed)))
        (else
          (Class|MmoUtilities|LogString (Variables|Default|GetWorld%20Context%20Object) "HttpRequest: JSON couldn't be turned into string! Request not sent." "Verbosity_Normal" true true "(R=1.000000,G=0.000000,B=0.027179,A=1.000000)" 5.0))))
    (:Delete
      (if (Variables|Default|GetValidRequestBody)
        (bind (_outheader_3 _result_body_3) (|HttpRequest (Variables|Default|GetRequestUrl) "Delete" (Variables|Default|GetHeader) (Variables|Default|GetRequestBody))
          (:then
            (CallFunction|OnRequestProcessing))
          (:On%20Success
            (CallFunction|OnRequestSuccessful _outheader_3 _result_body_3))
          (:On%20Error
            (CallFunction|OnRequestFailed)))
        (else
          (Class|MmoUtilities|LogString (Variables|Default|GetWorld%20Context%20Object) "HttpRequest: JSON couldn't be turned into string! Request not sent." "Verbosity_Normal" true true "(R=1.000000,G=0.000000,B=0.027179,A=1.000000)" 5.0))))
    (:Patch
      (if (Variables|Default|GetValidRequestBody)
        (bind (_outheader_4 _result_body_4) (|HttpRequest (Variables|Default|GetRequestUrl) "Patch" (Variables|Default|GetHeader) (Variables|Default|GetRequestBody))
          (:then
            (CallFunction|OnRequestProcessing))
          (:On%20Success
            (CallFunction|OnRequestSuccessful _outheader_4 _result_body_4))
          (:On%20Error
            (CallFunction|OnRequestFailed)))
        (else
          (Class|MmoUtilities|LogString (Variables|Default|GetWorld%20Context%20Object) "HttpRequest: JSON couldn't be turned into string! Request not sent." "Verbosity_Normal" true true "(R=1.000000,G=0.000000,B=0.027179,A=1.000000)" 5.0))))
    (:Get
      ;;[0.7865 0.1065 0.7201] GET requests can't have a body, so we check that the developer didn't pass a body by mistake
      (if (<= (Utilities|String|Len (Variables|Default|GetRequestBody)) 2)
        _
        (else
          (Development|PrintString (Variables|Default|GetWorld%20Context%20Object) "Error: Your GET request had a body. The body will be ignored, it won't be sent!" true true "(R=1.000000,G=0.000000,B=0.042729,A=1.000000)" 5.0)))
      (bind (_outheader_5 _result_body_5) (|HttpRequest (Variables|Default|GetRequestUrl) "Get" (Variables|Default|GetHeader))
        (:then
          (CallFunction|OnRequestProcessing))
        (:On%20Success
          (CallFunction|OnRequestSuccessful _outheader_5 _result_body_5))
        (:On%20Error
          (CallFunction|OnRequestFailed))))))

(fn PrintHeaders
  (params (Headers :type Http%20Header%20Structure))
  (Development|PrintString (Variables|Default|GetWorld%20Context%20Object) "Headers:")
  (for _array_element (Class|HttpBlueprintFunctionLibrary|GetAllHeaders Headers)
    (Development|PrintString (Variables|Default|GetWorld%20Context%20Object) _array_element)))

(fn PrintBody
  (Development|PrintString (Variables|Default|GetWorld%20Context%20Object) (Utilities|String|Append "Response body: " (Variables|Default|GetResponseBody))))

(fn OnRequestProcessing
  (if (or (Variables|Default|GetDebugHeaders) (Variables|Default|GetDebugRequest))
    (Development|PrintString (Variables|Default|GetWorld%20Context%20Object) "HTTP Request: ")
    (Utilities|FlowControl|Sequence
      (:then_0
        (if (Variables|Default|GetDebugHeaders)
          (CallFunction|PrintHeaders (Variables|Default|GetHeader))))
      (:then_1
        (if (Variables|Default|GetDebugRequest)
          (Development|PrintString (Variables|Default|GetWorld%20Context%20Object) (Utilities|String|Append "Request body: " (Variables|Default|GetRequestBody))))))))

(fn OnRequestSuccessful
  (params (ResponseHeader :type Http%20Header%20Structure) (ResponseBody :type String))
  ;[0.7865 0.1065 0.7201] OnRequestSuccessful
  ; Request is almost always successful, because currently unreal doesn't expose Status Code
  ; We try to read status code in JSON, which C# can return, e.g. if you return Unauthorized() or NotFound()
  ; If there's any status code in JSON and it's >= 400, we'll call OnRequestFailed instead
  ; You can set DebugResponse to true to print response headers and body
  (Variables|Default|SetResponseHeader ResponseHeader)
  (Variables|Default|SetResponseBody ResponseBody)
  (Utilities|FlowControl|Sequence
    (:then_0
      (bind (_outjsonobject _returnvalue) (Class|JsonBlueprintFunctionLibrary|FromString (Variables|Default|GetResponseBody)))
      (if _returnvalue
        (bind _returnvalue_2 (Class|JsonBlueprintFunctionLibrary|HasField _outjsonobject "status"))
        (if _returnvalue_2
          (bind (_outvalue _returnvalue_3) (|GetJsonField _outjsonobject "status"))
          (if _returnvalue_3
            (bind _output_get (LocalVariables|SetStatusCode _outvalue))
            (if (>= _output_get 400)
              (Development|PrintString (Variables|Default|GetWorld%20Context%20Object) (Utilities|String|ToString(Text) (Utilities|Text|FormatText "Request ({url}) failed. Status code: {code}" (Variables|Default|GetRequestUrl) (Utilities|String|ToString(Integer) (LocalVariables|GetStatusCode)))) true true "(R=1.000000,G=0.016577,B=0.000000,A=1.000000)" 4.0)
              (CallFunction|OnRequestFailed)
              (return))))))
    (:then_1
      (if (or (Variables|Default|GetDebugHeaders) (Variables|Default|GetDebugResponse))
        (Development|PrintString (Variables|Default|GetWorld%20Context%20Object) "HTTP Response:"))
      (Utilities|FlowControl|Sequence
        (:then_0
          (if (Variables|Default|GetDebugHeaders)
            (CallFunction|PrintHeaders ResponseHeader)))
        (:then_1
          (if (Variables|Default|GetDebugResponse)
            (CallFunction|PrintBody)))
        (:then_2
          (Class|HttpRequestCpp|CallonResponseDelegate true (Variables|Default|GetResponseBody))
          (Default|CallOnReadyforDeletion self))))))

(fn OnRequestFailed
  (Class|HttpRequestCpp|CallonResponseDelegate false (Variables|Default|GetResponseBody))
  (Default|CallOnReadyforDeletion self))
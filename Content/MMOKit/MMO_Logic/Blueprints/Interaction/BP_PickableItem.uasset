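; World pickup actor holding an item and amount that a character can collect into their inventory.
; Interact is server-only: after CanInteract and a free-slot check, it adds the item and destroys the actor.
; OnRep_Item makes clients async-load the item's static or skeletal mesh through BPI_HasWorldRepresentation, falling back to a bag mesh.
; Client physics is optional, with CCD against falling through floors; the persistency-component setup is unconnected.
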(event Custom|SetMeshOnClient
  (bind _staticmesh (Variables|Default|GetStaticMesh))
  (bind _withclientphysics (Variables|Default|GetWithClientPhysics))
  (bind _withclientphysics_2 (Variables|Default|GetWithClientPhysics))
  (bind _withclientphysics_3 (Variables|Default|GetWithClientPhysics))
  (bind _staticmesh_2 (Variables|Default|GetStaticMesh))
  (bind _skeletalmesh (Variables|Default|GetSkeletalMesh))
  ;[1 0.312 0.302] On BeginPlay, the BP_PickableItem will set its mesh on Clients after async loading it
  ; Called from OnRep_Item
  (bind _loaded (|AsyncLoadPrimaryAsset (Variables|Default|GetItem))
    (:Completed
      (bind _asbpi_has_world_representation (Utilities|Casting|CastToBPI_HasWorldRepresentation _loaded)
        (:then
          (bind (_statmesh _hasstatmesh) (Default|GetStatMesh _asbpi_has_world_representation))
          (if _hasstatmesh
            (bind _object (Utilities|AsyncLoadAsset _statmesh)
              (:Completed
                (bind _asstatic_mesh (Utilities|Casting|CastToStaticMesh _object)
                  (:then
                    (Components|StaticMesh|SetStaticMesh _staticmesh_2 _asstatic_mesh)
                    (Physics|SetSimulatePhysics _staticmesh_2 _withclientphysics_2)
                    (Class|PrimitiveComponent|SetUseCCD _staticmesh_2 _withclientphysics_2 "None") ; helps to prevent mesh falling through the floor
                    (Components|SkeletalMesh|SetSkeletalMeshAsset (Variables|Default|GetSkeletalMesh) 0) ; if we're changing a static mesh to a skeletal mesh or vice versa, disable the old one
                  )
                  (:CastFailed
                    ;;[1 0.312 0.302] if no mesh is found, use the bag mesh
                    (Components|StaticMesh|SetStaticMesh _staticmesh "/Game/MMOKit/MMO_Assets/Bag/SM_Bag.SM_Bag" :!label _label)
                    (Physics|SetSimulatePhysics _staticmesh _withclientphysics)
                    (Class|PrimitiveComponent|SetUseCCD _staticmesh _withclientphysics "None")
                    (Components|SkeletalMesh|SetSkeletalMeshAsset (Variables|Default|GetSkeletalMesh) 0) ; if we're changing a static mesh to a skeletal mesh or vice versa, disable the old one
                  ))))
            (else
              (bind (_skelmesh _hasskelmesh) (Default|GetSkelMesh _asbpi_has_world_representation))
              (if _hasskelmesh
                (bind _object_2 (Utilities|AsyncLoadAsset _skelmesh)
                  (:Completed
                    (bind _asskeletal_mesh (Utilities|Casting|CastToSkeletalMesh _object_2)
                      (:then
                        (Components|SkeletalMesh|SetSkeletalMeshAsset _skeletalmesh _asskeletal_mesh)
                        (Class|SkeletalMeshComponent|SetAllBodiesSimulatePhysics _skeletalmesh _withclientphysics_3)
                        (Class|PrimitiveComponent|SetUseCCD _skeletalmesh _withclientphysics_3 "None") ; helps to prevent mesh falling through the floor
                        (Components|StaticMesh|SetStaticMesh (Variables|Default|GetStaticMesh) 0) ; if we're changing a static mesh to a skeletal mesh or vice versa, disable the old one
                      )
                      (:CastFailed
                        (goto _label)))))
                (else
                  (goto _label))))))
        (:CastFailed
          (goto _label))))))

(event EventBeginPlay
  ;[0.4452 0.6332 1] BeginPlay
)

(event EventInteract
  (params (Character :type BP%20Player%20Character%20Object%20Reference))
  (bind _bpcontroller (Default|GetBpController Character))
  (bind _inventorycomponent (Variables|/Game/MMOKit/MMO_Logic/Blueprints/BP_PlayerController.BP_PlayerController_C|GetInventoryComponent _bpcontroller))
  ;[0.7865 0.1065 0.7201] Interact
  (Networking|CanExecuteCosmeticEvents
    (:True
      ;[1 0.312 0.302] Interact: Client
      (Class|MmoUtilities|LogString "LootBag: Interact is being called on client! Must be called on server." "Verbosity_Normal" true true "(R=1.000000,G=0.000000,B=0.024480,A=1.000000)" 5.0))
    (:False
      ;[0.4452 0.6332 1] Interact: Server
      (if (not (Game|IsActorBeingDestroyed))
        (bind _can (Default|CanInteract self))
        (if _can
          (bind _hasavailable (Class|BPIStorage|GetFirstAvailableSlot(Message) _inventorycomponent))
          (if _hasavailable
            (Class|BPIStorage|AddItem(Message) _inventorycomponent (Variables|Default|GetItem) (Variables|Default|GetAmount))
            (Actor|DestroyActor)
            (else
              ;[1 0.4857 0] TODO: display "no free slots" to player
              (Class|MmoUtilities|LogString "BP_PickableItem: can't pick up - no free slots" "Verbosity_SuperVerbose"))))))))

(fn ConstructionScript)

(fn OnRepItem
  (CallFunction|SetMeshonClient))

(fn CanInteract
  (return true))
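; WoW-style interaction component that handles mouse-driven targeting, interaction and auto-attack for the player.
; Right-click release interacts with in-range objects under the cursor, or selects a character and starts a looping timer that fires the default ability at non-friendly targets.
; Left-click release selects or deselects, using accumulated look-around movement to keep the target after camera drags.
; Selection shows a decal with a dynamic material tinted by the target's reaction.
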(event Custom|OnLmbDown
  (params (Down :type Boolean))
  ;[1 0.312 0.302] On LMB Down: try selecting/deselecting
  ; Will not deselect target if we just dragged our camera
  (if Down
    (CallFunction|ResetLookAroundAccumulation) ; For explanation, see DidMouseDrag
    (else
      (bind _foundcharacter (CallFunction|GetActorUnderCursor))
      (Utilities|IsValid _foundcharacter
        (:Is%20Valid
          (CallFunction|Select _foundcharacter))
        (:Is%20Not%20Valid
          (if (not (CallFunction|DidMouseDrag))
            (CallFunction|Deselect)))))))

(event Custom|OnRmbDown
  (params (Down :type Boolean))
  ;[1 0.312 0.302] On RMB Down: try interact or try select and attack
  (if (not Down) ; Act on RMB Down
    (bind _hitactor (CallFunction|GetInteractableUnderCursor))
    (Utilities|IsValid _hitactor
      (:Is%20Valid
        (CallFunction|TryInteract))
      (:Is%20Not%20Valid
        (bind _foundcharacter (CallFunction|GetActorUnderCursor))
        (Utilities|IsValid _foundcharacter
          (:Is%20Valid
            (CallFunction|Select _foundcharacter)
            (if (CallFunction|IsValidAttackTarget _foundcharacter)
              (CallFunction|StartAutoAttack))))))))

(event Custom|Attack
  ;[1 0.312 0.302] Attack
  (bind _alive (Class|BPICharacter|IsAlive(Message) (Variables|Default|GetSelectedCharacter)))
  (if _alive
    (Class|BPIAbilities|UseAbility(Message) (Variables|Default|GetOwnerCharacter) (Variables|/Game/MMOKit/MMO_Logic/Blueprints/BP_PlayerController.BP_PlayerController_C|GetDefaultAbility (.AsBP%20Player%20Controller (Utilities|Casting|CastToBP_PlayerController (Game|GetPlayerController 0)))))
    (else
      (CallFunction|StopAutoAttack))))

(event Custom|Deselect
  ;[1 0.312 0.302] Select/Deselect
  (Utilities|FlowControl|Sequence
    (:then_0
      (Utilities|IsValid (Variables|Default|GetSelectedCharacter)
        (:Is%20Valid
          (bind _asbp_base_character (Utilities|Casting|CastToBP_BaseCharacter (Variables|Default|GetSelectedCharacter)))
          (Rendering|SetVisibility (Variables|/Game/MMOKit/MMO_Logic/Blueprints/BP_BaseCharacter.BP_BaseCharacter_C|GetSelectionDecal _asbp_base_character) false false))))
    (:then_1
      (Variables|Default|SetSelectedCharacter 0)
      (CallFunction|StopAutoAttack))))

(event Custom|Select
  (params (CharacterToSelect :type Character%20Object%20Reference))
  (bind _selectioncirclematerialinstance (Variables|Default|GetSelectionCircleMaterialInstance))
  ;[1 0.312 0.302] Select/Deselect
  (CallFunction|Deselect)
  (bind _output_get (Variables|Default|SetSelectedCharacter CharacterToSelect))
  (bind _decal (Class|BPIReaction|GetSelectionDecal(Message) _output_get))
  (Utilities|IsValid _decal
    (:Is%20Valid
      (Rendering|Components|Decal|SetDecalMaterial _decal _selectioncirclematerialinstance)
      (bind _reaction (Class|BPIReaction|GetReaction(Message) _output_get))
      (Rendering|Material|SetVectorParameterValue _selectioncirclematerialinstance "Tint" (Utilities|Select :Index _reaction :NewEnumerator0 "(R=0.129583,G=1.000000,B=0.000000,A=1.000000)" :NewEnumerator1 "(R=0.901042,G=0.803193,B=0.000000,A=1.000000)" :NewEnumerator2 "(R=1.000000,G=0.000000,B=0.000000,A=1.000000)" :NewEnumerator3 "(R=0.000000,G=0.727732,B=1.000000,A=1.000000)") :!class /Script/Engine.MaterialInstanceDynamic)
      (Rendering|SetVisibility _decal true false))))

(event Custom|StartAutoAttack
  ;[1 0.312 0.302] Start autoattack
  (bind _returnvalue (Utilities|Time|SetTimerbyEvent (delegate Custom|Attack) 0.032 true))
  (Variables|Default|SetAutoAttackTimer _returnvalue))

(event Custom|CreateSelectionMaterialInstance
  ;[1 0.312 0.302] Create material instance for selection circle
  (bind _returnvalue (Rendering|Material|CreateDynamicMaterialInstance "/Game/MMOKit/MMO_Assets/SelectionCircle/MI_SelectionDecal.MI_SelectionDecal" "None" "None" :!class /Script/Engine.KismetMaterialLibrary))
  (Variables|Default|SetSelectionCircleMaterialInstance _returnvalue))

(event Custom|StopAutoAttack
  ;[1 0.312 0.302] Stop autoattack
  (Utilities|Time|ClearandInvalidateTimerbyHandle (Variables|Default|GetAutoAttackTimer)))

(event EventBeginPlay
  ;[1 0.312 0.302] WowStyle Interaction system tries to interract
  ; on Right Mouse and not on Interact hotkey
  (|CallParentFunction)
  (bind _asbp_player_controller (Utilities|Casting|CastToBP_PlayerController (Game|GetPlayerController 0))
    (:then
      (EventDispatchers|BindEventtoOnRmbDown _asbp_player_controller (EventDispatchers|CreateEvent :!event Custom|OnRmbDown))
      (EventDispatchers|BindEventtoOnLmbDown _asbp_player_controller (EventDispatchers|CreateEvent :!event Custom|OnLmbDown))
      (EventDispatchers|BindEventtoOnLookAround _asbp_player_controller (EventDispatchers|CreateEvent :!event CollectLookAround))
      (CallFunction|CreateSelectionMaterialInstance))
    (:CastFailed
      (Class|MmoUtilities|LogString "No controller in InteractionWowStyle" "Verbosity_Normal" true true "(R=1.000000,G=0.000000,B=0.024480,A=1.000000)" 5.0))))

(event EventStartObserveInteractable
  (params (Interactable :type BPI%20Interactable%20Interface))
  ;[1 0.312 0.302] Start Observe Interactable: observe a lootable object
  (|CallParentFunction Interactable)
  (bind _asbp_player_controller (Utilities|Casting|CastToBP_PlayerController (Game|GetPlayerController 0)))
  (Default|ForceInventory _asbp_player_controller true))

(event EventTryInteract
  (bind _returnvalue (Game|GetPlayerCharacter 0))
  ;[1 0.312 0.302] Try Interact: search for objects under mouse cursor
  (|CallParentFunction)
  (bind _hitactor (CallFunction|GetInteractableUnderCursor))
  (Utilities|IsValid _hitactor
    (:Is%20Valid
      (bind _asbpi_interactable (Utilities|Casting|CastToBPI_Interactable _hitactor))
      (bind _can (Default|CanInteract _asbpi_interactable))
      (if _can
        (Utilities|IsValid _returnvalue
          (:Is%20Valid
            (if (<= (Transformation|GetSquaredDistanceTo _returnvalue _hitactor) (Math|Float|Square (Variables|Default|GetInteractDistance)))
              (Default|StopInteractonServer (Variables|Default|GetOwnerCharacter) (Variables|Default|GetCurrentInteractable))
              (Variables|Default|SetCurrentInteractable _asbpi_interactable)
              (Default|InteractonServer (Variables|Default|GetOwnerCharacter) _asbpi_interactable)
              (else
                (Default|CallOnInteractionFailed "NewEnumerator0")))))
        (else
          (Default|CallOnInteractionFailed "NewEnumerator1"))))))

(event EventEndPlay
  (params (EndPlayReason :type EEndPlayReason%20Enum :default "Destroyed"))
  ;[1 0.312 0.302] WowStyle Interaction system tries to interract
  ; on Right Mouse and not on Interact hotkey
  (CallFunction|Deselect))

(fn GetActorUnderCursor
  (bind _returnvalue (Game|GetPlayerController 0))
  (bind _actorchannels (Variables|Default|GetActorChannels))
  (bind (_hitresult _returnvalue_2) (Class|PlayerController|GetHitResultUnderCursorforObjects _returnvalue _actorchannels false))
  (bind _hitactor (Collision|BreakHitResult _hitresult))
  (Utilities|IsValid _returnvalue
    (:Is%20Valid
      (if _returnvalue_2
        (Utilities|IsValid _hitactor
          (:Is%20Valid
            (bind _ascharacter (Utilities|Casting|CastToCharacter _hitactor)
              (:then
                (if (!= (Game|GetPlayerCharacter 0) _hitactor)
                  (return _ascharacter)
                  (else
                    _)))
              (:CastFailed
                _)))
          (:Is%20Not%20Valid
            _)))
      (return 0))))

(fn GetInteractableUnderCursor
  (bind _returnvalue (Game|GetPlayerController 0))
  (bind _interactablechannels (Variables|Default|GetInteractableChannels))
  (bind (_hitresult _returnvalue_2) (Class|PlayerController|GetHitResultUnderCursorforObjects _returnvalue _interactablechannels false))
  (bind _hitactor (Collision|BreakHitResult _hitresult))
  ;[1 0.312 0.302] Only searches for interactable objects, not characters
  (Utilities|IsValid _returnvalue
    (:Is%20Valid
      (if _returnvalue_2
        (Utilities|IsValid _hitactor
          (:Is%20Valid
            (return _hitactor))
          (:Is%20Not%20Valid
            _))))
    (:Is%20Not%20Valid
      _))
  (return 0))

(fn ResetLookAroundAccumulation
  (Variables|Default|SetMouseMovementCollected ""))

(fn DidMouseDrag
  ;[1 0.312 0.302] When LMB UP is triggered, we need to determine whether we need to deselect current target or not
  ; It depends on whether we just dragged our camera with LMB
  ; If we did drag, then we don't need to deselect current target
  ; The way we determine that is as follows:
  ; - on LMB DOWN, we reset MouseMovementCollected (2D Vector) to zero
  ; - on IA_LookAround, we collect any movement the mouse does
  ; - on LMB UP, we check how much movement the mouse has done between Down and Up, by a tolerance. This shows us if the mouse just dragged (and by extension, if the camera dragged)
  (return (not (Class|KismetMathLibrary|IsNearlyZero2D (Variables|Default|GetMouseMovementCollected) 0.1))))

(fn CollectLookAround
  (params (CollectVector :type Vector%202D%20Structure))
  ;[1 0.312 0.302] For explanation, see DidMouseDrag
  (Variables|Default|SetMouseMovementCollected (+ (Variables|Default|GetMouseMovementCollected) CollectVector)))

(fn IsValidAttackTarget
  (params (Char :type Character%20Object%20Reference))
  (bind _reaction (Class|BPIReaction|GetReaction(Message) Char))
  (if (or (Utilities|Enum|Equal(Enum) _reaction "NewEnumerator0") (Utilities|Enum|Equal(Enum) _reaction "NewEnumerator3"))
    (return false)
    (else
      (return true))))
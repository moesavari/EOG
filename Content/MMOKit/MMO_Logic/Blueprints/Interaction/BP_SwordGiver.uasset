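; BP_SwordGiver is an interactable that awards one item, presumably a sword, to the interacting character's inventory.
; Interact uses CanExecuteCosmeticEvents as a server guard, logging a redirect to InteractOnServer when cosmetic events can run.
; Otherwise it checks CanInteract, which always returns true, then calls AddItemMessage on the InventoryComponent of the character's controller.
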(event EventInteract
  (params (Character :type BP%20Player%20Character%20Object%20Reference))
  (Networking|CanExecuteCosmeticEvents
    (:True
      (Class|MmoUtilities|LogString "You've called Interact on an Interactable CLIENT-SIDE! Call BP_Character->InteractOnServer() instead!" "Verbosity_Normal" true true "(R=1.000000,G=0.000000,B=0.024480,A=1.000000)" 5.0))
    (:False
      (bind _can (CallFunction|CanInteract self))
      (if _can
        (Class|BPIStorage|AddItem(Message) (Variables|/Game/MMOKit/MMO_Logic/Blueprints/BP_PlayerController.BP_PlayerController_C|GetInventoryComponent (Default|GetBpController Character)) "Equipment:Sword_01" 1)
        (Class|MmoUtilities|LogString "Container awards you an item!" "Verbosity_SuperVerbose")))))

(fn ConstructionScript)

(fn CanInteract
  (return true))
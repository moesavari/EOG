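; Point-and-click interaction logic for the player that turns targets reached by BP_PointNClickCameraComponent into attacks or interactions.
; BeginPlay retries each tick until that component exists, then binds to its reached-target event.
; Characters passing the reaction check are attacked with the controller's default ability; interactables go through alive, CanInteract and distance checks before InteractOnServer.
; A cursor trace helper sets AttackTarget, including world geometry to block selection through walls.
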(event Custom|OnTargetReached
  (params (Target :type Actor%20Object%20Reference))
  ;[1 0.312 0.302] On Target Reached (emitted by BP_PointNClickCameraComponent)
  (bind _ascharacter (Utilities|Casting|CastToCharacter Target)
    (:then
      (if (CallFunction|IsValidAttackTarget _ascharacter)
        (Variables|Default|SetAttackTarget _ascharacter)
        (CallFunction|Attack)))
    (:CastFailed
      (Utilities|Casting|CastToBPI_Interactable Target)
      (Variables|Default|SetNewInteractable Target)
      (CallFunction|TryInteract))))

(event Custom|Attack
  ;[1 0.312 0.302] Attack
  (Utilities|IsValid (Variables|Default|GetAttackTarget)
    (:Is%20Valid
      (bind _alive (Class|BPICharacter|IsAlive(Message) (Variables|Default|GetAttackTarget)))
      (if _alive
        (Class|BPIAbilities|UseAbility(Message) (Variables|Default|GetOwnerCharacter) (Variables|/Game/MMOKit/MMO_Logic/Blueprints/BP_PlayerController.BP_PlayerController_C|GetDefaultAbility (.AsBP%20Player%20Controller (Utilities|Casting|CastToBP_PlayerController (Game|GetPlayerController 0)))))
        (else
          (Variables|Default|SetAttackTarget 0))))))

(event EventBeginPlay
  (bind _ownercharacter (Variables|Default|GetOwnerCharacter))
  (bind _returnvalue (Actor|GetComponentbyClass _ownercharacter "/Game/MMOKit/MMO_Logic/Blueprints/Camera/BP_PointNClickCameraComponent.BP_PointNClickCameraComponent_C"))
  ;[1 0.312 0.302] BeginPlay
  (|CallParentFunction)
  (bind _asbp_player_controller (Utilities|Casting|CastToBP_PlayerController (Game|GetPlayerController 0))
    (:then
      (Variables|Default|SetOwnerController _asbp_player_controller)
      (Utilities|IsValid _returnvalue :!label _label
        (:Is%20Valid
          (EventDispatchers|BindEventtoReachedTarget _returnvalue (EventDispatchers|CreateEvent :!event Custom|OnTargetReached)))
        (:Is%20Not%20Valid
          (Utilities|FlowControl|DelayUntilNextTick)
          (goto _label))))
    (:CastFailed
      (Class|MmoUtilities|LogString "No controller in InteractionPointNClick" "Verbosity_Normal" true true "(R=1.000000,G=0.000000,B=0.024480,A=1.000000)" 5.0))))

(event EventStartObserveInteractable
  (params (Interactable :type BPI%20Interactable%20Interface))
  ;[1 0.312 0.302] Start Observe Interactable: observe a lootable object
  (|CallParentFunction Interactable)
  (bind _asbp_player_controller (Utilities|Casting|CastToBP_PlayerController (Game|GetPlayerController 0)))
  (Default|ForceInventory _asbp_player_controller true))

(event EventTryInteract
  (bind _returnvalue (Game|GetPlayerCharacter 0))
  (bind _newinteractable (Variables|Default|GetNewInteractable))
  ;[1 0.312 0.302] Try Interact: search for objects under mouse cursor
  (|CallParentFunction)
  (bind _alive (Default|IsAlive (Variables|Default|GetOwnerCharacter)))
  (if _alive
    (bind _asbpi_interactable (Utilities|Casting|CastToBPI_Interactable _newinteractable))
    (bind _can (Default|CanInteract _asbpi_interactable))
    (if _can
      (Utilities|IsValid _returnvalue
        (:Is%20Valid
          (if (<= (Transformation|GetSquaredDistanceTo _returnvalue _newinteractable) (Math|Float|Square (Variables|Default|GetInteractDistance)))
            (Default|StopInteractonServer (Variables|Default|GetOwnerCharacter) (Variables|Default|GetCurrentInteractable))
            (Variables|Default|SetCurrentInteractable _asbpi_interactable)
            (Default|InteractonServer (Variables|Default|GetOwnerCharacter) _asbpi_interactable)
            (else
              (Default|CallOnInteractionFailed "NewEnumerator0")))))
      (else
        (Default|CallOnInteractionFailed "NewEnumerator1" :!label _label)))
    (else
      (goto _label))))

(fn GetAnythingUnderCursor
  (bind _array (Utilities|Array|MakeArray "ObjectTypeQuery7" "ObjectTypeQuery1" "ObjectTypeQuery2"))
  (bind _array_2 (Utilities|Array|MakeArray "ObjectTypeQuery3" "ObjectTypeQuery4" "ObjectTypeQuery1" "ObjectTypeQuery2"))
  (bind _ownercontroller (Variables|Default|GetOwnerController))
  (bind _ownercharacter (Variables|Default|GetOwnerCharacter))
  (bind _ownercontroller_2 (Variables|Default|GetOwnerController))
  (bind _ownercharacter_2 (Variables|Default|GetOwnerCharacter))
  (bind _array_3 (Utilities|Array|MakeArray _ownercharacter))
  (bind _array_4 (Utilities|Array|MakeArray _ownercharacter_2))
  (bind (_hitresult _returnvalue) (Class|PlayerControllerCpp|GetHitResultUnderCursorforObjectswithIgnore _ownercontroller _array_2 true _array_3))
  (bind (_hitresult_2 _returnvalue_2) (Class|PlayerControllerCpp|GetHitResultUnderCursorforObjectswithIgnore _ownercontroller_2 _array true _array_4))
  (Utilities|FlowControl|Sequence
    (:then_0
      (if _returnvalue
        (LocalVariables|SetHitResult _hitresult)
        (bind _ascharacter (Utilities|Casting|CastToCharacter (.HitActor (Collision|BreakHitResult (LocalVariables|GetHitResult))))
          (:then
            (bind _reaction (Class|BPIReaction|GetReaction(Message) _ascharacter))
            (if (or (Utilities|Enum|Equal(Enum) _reaction "NewEnumerator2") (Utilities|Enum|Equal(Enum) _reaction "NewEnumerator1")) ; If friendly character, reset to not attack target
              (Variables|Default|SetAttackTarget _ascharacter)
              (return)
              (else
                (Variables|Default|SetAttackTarget 0) ; Reset AttackTarget to null
              )))
          (:CastFailed
            (Variables|Default|SetAttackTarget 0) ; Reset AttackTarget to null
          ))
        (else
          (Variables|Default|SetAttackTarget 0) ; Reset AttackTarget to null
        )))
    (:then_1
      (if _returnvalue_2
        (bind _output_get (LocalVariables|SetHitResult _hitresult_2))
        (bind _can (Class|BPIInteractable|CanInteract(Message) (.HitActor (Collision|BreakHitResult _output_get))))
        (if _can
          _)))))

(fn IsValidAttackTarget
  (params (Char :type Character%20Object%20Reference))
  (bind _reaction (Class|BPIReaction|GetReaction(Message) Char))
  (if (or (Utilities|Enum|Equal(Enum) _reaction "NewEnumerator0") (Utilities|Enum|Equal(Enum) _reaction "NewEnumerator3"))
    (return false)
    (else
      (return true))))
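; BP_LootBag is an interactable loot container that lets multiple characters view and take its items.
; The server keeps parallel item and amount arrays plus a set of observing characters, logging misuse from clients.
; Looting checks the item at the given index and a free inventory slot, then transfers a clamped amount.
; Observers receive updated contents, or are closed out when the bag empties and destroys itself after a delay.
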(event Custom|OnLootedCompletely
  ;[0.4452 0.6332 1] OnLootedCompletely
  (bind _result (Utilities|Set|ToArray (Variables|Default|GetObservers)))
  (for _array_element _result
    (Default|StopInteractClient _array_element))
  (Utilities|Set|Clear (Variables|Default|GetObservers))
  (Utilities|FlowControl|Delay 2.0)
  (Actor|DestroyActor))

(event Custom|SendLootToObservers
  ;[0.4452 0.6332 1] Send Loot to Observers
  (bind _result (Utilities|Set|ToArray (Variables|Default|GetObservers)))
  (for _array_element _result
    (Default|ReceiveLootClient _array_element (Variables|Default|GetLoot) (Variables|Default|GetLootAmounts))))

(event EventInteract
  (params (Character :type BP%20Player%20Character%20Object%20Reference))
  ;[0.4452 0.6332 1] Interact (server) - open bag
  (Networking|CanExecuteCosmeticEvents
    (:True
      (Class|MmoUtilities|LogString "LootBag: Interact is being called on client! Must be called on server." "Verbosity_Normal" true true "(R=1.000000,G=0.000000,B=0.024480,A=1.000000)" 5.0))
    (:False
      (Utilities|Set|Add (Variables|Default|GetObservers) Character)
      (Default|ObserveInteractable Character self)
      (Default|ReceiveLootClient Character (Variables|Default|GetLoot) (Variables|Default|GetLootAmounts)))))

(event EventStopInteract
  (params (Character :type BP%20Player%20Character%20Object%20Reference))
  ;[0.4452 0.6332 1] Stop Interact (server) - close bag
  (Networking|CanExecuteCosmeticEvents
    (:True
      (Class|MmoUtilities|LogString "LootBag: StopInteract is being called on client! Must be called on server." "Verbosity_Normal" true true "(R=1.000000,G=0.000000,B=0.024480,A=1.000000)" 5.0))
    (:False
      (Utilities|Set|Remove (Variables|Default|GetObservers) Character))))

(event EventLootItem
  (params (Item :type Primary%20Asset%20Id%20Structure) (Id :type Integer) (AmountOptional :type Integer) (Looter :type BP%20Player%20Controller%20Object%20Reference))
  (bind _returnvalue (> AmountOptional 0))
  (bind _inventorycomponent (Variables|/Game/MMOKit/MMO_Logic/Blueprints/BP_PlayerController.BP_PlayerController_C|GetInventoryComponent Looter))
  (bind _loot (Variables|Default|GetLoot))
  (bind _lootamounts (Variables|Default|GetLootAmounts))
  (bind _lootamounts_2 (Variables|Default|GetLootAmounts))
  (bind _output (Utilities|Array|Get(acopy) _loot Id))
  (bind _output_2 (Utilities|Array|Get(acopy) _lootamounts Id))
  (bind _output_3 (Utilities|Array|Get(acopy) _lootamounts_2 Id))
  (bind _returnvalue_2 (Math|Integer|Min(Integer) _output_2 AmountOptional))
  (bind _returnvalue_3 (Math|Integer|SelectInt _returnvalue_2 1 _returnvalue))
  (bind _returnvalue_4 (- _output_3 _returnvalue_3))
  ;[0.4452 0.6332 1] Loot Item (server)
  ;;[1 1 1] Check that the item that the player wants to loot is still here
  (Networking|CanExecuteCosmeticEvents
    (:True
      (Class|MmoUtilities|LogString "LootBag: Loot Item must be called on server!" "Verbosity_Normal" true true "(R=1.000000,G=0.000000,B=0.024480,A=1.000000)" 5.0))
    (:False
      (if (== _output Item)
        ;;[1 1 1] check that character has a free slot
        (bind _hasavailable (Default|GetFirstAvailableSlot _inventorycomponent))
        (if _hasavailable
          (Utilities|FlowControl|Sequence
            (:then_0
              (Class|BPIStorage|AddItem(Message) _inventorycomponent _output _returnvalue_3)
              (|SetBy-RefVar _output_3 _returnvalue_4)
              (if (< _returnvalue_4 1)
                (Utilities|Array|RemoveIndex (Variables|Default|GetLoot) Id)
                (Utilities|Array|RemoveIndex (Variables|Default|GetLootAmounts) Id)))
            (:then_1
              (if (== (Utilities|Array|Length (Variables|Default|GetLoot)) 0)
                (CallFunction|OnLootedCompletely)
                (else
                  (CallFunction|SendLoottoObservers)))))
          (else
            ;[1 0.4857 0] TODO: display "no free slots" to player
            (Class|MmoUtilities|LogString "BP_LootBag: can't pick up - no free slots" "Verbosity_SuperVerbose")))))))

(event EventAddLoot
  (params (Item :type Primary%20Asset%20Id%20Structure) (Amount :type Integer))
  ;[0.4452 0.6332 1] Add Loot
  (Networking|CanExecuteCosmeticEvents
    (:True
      (Class|MmoUtilities|LogString "LootBag: Add Loot must only be called on server!" "Verbosity_Normal" true true "(R=1.000000,G=0.000000,B=0.024480,A=1.000000)" 5.0))
    (:False
      (Utilities|Array|Add (Variables|Default|GetLoot) Item)
      (Utilities|Array|Add (Variables|Default|GetLootAmounts) Amount))))

(fn ConstructionScript)

(fn CanInteract
  (return true))
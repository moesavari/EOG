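; Base class for the MMO player interaction system, tracking the interactable the local player observes, such as loot.
; TryInteract is an empty hook for child classes, bound to different events depending on camera type.
; Observe, stop and loot-received events update state where needed and broadcast to listeners.
; Tick compares squared distance to the observed actor and has the player character stop interacting when it exceeds the limit.
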(event Custom|TryInteract
  ;[1 1 1] To override in child classes
  ; It's bound to different events depending on camera type
)

(event Custom|StopInteract
  ;[1 1 1] Observe loot / stop observing
  (Variables|Default|SetObservedInteractable 0)
  (Default|CallOnInteractionStopped)
  (Class|MmoUtilities|LogString "Stop Interact" "Verbosity_SuperVerbose"))

(event Custom|StartObserveInteractable
  (params (Interactable :type BPI%20Interactable%20Interface))
  ;[1 1 1] Observe loot / stop observing
  (bind _output_get (Variables|Default|SetObservedInteractable Interactable))
  (Default|CallOnStartObserve _output_get))

(event Custom|LootReceived
  (params (Items :type Array%20of%20Primary%20Asset%20Id%20Structures) (Amounts :type Array%20of%20Integers))
  ;[1 1 1] Observe loot / stop observing
  (Default|CallOnReceivedLoot Items Amounts))

(event EventTick
  (params (DeltaSeconds :type Float%20%28single-precision%29))
  (bind _observedinteractable (Variables|Default|GetObservedInteractable))
  (bind _returnvalue (Utilities|ToObject(Interface) _observedinteractable))
  ;[1 1 1] Break interaction if exceeding ObserveDistanceSquared
  (Utilities|IsValid _returnvalue
    (:Is%20Valid
      (bind _asactor (Utilities|Casting|CastToActor _returnvalue))
      (if (> (Transformation|GetSquaredDistanceTo (Variables|Default|GetOwnerCharacter) _asactor) (Variables|Default|GetObserveDistanceSquared))
        (Default|StopInteractLocal (Variables|Default|GetOwnerCharacter) (Variables|Default|GetObservedInteractable))))))

(event EventBeginPlay
  ;[1 1 1] BeginPlay
  (bind _asbp_player_character (Utilities|Casting|CastToBP_PlayerCharacter (Game|GetPlayerCharacter 0)))
  (Variables|Default|SetOwnerCharacter _asbp_player_character))
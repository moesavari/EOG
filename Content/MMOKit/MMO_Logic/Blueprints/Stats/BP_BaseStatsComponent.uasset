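; Base stats component in the MMO kit that tracks an actor's HP and handles damage, healing, death and resurrection.
; HP changes are clamped and broadcast through RepNotifies, with DieFastOwner zeroing HP ahead of normal replication and death or resurrection messages sent to the owner.
; Buff effects are summed by type into a map, where an immortality effect holds lethal damage at 1 HP.
; Name functions are stubs for child classes.
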(event Custom|EmitNameUpdated)

(event Custom|EmitHpUpdated
  ;[1 0.312 0.302] Emit Hp Updated
  (Default|CallOnHpUpdated (Variables|Default|GetCurHp) (Variables|Default|GetMaxHp)))

(event Custom|TakeDamage
  (params (Attacker :type Character%20Object%20Reference) (Dmg :type Integer))
  ;[0.4452 0.6332 1] Take dmg (server)
  (if (CallFunction|IsAlive)
    (Variables|Default|SetCurHp (Math|Integer|Clamp(Integer) (- (Variables|Default|GetCurHp) Dmg) 0 (Variables|Default|GetMaxHp)))
    (if (not (CallFunction|IsAlive))
      (bind _found (CallFunction|StatsHaveEffect "NewEnumerator5")) ; if under immortality, prevent death and set hp to 1
      (if _found
        (Variables|Default|SetCurHp 1)
        (else
          (CallFunction|DieFastOwner)
          (Class|BPICharacter|Die(Message) (Components|GetOwner) Attacker))))))

(event Custom|HealHp
  (params (Healer :type Character%20Object%20Reference) (HpHealed :type Integer))
  (if (CallFunction|IsAlive)
    (Variables|Default|SetCurHp (Math|Integer|Clamp(Integer) (+ (Variables|Default|GetCurHp) HpHealed) 0 (Variables|Default|GetMaxHp)))))

(event Custom|Resurrect
  ;[0.4452 0.6332 1] Resurrect
  (if (not (CallFunction|IsAlive))
    (Variables|Default|SetCurHp (Variables|Default|GetMaxHp))
    (if (CallFunction|IsAlive)
      (Class|BPICharacter|Resurrect(Message) (Components|GetOwner)))))

(event Custom|DieFastOwner
  ;[1 0.312 0.302] Sets our character's HP faster than a normal replication would
  (Variables|Default|SetCurHp 0))

(fn OnRepCurHp
  (CallFunction|EmitHpUpdated))

(fn OnRepMaxHp
  (CallFunction|EmitHpUpdated))

(fn GetName
  (return "NoName"))

(fn IsAlive
  (return (> (Variables|Default|GetCurHp) 0)))

(fn StatsHaveEffect
  (params (Effect :type EBuffEffectType%20Enum :default "NewEnumerator0"))
  (bind _buffstatuseffects (Variables|Default|GetBuffStatusEffects))
  (bind (_value _returnvalue) (Utilities|Map|Find _buffstatuseffects Effect))
  ;[1 0.4857 0] This is the most basic implementation.
  ; Ideally you'd have native Effects in one map, from gear in another, from buffs in another, etc...
  (if _returnvalue
    (return true _value)
    (else
      (return false 0.0))))

(fn RecalculateBuffStatusEffects
  (params (Effects :type Array%20of%20F%20Buff%20Effect%20Data%20Structures))
  (bind _buffstatuseffects (Variables|Default|GetBuffStatusEffects))
  (Utilities|Map|Clear (Variables|Default|GetBuffStatusEffects))
  (for _array_element Effects
    (bind _output_get (LocalVariables|SetBuffEffect _array_element))
    (if (.ReturnValue (Utilities|Map|Find (Variables|Default|GetBuffStatusEffects) (.Effect (Utilities|Struct|BreakFBuffEffectData _output_get))))
      (LocalVariables|SetValueBeforeAdd (.Value (Utilities|Map|Find (Variables|Default|GetBuffStatusEffects) (.Effect (Utilities|Struct|BreakFBuffEffectData _output_get)))))
      (Utilities|Map|Remove _buffstatuseffects (.Effect (Utilities|Struct|BreakFBuffEffectData (LocalVariables|GetBuffEffect))))
      (Utilities|Map|Add _buffstatuseffects (.Effect (Utilities|Struct|BreakFBuffEffectData (LocalVariables|GetBuffEffect))) (+ (LocalVariables|GetValueBeforeAdd) (.Value (Utilities|Struct|BreakFBuffEffectData (LocalVariables|GetBuffEffect)))))
      (else
        (Utilities|Map|Add (Variables|Default|GetBuffStatusEffects) (.Effect (Utilities|Struct|BreakFBuffEffectData (LocalVariables|GetBuffEffect))) (.Value (Utilities|Struct|BreakFBuffEffectData (LocalVariables|GetBuffEffect))))))))

(fn AddBuffStatusEffects
  (params (BuffEffects :type Array%20of%20F%20Buff%20Effect%20Data%20Structures))
  (for _array_element BuffEffects
    (if (.ReturnValue (Utilities|Map|Find (Variables|Default|GetBuffStatusEffects) (.Effect (Utilities|Struct|BreakFBuffEffectData _array_element))))
      (bind _output_get (LocalVariables|SetValueBefore (.Value (Utilities|Map|Find (Variables|Default|GetBuffStatusEffects) (.Effect (Utilities|Struct|BreakFBuffEffectData _array_element))))))
      (Utilities|Map|Remove (Variables|Default|GetBuffStatusEffects) (.Effect (Utilities|Struct|BreakFBuffEffectData _array_element)))
      (Utilities|Map|Add (Variables|Default|GetBuffStatusEffects) (.Effect (Utilities|Struct|BreakFBuffEffectData _array_element)) (+ _output_get (.Value (Utilities|Struct|BreakFBuffEffectData _array_element))))
      (else
        (Utilities|Map|Add (Variables|Default|GetBuffStatusEffects) (.Effect (Utilities|Struct|BreakFBuffEffectData _array_element)) (.Value (Utilities|Struct|BreakFBuffEffectData _array_element)))))))
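; Server-side buff component for characters that applies, ticks, expires, cancels and serializes buffs, and recreates saved ones on initialization.
; Active buffs are keyed by GUID and timed by BuffsSubsystem, driving each asset's BuffDynamics and BuffTriggers and updating StatsComponent effects.
; Displayable buffs are mirrored into replicated proxies that notify the local player's UI through OnRep.
; Death cancels buffs flagged RemoveOnDeath, and EndPlay stops ticking.
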(event Custom|InitializeBuffsComponent
  (params (SerializedBuffs :type Array%20of%20F%20Serialized%20Buff%20Structures))
  ;[0.4452 0.6332 1] On Initialize - called from BP_PlayerCharacter's Construct
  ; 1. Sign up to OnDeath to remove all buffs
  ; 2. Replicate all buffs
  (Variables|Default|SetInBuffs SerializedBuffs)
  (bind _ascharacter (Utilities|Casting|CastToCharacter (Components|GetOwner)))
  (Variables|Default|SetOwnerCharacter _ascharacter)
  (Networking|CanExecuteCosmeticEvents
    (:False
      (bind _charactereventbus (Class|BPICharacter|GetCharacterEventBus(Message) (Variables|Default|GetOwnerCharacter)))
      (EventDispatchers|BindEventtoOnDeath _charactereventbus (EventDispatchers|CreateEvent :!event RemoveBuffsonDeath))
      (CallFunction|RecreateBuffsfromDb (Variables|Default|GetInBuffs))
      (bind _statscomp (Class|BPIStats|GetStatsComponent(Message) (Variables|Default|GetOwnerCharacter)))
      (bind _effects (CallFunction|GetActiveBuffEffects))
      (Default|RecalculateBuffStatusEffects _statscomp _effects)
      (CallFunction|AddAllBuffstoReplication))))

(event Custom|RequestRemoveBuff
  (params (Guid :type Guid%20Structure))
  (bind _activebuffs (Variables|Default|GetActiveBuffs))
  (bind (_value _returnvalue) (Utilities|Map|Find _activebuffs Guid))
  ;[0.4452 0.6332 1] Request Remove Buff (right click on buff)
  (if _returnvalue
    (bind _asbuff_asset (Utilities|Casting|CastToBuffAsset (Class|KismetSystemLibrary|GetObjectfromPrimaryAssetId (Utilities|Struct|BreakFActiveBuff _value))))
    (if (Variables|/Game/MMOKit/MMO_Logic/Blueprints/DataAssetTypes/BuffAsset.BuffAsset_C|GetAllowSelfRemove _asbuff_asset)
      (CallFunction|CancelBuff Guid))))

(event Custom|DispatchBuffsUpdated
  (Default|CallOnBuffsUpdated (Variables|Default|GetReplicatedBuffProxies)))

(event EventEndPlay
  (params (EndPlayReason :type EEndPlayReason%20Enum :default "Destroyed"))
  ;[0.4452 0.6332 1] When character disconnects, stop ticking his buffs
  (Networking|CanExecuteCosmeticEvents
    (:False
      (if (or (Utilities|Enum|Equal(Enum) EndPlayReason "Destroyed") (Utilities|Enum|Equal(Enum) EndPlayReason "Quit"))
        (bind _keys (Utilities|Map|Keys (Variables|Default|GetActiveBuffs)))
        (for _array_element _keys
          (Class|BuffsSubsystem|StopTickingBuff (Subsystems|GetBuffsSubsystem) _array_element))))))

(fn ApplyBuff
  (params (BuffAsset :type Primary%20Asset%20Id%20Structure) (AbilityAsset :type Primary%20Asset%20Id%20Structure) (Instigator :type Character%20Object%20Reference))
  (bind _ascharacter (Utilities|Casting|CastToCharacter (Components|GetOwner))
    (:then
      (LocalVariables|SetVictim _ascharacter)
      (bind _asbuff_asset (Utilities|Casting|CastToBuffAsset (Class|KismetSystemLibrary|GetObjectfromPrimaryAssetId BuffAsset))
        (:then
          (LocalVariables|SetBuffAssetObject _asbuff_asset)
          (Utilities|FlowControl|Sequence
            (:then_0
              (bind _statscomp (Class|BPIStats|GetStatsComponent(Message) Instigator))
              (Utilities|IsValid _statscomp
                (:Is%20Valid
                  (bind _creaturename (Default|GetName _statscomp))
                  (bind _isplayer (Class|BPICharacter|IsPlayerCharacter(Message) Instigator))
                  (LocalVariables|SetInstigatorInfo (Utilities|Struct|MakeFBuffInstigatorInfo (Utilities|String|ToString(Text) _creaturename) _isplayer)))))
            (:then_1
              (bind _duration (Default|GetDuration (LocalVariables|GetBuffAssetObject) Instigator))
              (LocalVariables|SetBuffDuration _duration)
              (bind _effects (Default|GetEffects (LocalVariables|GetBuffAssetObject) Instigator))
              (LocalVariables|SetBuffEffects _effects)
              (LocalVariables|SetBuffGuid (Guid|NewGuid))
              (if (Utilities|IsValidClass (Variables|/Game/MMOKit/MMO_Logic/Blueprints/DataAssetTypes/BuffAsset.BuffAsset_C|GetBuffTriggers (LocalVariables|GetBuffAssetObject)))
                (bind _returnvalue (Game|ConstructObjectfromClass (Variables|/Game/MMOKit/MMO_Logic/Blueprints/DataAssetTypes/BuffAsset.BuffAsset_C|GetBuffTriggers (LocalVariables|GetBuffAssetObject))))
                (bind _output_get (LocalVariables|SetBuffTriggersObject _returnvalue))
                (Default|SignUptoEvents _output_get (LocalVariables|GetVictim) (LocalVariables|GetBuffEffects)))
              (Class|MmoUtilities|LogString (Utilities|String|Append "Adding buff: " (Guid|ToString(Guid) (LocalVariables|GetBuffGuid))) "Verbosity_SuperVerbose"))
            (:then_2
              (bind _output_get_2 (LocalVariables|SetAppliedBuff (Utilities|Struct|MakeFActiveBuff (LocalVariables|GetBuffEffects) BuffAsset AbilityAsset (LocalVariables|GetInstigatorInfo) (LocalVariables|GetBuffDuration) (GameState|GetServerWorldTimeSeconds (Game|GetGameState)) (LocalVariables|GetBuffTriggersObject))))
              (Utilities|Map|Add (Variables|Default|GetActiveBuffs) (LocalVariables|GetBuffGuid) _output_get_2))
            (:then_3
              (Utilities|IsValid (LocalVariables|GetBuffAssetObject)
                (:Is%20Valid
                  (Utilities|IsValid (Variables|/Script/MMOKitCode.BuffAssetCpp|GetBuffDynamics (LocalVariables|GetBuffAssetObject))
                    (:Is%20Valid
                      (bind _asbuff_dynamics (Utilities|Casting|CastToBuffDynamics (Variables|/Script/MMOKitCode.BuffAssetCpp|GetBuffDynamics (LocalVariables|GetBuffAssetObject))))
                      (Default|OnBuffApply _asbuff_dynamics (LocalVariables|GetVictim) (LocalVariables|GetAppliedBuff)))))))
            (:then_4
              (Class|BuffsSubsystem|RegisterBuff (Subsystems|GetBuffsSubsystem) (LocalVariables|GetBuffGuid) (LocalVariables|GetBuffDuration) (EventDispatchers|CreateEvent :!event OnBuffExpired)) ; Registering the buff with the Subsystem will allow the buff to expire after its Duration has run out
            )
            (:then_5
              (if (and (Variables|/Game/MMOKit/MMO_Logic/Blueprints/DataAssetTypes/BuffAsset.BuffAsset_C|GetTicks (LocalVariables|GetBuffAssetObject)) (!= (LocalVariables|GetBuffDuration) 0.0))
                (Class|BuffsSubsystem|StartTickingBuff (Subsystems|GetBuffsSubsystem) (LocalVariables|GetBuffGuid) 0.0 (Variables|/Game/MMOKit/MMO_Logic/Blueprints/DataAssetTypes/BuffAsset.BuffAsset_C|GetTickFrequency (LocalVariables|GetBuffAssetObject)) (EventDispatchers|CreateEvent :!event OnBuffTicks))))
            (:then_6
              (if (and (Variables|/Game/MMOKit/MMO_Logic/Blueprints/DataAssetTypes/BuffAsset.BuffAsset_C|GetDisplayIcon (LocalVariables|GetBuffAssetObject)) (!= (LocalVariables|GetBuffDuration) 0.0))
                (CallFunction|AddBufftoReplication (LocalVariables|GetBuffGuid))))
            (:then_7
              (if (Utilities|Array|IsNotEmpty (LocalVariables|GetBuffEffects))
                (bind _statscomp_2 (Class|BPIStats|GetStatsComponent(Message) (LocalVariables|GetVictim)))
                (Default|AddBuffStatusEffects _statscomp_2 (LocalVariables|GetBuffEffects))))))
        (:CastFailed
          (Class|MmoUtilities|LogString (Utilities|String|Append "Apply Buff failed: BuffAsset invalid " (Utilities|String|ToString(Integer) BuffAsset)) "Verbosity_Normal"))))
    (:CastFailed
      (Development|PrintString "ApplyBuff fail: BuffComponent is attached to a non-Character" true true "(R=1.000000,G=0.000000,B=0.058691,A=1.000000)" 5.0))))

(fn OnBuffExpired
  (params (Guid :type Guid%20Structure%20%28by%20ref%29))
  (bind _activebuffs (Variables|Default|GetActiveBuffs))
  (bind (_value _returnvalue) (Utilities|Map|Find _activebuffs Guid))
  (Utilities|FlowControl|Sequence
    (:then_0
      (if _returnvalue
        (CallFunction|RemoveBufffromReplication Guid)
        (bind _output_get (LocalVariables|SetActiveBuff _value))
        (LocalVariables|SetBuffHadStatusEffects (Utilities|Array|IsNotEmpty (.Effects (Utilities|Struct|BreakFActiveBuff _output_get))))
        (Utilities|FlowControl|Sequence
          (:then_0
            (Class|MmoUtilities|LogString (Utilities|String|ToString(Text) (Utilities|Text|FormatText "Buff Expired, duration: {dur}, GUID: {guid}" (.Duration (Utilities|Struct|BreakFActiveBuff (LocalVariables|GetActiveBuff))) (Guid|ToString(Guid) Guid))) "Verbosity_SuperVerbose")
            (if (AssetManager|IsValidPrimaryAssetId (.BuffAsset (Utilities|Struct|BreakFActiveBuff (LocalVariables|GetActiveBuff))))
              (Utilities|IsValid (Class|KismetSystemLibrary|GetObjectfromPrimaryAssetId (.BuffAsset (Utilities|Struct|BreakFActiveBuff (LocalVariables|GetActiveBuff))))
                (:Is%20Valid
                  (bind _asbuff_asset (Utilities|Casting|CastToBuffAsset (Class|KismetSystemLibrary|GetObjectfromPrimaryAssetId (.BuffAsset (Utilities|Struct|BreakFActiveBuff (LocalVariables|GetActiveBuff))))))
                  (Utilities|IsValid (Variables|/Script/MMOKitCode.BuffAssetCpp|GetBuffDynamics _asbuff_asset)
                    (:Is%20Valid
                      (bind _asbuff_dynamics (Utilities|Casting|CastToBuffDynamics (Variables|/Script/MMOKitCode.BuffAssetCpp|GetBuffDynamics _asbuff_asset)))
                      (Default|OnBuffEnd _asbuff_dynamics (.AsCharacter (Utilities|Casting|CastToCharacter (Components|GetOwner))) (LocalVariables|GetActiveBuff))))))))
          (:then_1
            (Class|BuffsSubsystem|StopTickingBuff (Subsystems|GetBuffsSubsystem) Guid)
            (Utilities|Map|Remove (Variables|Default|GetActiveBuffs) Guid)))
        (else
          (Class|MmoUtilities|LogString "Buff Expired, but not found. This is normal, it was removed previously." "Verbosity_SuperVerbose"))))
    (:then_1
      (if (LocalVariables|GetBuffHadStatusEffects)
        (bind _statscomp (Class|BPIStats|GetStatsComponent(Message) (Variables|Default|GetOwnerCharacter)))
        (bind _effects (CallFunction|GetActiveBuffEffects))
        (Default|RecalculateBuffStatusEffects _statscomp _effects)))))

(fn OnBuffTicks
  (params (Guid :type Guid%20Structure%20%28by%20ref%29))
  (bind _activebuffs (Variables|Default|GetActiveBuffs))
  (bind (_value _returnvalue) (Utilities|Map|Find _activebuffs Guid))
  (if _returnvalue
    (LocalVariables|SetActiveBuff _value)
    (Class|MmoUtilities|LogString (Utilities|String|ToString(Text) (Utilities|Text|FormatText "Ticking Buff, duration: {dur}, GUID: {guid}" (.Duration (Utilities|Struct|BreakFActiveBuff (LocalVariables|GetActiveBuff))) (Guid|ToString(Guid) Guid))) "Verbosity_SuperVerbose")
    (if (AssetManager|IsValidPrimaryAssetId (.BuffAsset (Utilities|Struct|BreakFActiveBuff (LocalVariables|GetActiveBuff))))
      (Utilities|IsValid (Class|KismetSystemLibrary|GetObjectfromPrimaryAssetId (.BuffAsset (Utilities|Struct|BreakFActiveBuff (LocalVariables|GetActiveBuff))))
        (:Is%20Valid
          (bind _asbuff_asset (Utilities|Casting|CastToBuffAsset (Class|KismetSystemLibrary|GetObjectfromPrimaryAssetId (.BuffAsset (Utilities|Struct|BreakFActiveBuff (LocalVariables|GetActiveBuff))))))
          (Utilities|IsValid (Variables|/Script/MMOKitCode.BuffAssetCpp|GetBuffDynamics _asbuff_asset)
            (:Is%20Valid
              (bind _asbuff_dynamics (Utilities|Casting|CastToBuffDynamics (Variables|/Script/MMOKitCode.BuffAssetCpp|GetBuffDynamics _asbuff_asset)))
              (Default|TickLogic _asbuff_dynamics (.AsCharacter (Utilities|Casting|CastToCharacter (Components|GetOwner))) (LocalVariables|GetActiveBuff) Guid))))))
    (else
      (Development|PrintString "Buff Ticking, not found?!"))))

(fn CancelBuff
  (params (Guid :type Guid%20Structure))
  (Class|BuffsSubsystem|UnregisterBuff (Subsystems|GetBuffsSubsystem) Guid)
  (CallFunction|OnBuffExpired Guid))

(fn GetBuffRemainingDuration
  (params (Buff :type F%20Active%20Buff%20Structure%20%28by%20ref%29))
  (bind (_duration _timeofcreation) (Utilities|Struct|BreakFActiveBuff Buff))
  ;[0.4452 0.6332 1] Get time remaining on an Active Buff
  (if (> _duration 0.0)
    (return (- (+ _duration _timeofcreation) (GameState|GetServerWorldTimeSeconds (Game|GetGameState))))
    (else
      (return _duration))))

(fn GetSerializedBuffs
  (bind _values (Utilities|Map|Values (Variables|Default|GetActiveBuffs)))
  (for _array_element _values
    (Utilities|Array|Add (LocalVariables|GetResult) (Utilities|Struct|MakeFSerializedBuff (.Effects (Utilities|Struct|BreakFActiveBuff _array_element)) (.BuffAsset (Utilities|Struct|BreakFActiveBuff _array_element)) (.InstigatingAbility (Utilities|Struct|BreakFActiveBuff _array_element)) (.InstigatorInfo (Utilities|Struct|BreakFActiveBuff _array_element)) (CallFunction|GetBuffRemainingDuration _array_element))))
  (return (LocalVariables|GetResult)))

(fn RecreateBuffsfromDb
  (params (BuffsToRecreate :type Array%20of%20F%20Serialized%20Buff%20Structures))
  (bind _ascharacter (Utilities|Casting|CastToCharacter (Components|GetOwner))
    (:then
      (LocalVariables|SetVictim _ascharacter)
      (for _array_element BuffsToRecreate
        (bind _output_get (LocalVariables|SetSerializedBuff _array_element))
        (bind _asbuff_asset (Utilities|Casting|CastToBuffAsset (Class|KismetSystemLibrary|GetObjectfromPrimaryAssetId (Utilities|Struct|BreakFSerializedBuff (LocalVariables|GetSerializedBuff))))
          (:then
            (LocalVariables|SetBuffAssetObject _asbuff_asset)
            (if (not (Math|Float|InRange(Float) (Utilities|Struct|BreakFSerializedBuff (LocalVariables|GetSerializedBuff)) -1.0 0.0 false false)) ; Skip buffs between -1 and 0, they're just buffs that should've run out, but didn't\nget the opportunity to get removed just before being saved.
              (LocalVariables|SetBuffGuid (Guid|NewGuid))
              (Utilities|FlowControl|Sequence
                (:then_0
                  (if (Utilities|IsValidClass (Variables|/Game/MMOKit/MMO_Logic/Blueprints/DataAssetTypes/BuffAsset.BuffAsset_C|GetBuffTriggers (LocalVariables|GetBuffAssetObject)))
                    (bind _returnvalue (Game|ConstructObjectfromClass (Variables|/Game/MMOKit/MMO_Logic/Blueprints/DataAssetTypes/BuffAsset.BuffAsset_C|GetBuffTriggers (LocalVariables|GetBuffAssetObject))))
                    (bind _output_get_2 (LocalVariables|SetBuffTriggersObject _returnvalue))
                    (Default|SignUptoEvents _output_get_2 (LocalVariables|GetVictim) (Utilities|Struct|BreakFSerializedBuff (LocalVariables|GetSerializedBuff)))))
                (:then_1
                  (bind _output_get_3 (LocalVariables|SetAppliedBuff (Utilities|Struct|MakeFActiveBuff (.Effects (Utilities|Struct|BreakFSerializedBuff (LocalVariables|GetSerializedBuff))) (.BuffAsset (Utilities|Struct|BreakFSerializedBuff (LocalVariables|GetSerializedBuff))) (.InstigatingAbility (Utilities|Struct|BreakFSerializedBuff (LocalVariables|GetSerializedBuff))) (.InstigatorInfo (Utilities|Struct|BreakFSerializedBuff (LocalVariables|GetSerializedBuff))) (.TimeRemaining (Utilities|Struct|BreakFSerializedBuff (LocalVariables|GetSerializedBuff))) (GameState|GetServerWorldTimeSeconds (Game|GetGameState)) (LocalVariables|GetBuffTriggersObject))))
                  (Utilities|Map|Add (Variables|Default|GetActiveBuffs) (LocalVariables|GetBuffGuid) _output_get_3))
                (:then_2
                  (Utilities|IsValid (LocalVariables|GetBuffAssetObject)
                    (:Is%20Valid
                      (Utilities|IsValid (Variables|/Script/MMOKitCode.BuffAssetCpp|GetBuffDynamics (LocalVariables|GetBuffAssetObject))
                        (:Is%20Valid
                          (bind _asbuff_dynamics (Utilities|Casting|CastToBuffDynamics (Variables|/Script/MMOKitCode.BuffAssetCpp|GetBuffDynamics (LocalVariables|GetBuffAssetObject))))
                          (Default|OnBuffApply _asbuff_dynamics (LocalVariables|GetVictim) (LocalVariables|GetAppliedBuff)))))))
                (:then_3
                  (Class|BuffsSubsystem|RegisterBuff (Subsystems|GetBuffsSubsystem) (LocalVariables|GetBuffGuid) (Utilities|Struct|BreakFSerializedBuff (LocalVariables|GetSerializedBuff)) (EventDispatchers|CreateEvent :!event OnBuffExpired)) ; Registering the buff with the Subsystem will allow the buff to expire after its Duration has run out
                )
                (:then_4
                  (if (and (Variables|/Game/MMOKit/MMO_Logic/Blueprints/DataAssetTypes/BuffAsset.BuffAsset_C|GetTicks (LocalVariables|GetBuffAssetObject)) (!= (Utilities|Struct|BreakFSerializedBuff (LocalVariables|GetSerializedBuff)) 0.0))
                    (Class|BuffsSubsystem|StartTickingBuff (Subsystems|GetBuffsSubsystem) (LocalVariables|GetBuffGuid) 0.0 (Variables|/Game/MMOKit/MMO_Logic/Blueprints/DataAssetTypes/BuffAsset.BuffAsset_C|GetTickFrequency (LocalVariables|GetBuffAssetObject)) (EventDispatchers|CreateEvent :!event OnBuffTicks))))
                (:then_5
                  (if (and (Variables|/Game/MMOKit/MMO_Logic/Blueprints/DataAssetTypes/BuffAsset.BuffAsset_C|GetDisplayIcon (LocalVariables|GetBuffAssetObject)) (!= (Utilities|Struct|BreakFSerializedBuff (LocalVariables|GetSerializedBuff)) 0.0))
                    _)))))
          (:CastFailed
            (Class|MmoUtilities|LogString (Utilities|String|Append "Recreate Buff failed: BuffAsset invalid " (Utilities|String|ToString(Integer) (Utilities|Struct|BreakFSerializedBuff _output_get))) "Verbosity_Normal")))))
    (:CastFailed
      (Development|PrintString "ApplyBuff fail: BuffComponent is attached to a non-Character" true true "(R=1.000000,G=0.000000,B=0.058691,A=1.000000)" 5.0))))

(fn AddBufftoReplication
  (params (Guid :type Guid%20Structure))
  (bind _activebuffs (Variables|Default|GetActiveBuffs))
  (bind (_value _returnvalue) (Utilities|Map|Find _activebuffs Guid))
  ;[0.4452 0.6332 1] Add Buff To Replication
  (if _returnvalue
    (bind _output_get (LocalVariables|SetReplicatedBuff (Utilities|Struct|MakeFReplicatedBuff (Utilities|Struct|BreakFActiveBuff _value) Guid (GameState|GetServerWorldTimeSeconds (Game|GetGameState)) (CallFunction|GetBuffRemainingDuration _value))))
    (Utilities|Array|Add (Variables|Default|GetReplicatedBuffProxies) _output_get)))

(fn RemoveBufffromReplication
  (params (Guid :type Guid%20Structure))
  ;[0.4452 0.6332 1] Remove Buff From Replication
  (bind (_array_element _array_index) (Utilities|Array|ForEachLoopwithBreak (Variables|Default|GetReplicatedBuffProxies) :!label _label)
    (:LoopBody
      (if (== (Utilities|Struct|BreakFReplicatedBuff _array_element) Guid)
        (Utilities|Array|RemoveIndex (Variables|Default|GetReplicatedBuffProxies) _array_index)
        (goto _label Break)))))

(fn HasBuffonClient
  (params (BuffAsset :type Primary%20Asset%20Id%20Structure))
  ;[0.4452 0.6332 1] Check if player has buff
  (for _array_element (Variables|Default|GetReplicatedBuffProxies)
    (if (== (Utilities|Struct|BreakFReplicatedBuff _array_element) BuffAsset)
      (return true)))
  (return false))

(fn HasBuffonServer
  (params (BuffAsset :type Primary%20Asset%20Id%20Structure))
  ;[0.4452 0.6332 1] Check if player has buff
  (bind _values (Utilities|Map|Values (Variables|Default|GetActiveBuffs)))
  (for _array_element _values
    (if (== BuffAsset (Utilities|Struct|BreakFActiveBuff _array_element))
      (return true)))
  (return false))

(fn RemoveBuffsonDeath
  ;[0.4452 0.6332 1] Remove Buffs On Death (called OnDeath)
  (bind _keys (Utilities|Map|Keys (Variables|Default|GetActiveBuffs)))
  (for _array_element _keys
    (bind _asbuff_asset (Utilities|Casting|CastToBuffAsset (Class|KismetSystemLibrary|GetObjectfromPrimaryAssetId (Utilities|Struct|BreakFActiveBuff (.Value (Utilities|Map|Find (Variables|Default|GetActiveBuffs) _array_element))))))
    (if (Variables|/Game/MMOKit/MMO_Logic/Blueprints/DataAssetTypes/BuffAsset.BuffAsset_C|GetRemoveOnDeath _asbuff_asset)
      (CallFunction|CancelBuff _array_element))))

(fn AddAllBuffstoReplication
  ;[0.4452 0.6332 1] Replicate All Buffs
  (bind _keys (Utilities|Map|Keys (Variables|Default|GetActiveBuffs)))
  (for _array_element _keys
    (bind _asbuff_asset (Utilities|Casting|CastToBuffAsset (Class|KismetSystemLibrary|GetObjectfromPrimaryAssetId (.BuffAsset (Utilities|Struct|BreakFActiveBuff (.Value (Utilities|Map|Find (Variables|Default|GetActiveBuffs) _array_element)))))))
    (if (Variables|/Game/MMOKit/MMO_Logic/Blueprints/DataAssetTypes/BuffAsset.BuffAsset_C|GetDisplayIcon _asbuff_asset)
      (CallFunction|AddBufftoReplication _array_element))))

(fn OnRepReplicatedBuffProxies
  (Networking|CanExecuteCosmeticEvents
    (:True
      (if (== (Components|GetOwner) (Game|GetPlayerCharacter 0))
        (Default|CallOnBuffsUpdated (Variables|Default|GetReplicatedBuffProxies))))))

(fn CancelBuffbyAsset
  (params (BuffAsset :type Primary%20Asset%20Id%20Structure))
  (bind _keys (Utilities|Map|Keys (Variables|Default|GetActiveBuffs)))
  (for _array_element _keys
    (LocalVariables|SetGuid _array_element)
    (if (== (Utilities|Struct|BreakFActiveBuff (.Value (Utilities|Map|Find (Variables|Default|GetActiveBuffs) _array_element))) BuffAsset)
      (CallFunction|CancelBuff (LocalVariables|GetGuid))
      (return))))

(fn GetActiveBuffEffects
  (bind _values (Utilities|Map|Values (Variables|Default|GetActiveBuffs)))
  (for _array_element _values
    (for _array_element_2 (.Effects (Utilities|Struct|BreakFActiveBuff _array_element))
      (Utilities|Array|Add (LocalVariables|GetResult) _array_element_2)))
  (return (LocalVariables|GetResult)))
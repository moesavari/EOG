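; Mob-specific stats component that extends its parent's begin-play and damage handling for MMO mobs.
; Where cosmetic events cannot execute, it fetches the owner's mob event bus at begin play, retrying each tick until valid.
; Damage runs the parent logic, then raises a got-hit event on that bus with attacker and amount.
; Name updates broadcast the mob name queried from the owner.
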(event EventBeginPlay
  (|CallParentFunction)
  ;[0.4452 0.6332 1] Set up Event Bus
  (Networking|CanExecuteCosmeticEvents
    (:False
      (bind _eventbus (Class|BPIMobSpecific|GetMobEventBus(Message) (Components|GetOwner) :!label _label))
      (Utilities|IsValid _eventbus
        (:Is%20Valid
          (Variables|Default|SetOwnerEventBus _eventbus))
        (:Is%20Not%20Valid
          (Utilities|FlowControl|DelayUntilNextTick)
          (Class|MmoUtilities|LogString "MobStatsComp: delay 1 frame" "Verbosity_SuperVerbose")
          (goto _label))))))

(event EventEmitNameUpdated
  ;[1 0.312 0.302] Emit Name Updated
  (bind _mobname (Class|BPIMobSpecific|GetMobName(Message) (Components|GetOwner)))
  (Default|CallOnNameUpdated (Utilities|String|ToString(Text) _mobname)))

(event EventTakeDamage
  (params (Attacker :type Character%20Object%20Reference) (Dmg :type Integer))
  ;[0.4452 0.6332 1] Take Damage (server)
  (|CallParentFunction Attacker Dmg)
  (Default|CallOnGotHit (Variables|Default|GetOwnerEventBus) Attacker Dmg))
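; Player state for the MMO kit that preloads ability and buff assets on the client and keeps them in memory.
; On BeginPlay, where cosmetic events can run, it retries each tick until player 0's PlayerState is valid, continuing only if that is itself.
; It async loads every primary asset of the types in PrimaryTypesToLoad, then sorts the results into LoadedAbilities and LoadedBuffs.
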(event EventBeginPlay
  (bind _returnvalue (Game|GetPlayerController 0))
  (bind _playerstate (Variables|/Script/Engine.Controller|GetPlayerState _returnvalue))
  ;[1 0.312 0.302] Loads Abilities and Buffs on client start, then keeps them in memory
  (Class|MmoUtilities|LogString "BeginPlay: PlayerState" "Verbosity_SuperVerbose")
  (Networking|CanExecuteCosmeticEvents
    (:True
      (Utilities|IsValid _playerstate :!label _label
        (:Is%20Valid
          (if (== _playerstate self) ; check that this is our PS\nnot someone else's
            (for _array_element (Variables|Default|GetPrimaryTypesToLoad)
              (bind _outprimaryassetidlist (Class|KismetSystemLibrary|GetPrimaryAssetIdList _array_element))
              (bind _loaded (|AsyncLoadPrimaryAssetList _outprimaryassetidlist)
                (:Completed
                  (for _array_element_2 _loaded
                    (bind _asability_asset (Utilities|Casting|CastToAbilityAsset _array_element_2)
                      (:then
                        (Utilities|Array|Add (Variables|Default|GetLoadedAbilities) _asability_asset)
                        (Class|MmoUtilities|LogString (Utilities|String|Append "Client Loaded Ability: " (Utilities|GetObjectName _asability_asset)) "Verbosity_SuperVerbose"))
                      (:CastFailed
                        (bind _asbuff_asset (Utilities|Casting|CastToBuffAsset _array_element_2))
                        (Utilities|Array|Add (Variables|Default|GetLoadedBuffs) _asbuff_asset)
                        (Class|MmoUtilities|LogString (Utilities|String|Append "Client Loaded Buff: " (Utilities|GetObjectName _asbuff_asset)) "Verbosity_SuperVerbose")))))))))
        (:Is%20Not%20Valid
          (Utilities|FlowControl|DelayUntilNextTick)
          (goto _label))))))

(fn ConstructionScript)
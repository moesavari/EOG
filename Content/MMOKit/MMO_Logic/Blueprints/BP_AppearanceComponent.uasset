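; Character component that holds a player's or NPC's replicated appearance (race, sex, body, equipped items) and applies it to the owner.
; Replication async-loads mesh, AnimBP and gear, then sets them through interface messages and caches battle stance, delaying newer updates while loading.
; Equipment updates edit the base of an appearance stack, reaching the replicated value only when it is the sole entry.
; Camera changes re-emit hands data for first-person view.
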(event Custom|OnCameraChanged
  (params (NewCamera :type ECameraType%20Enum :default "NewEnumerator0"))
  (bind _fullappearance (Variables|Default|GetFullAppearance))
  (bind (_appearance _sex _race _equippeditems) (Utilities|Struct|BreakFAppearanceFull _fullappearance))
  ;[1 1 1] When switching to First Person Camera, emit an event as if we just received a new appearance with new hands/weapon
  ; So that our FirstPersonCamera component can set up the First Person Hands mesh
  (if (Utilities|Enum|Equal(Enum) NewCamera "NewEnumerator0")
    (Class|BPIFirstPersonCharacter|EmitUpdateHands(Message) (Variables|Default|GetOwnerCharacter) (Utilities|Array|Get(acopy) _equippeditems 1) _appearance _sex) ; If the character implements FirstPerson interface
  ))

(event Custom|InitializeNpcAppearance
  ;[0.7865 0.1065 0.7201] Initialize NPC appearance on BeginPlay
  (Utilities|IsValid (.Appearance (Utilities|Struct|BreakFAppearanceFull (Variables|Default|GetFullAppearance)))
    (:Is%20Valid
      (CallFunction|UpdateFullAppearance)
      ;[0.4452 0.6332 1] server-side
      (Networking|CanExecuteCosmeticEvents
        (:False
          (Utilities|Array|Add :TargetArray (Variables|Default|GetAppearancesStack)))))
    (:Is%20Not%20Valid
      (bind _returnvalue (Game|GetCurrentLevelName true))
      (if (not (Utilities|Enum|Equal(Enum) _returnvalue "StartMap"))
        (Class|MmoUtilities|LogString "ERROR: Mob's appearance is not set!" "Verbosity_Normal" true true "(R=1.000000,G=0.000000,B=0.024480,A=1.000000)" 1e+01)))))

(event Custom|UpdateFullAppearance
  (bind _fullappearance (Variables|Default|GetFullAppearance))
  (bind _fullappearance_2 (Variables|Default|GetFullAppearance))
  (bind _ownercharacter (Variables|Default|GetOwnerCharacter))
  (bind (_appearance _sex _equippeditems) (Utilities|Struct|BreakFAppearanceFull _fullappearance_2))
  (bind (_appearance_2 _sex_2 _race) (Utilities|Struct|BreakFAppearanceFull _fullappearance))
  ;[1 1 1] When FullAppearance replicates, we call UpdateFullAppearance
  ; It will load all the necessary items and call Character->SetBody and Character->SetEquipment, which are interface functions
  (Class|MmoUtilities|LogString "Appearance: UpdateFullAppearance" "Verbosity_SuperVerbose")
  (Utilities|IsValid (Variables|Default|GetOwnerCharacter) :!label _label
    (:Is%20Valid
      (if (Variables|AsyncLoad|GetLoadingAssets) :!label _label_2
        ;;[0 0.2214 1] One of the biggest issues with this replication is: if we're in the middle of loading
        ;; some models and a NEW FullAppearance arrives from the server, we can load the new one faster than the old one. And then once the old one loads, it can override the new one.
        ;; To prevent that, we'll use a LoadingAssets bool
        ;; If assets are being loaded, we'll wait for them, and only then we'll work on setting the newer appearance
        (Class|MmoUtilities|LogString "Loading assets: so delay" "Verbosity_SuperVerbose")
        (Utilities|FlowControl|DelayUntilNextTick)
        (goto _label_2)
        (else
          (Class|MmoUtilities|LogString "Start loading assets" "Verbosity_SuperVerbose")
          (Variables|AsyncLoad|SetLoadingAssets true)
          (bind (_foundvalid _mesh _animbp) (CallFunction|GetAppearanceMeshandAnimBp))
          (bind (_loadedskelmesh _loadedanimbpclass _loadedgearassets) (|AsyncLoadAppearanceAssets _mesh _animbp (Utilities|Struct|BreakFAppearanceFull (Variables|Default|GetFullAppearance)))
            (:LoadComplete
              (Variables|AsyncLoad|SetLoadedGearAssets _loadedgearassets)
              ;;[1 0.2374 0] TODO: SetBody and SetGear need to be async tasks
              ;; And we should await them, before seting LoadingAssets=false
              (Class|BPIAppearance|SetBody(Message) (Variables|Default|GetOwnerCharacter) _loadedskelmesh _loadedanimbpclass _sex_2 _race)
              (if (Variables|/Game/MMOKit/MMO_Logic/Blueprints/DataAssetTypes/CreatureAppearance.CreatureAppearance_C|GetPlayerAppearance _appearance_2)
                (Class|BPIAppearance|SetGear(Message) _ownercharacter (Utilities|Struct|BreakFAppearanceFull (Variables|Default|GetFullAppearance)))
                (else
                  (Class|BPIAppearance|EmptyGear(Message) _ownercharacter)))
              (Class|BPIFirstPersonCharacter|EmitUpdateHands(Message) _ownercharacter (Utilities|Array|Get(acopy) _equippeditems 1) _appearance _sex) ; If the character implements FirstPerson interface
              ;;[1 1 1] cleanup
              (CallFunction|SaveStance)
              (Utilities|Array|Clear (Variables|AsyncLoad|GetLoadedGearAssets))
              (Variables|AsyncLoad|SetLoadingAssets false))))))
    (:Is%20Not%20Valid
      (Utilities|FlowControl|DelayUntilNextTick) ; We need to wait for BeginPlay to finish doing its job\nBefore we can react to FullAppearance replication
      (Class|MmoUtilities|LogString "UpdateFullAppearance: delaying by 1 frame" "Verbosity_SuperVerbose")
      (goto _label))))

(event Custom|InitializePlayerAppearance
  (params (InAppearance :type F%20Appearance%20Partial%20Structure))
  (bind (_sex _race) (Utilities|Struct|BreakFAppearancePartial InAppearance))
  ;[0.4452 0.6332 1] Initialize player appearance
  (bind _output_get (Variables|Default|SetFullAppearance (Utilities|Struct|MakeFAppearanceFull (Utilities|Select :Index _race :NewEnumerator2 0 :NewEnumerator0 "/Game/MMOKit/MMO_Content/CreatureAppearances/Mannequin.Mannequin" :NewEnumerator1 "/Game/MMOKit/MMO_Content/CreatureAppearances/Human.Human") _sex _race)))
  (Utilities|Array|Add (Variables|Default|GetAppearancesStack) _output_get))

(event Custom|SignUpToControllerEvents
  (params (EquipComp :type BP%20Equipment%20Component%20Object%20Reference))
  ;[1 1 1] BeginPlay
  (EventDispatchers|AssignOnAppearanceUpdated EquipComp (EventDispatchers|CreateEvent :!event OnEquipmentUpdatesAppearance))
  (Class|MmoUtilities|LogString "Apperance: bound to equipment" "Verbosity_SuperVerbose"))

(event EventBeginPlay
  (bind _returnvalue (Game|GetPlayerController 0))
  ;[1 1 1] BeginPlay
  (Class|MmoUtilities|LogString "Appearance Component: BeginPlay" "Verbosity_SuperVerbose")
  (bind _ascharacter (Utilities|Casting|CastToCharacter (Components|GetOwner)))
  (bind _output_get (Variables|Default|SetOwnerCharacter _ascharacter))
  (bind _isplayer (Class|BPICharacter|IsPlayerCharacter(Message) _output_get))
  (if _isplayer
    (Networking|CanExecuteCosmeticEvents
      (:True
        ;[1 1 1] When switching to First Person Camera, emit an event as if we just received a new appearance with new hands/weapon
        ; So that our FirstPersonCamera component can set up the First Person Hands mesh
        (if (== (Variables|Default|GetOwnerCharacter) (Game|GetPlayerCharacter 0)) ; is this our character?
          (Utilities|IsValid _returnvalue :!label _label
            (:Is%20Valid
              (bind _asbp_player_controller (Utilities|Casting|CastToBP_PlayerController _returnvalue))
              (EventDispatchers|BindEventtoOnCameraChanged _asbp_player_controller (delegate Custom|OnCameraChanged)))
            (:Is%20Not%20Valid
              (Utilities|FlowControl|DelayUntilNextTick)
              (goto _label)))))
      (:False))
    (else
      (CallFunction|InitializeNpcAppearance))))

(fn GetAppearanceMeshandAnimBp
  (bind _fullappearance (Variables|Default|GetFullAppearance))
  (bind _fullappearance_2 (Variables|Default|GetFullAppearance))
  (bind _fullappearance_3 (Variables|Default|GetFullAppearance))
  (bind _fullappearance_4 (Variables|Default|GetFullAppearance))
  (bind (_appearance _sex) (Utilities|Struct|BreakFAppearanceFull _fullappearance))
  (bind (_appearance_2 _sex_2) (Utilities|Struct|BreakFAppearanceFull _fullappearance_2))
  (bind (_appearance_3 _sex_3) (Utilities|Struct|BreakFAppearanceFull _fullappearance_3))
  (bind (_appearance_4 _sex_4) (Utilities|Struct|BreakFAppearanceFull _fullappearance_4))
  (bind _skeletalmeshmale (Variables|/Game/MMOKit/MMO_Logic/Blueprints/DataAssetTypes/CreatureAppearance.CreatureAppearance_C|GetSkeletalMeshMale _appearance_3))
  (bind _animbpmale (Variables|/Game/MMOKit/MMO_Logic/Blueprints/DataAssetTypes/CreatureAppearance.CreatureAppearance_C|GetAnimBpMale _appearance_4))
  (bind _animbpfemale (Variables|/Game/MMOKit/MMO_Logic/Blueprints/DataAssetTypes/CreatureAppearance.CreatureAppearance_C|GetAnimBpFemale _appearance_4))
  (bind _skeletalmeshmale_2 (Variables|/Game/MMOKit/MMO_Logic/Blueprints/DataAssetTypes/CreatureAppearance.CreatureAppearance_C|GetSkeletalMeshMale _appearance))
  (bind _skeletalmeshfemale (Variables|/Game/MMOKit/MMO_Logic/Blueprints/DataAssetTypes/CreatureAppearance.CreatureAppearance_C|GetSkeletalMeshFemale _appearance_3))
  (bind _skeletalmeshfemale_2 (Variables|/Game/MMOKit/MMO_Logic/Blueprints/DataAssetTypes/CreatureAppearance.CreatureAppearance_C|GetSkeletalMeshFemale _appearance))
  (bind _animbpmale_2 (Variables|/Game/MMOKit/MMO_Logic/Blueprints/DataAssetTypes/CreatureAppearance.CreatureAppearance_C|GetAnimBpMale _appearance_2))
  (bind _animbpfemale_2 (Variables|/Game/MMOKit/MMO_Logic/Blueprints/DataAssetTypes/CreatureAppearance.CreatureAppearance_C|GetAnimBpFemale _appearance_2))
  (bind _returnvalue (Utilities|Select :Index _sex_3 :NewEnumerator0 _skeletalmeshmale :NewEnumerator1 _skeletalmeshfemale))
  (bind _returnvalue_2 (Utilities|Select :Index _sex_4 :NewEnumerator0 _animbpmale :NewEnumerator1 _animbpfemale))
  (bind _returnvalue_3 (Utilities|Select :Index _sex :NewEnumerator0 _skeletalmeshfemale_2 :NewEnumerator1 _skeletalmeshmale_2))
  (bind _returnvalue_4 (Utilities|Select :Index _sex_2 :NewEnumerator0 _animbpfemale_2 :NewEnumerator1 _animbpmale_2))
  (Utilities|FlowControl|Sequence
    (:then_0
      ;[1 1 1] Get mesh by sex, but fallback to the wrong sex mesh if not set
      (if (Utilities|IsValidSoftObjectReference _returnvalue)
        (LocalVariables|SetMeshToReturn _returnvalue)
        (elif (Utilities|IsValidSoftObjectReference _returnvalue_3)
          (LocalVariables|SetMeshToReturn _returnvalue_3))))
    (:then_1
      ;[1 1 1] Get anim bp by sex, but fallback to the wrong sex animbp if not set
      (if (Utilities|IsValidSoftClassReference _returnvalue_2)
        (LocalVariables|SetAnimBpToReturn _returnvalue_2)
        (elif (Utilities|IsValidSoftClassReference _returnvalue_4)
          (LocalVariables|SetAnimBpToReturn _returnvalue_4))))
    (:then_2
      (return (and (Utilities|IsValidSoftObjectReference (LocalVariables|GetMeshToReturn)) (Utilities|IsValidSoftClassReference (LocalVariables|GetAnimBpToReturn))) (LocalVariables|GetMeshToReturn) (LocalVariables|GetAnimBpToReturn)))))

(fn OnRepFullAppearance
  (CallFunction|UpdateFullAppearance))

(fn SwapSex
  (bind _output_get (Variables|Default|SetFullAppearance (Utilities|Struct|MakeFAppearanceFull (.Appearance (Utilities|Struct|BreakFAppearanceFull (Variables|Default|GetFullAppearance))) (Utilities|Select :Index (.Sex (Utilities|Struct|BreakFAppearanceFull (Variables|Default|GetFullAppearance))) :NewEnumerator0 "NewEnumerator1" :NewEnumerator1 "NewEnumerator0") (.Race (Utilities|Struct|BreakFAppearanceFull (Variables|Default|GetFullAppearance))) (.EquippedItems (Utilities|Struct|BreakFAppearanceFull (Variables|Default|GetFullAppearance))))))
  (Utilities|Array|SetArrayElem (Variables|Default|GetAppearancesStack) 0 _output_get))

(fn OnEquipmentUpdatesAppearance
  (params (EquippedItems :type Array%20of%20Primary%20Asset%20Id%20Structures))
  (bind _appearancesstack (Variables|Default|GetAppearancesStack))
  (bind _output (Utilities|Array|Get(acopy) _appearancesstack))
  (bind (_appearance _sex _race) (Utilities|Struct|BreakFAppearanceFull _output))
  (bind _fappearancefull (Utilities|Struct|MakeFAppearanceFull _appearance _sex _race EquippedItems))
  ;[1 1 1] 1. Modifies the first element in the Stack of appearances
  ; 2. If we only have 1 appearance on stack, also modifies replicated appearance
  ;;[1 0.2374 0] TODO: what is this? why length 1?
  (|SetBy-RefVar (Utilities|Array|Get(acopy) (Variables|Default|GetAppearancesStack)) _fappearancefull)
  (if (== (Utilities|Array|Length (Variables|Default|GetAppearancesStack)) 1)
    (Variables|Default|SetFullAppearance _fappearancefull)))

(fn ShouldAttachEyes
  (return (Variables|/Game/MMOKit/MMO_Logic/Blueprints/DataAssetTypes/CreatureAppearance.CreatureAppearance_C|GetAttachEyes (.Appearance (Utilities|Struct|BreakFAppearanceFull (Variables|Default|GetFullAppearance))))))

(fn IsAppearanceFemale
  (return (not (Utilities|Enum|Equal(Enum) (.Sex (Utilities|Struct|BreakFAppearanceFull (Variables|Default|GetFullAppearance))) "NewEnumerator0"))))

(fn GetBattleStance
  (return (Variables|Default|GetStanceCache)))

(fn SaveStance
  (bind _fullappearance (Variables|Default|GetFullAppearance))
  (bind _equippeditems (Utilities|Struct|BreakFAppearanceFull _fullappearance))
  (bind _output (Utilities|Array|Get(acopy) _equippeditems 1))
  ;[1 1 1] Caches stance from current appearance
  ; It's called from UpdateFullAppearance, which is called from OnRep_FullAppearance
  (if (Utilities|Array|IsValidIndex _equippeditems 1)
    (if (AssetManager|IsValidPrimaryAssetId _output)
      (bind _asequipment_asset (Utilities|Casting|CastToEquipmentAsset (Class|KismetSystemLibrary|GetObjectfromPrimaryAssetId _output))
        (:then
          (bind _array_element (Utilities|Array|ForEachLoopwithBreak (Variables|/Script/MMOKitCode.ItemAsset|GetProperties _asequipment_asset) :!label _label)
            (:LoopBody
              (bind _asweapon_property (Utilities|Casting|CastToWeaponProperty _array_element))
              (Variables|Default|SetStanceCache (Variables|/Game/MMOKit/MMO_Logic/Blueprints/DataAssetTypes/ItemProperties/WeaponProperty.WeaponProperty_C|GetBattleStance _asweapon_property))
              (LocalVariables|SetFoundStance true)
              (goto _label Break))
            (:Completed
              (if (not (LocalVariables|GetFoundStance))
                (Variables|Default|SetStanceCache "NewEnumerator0")))))
        (:CastFailed
          (Variables|Default|SetStanceCache "NewEnumerator0")))
      (else
        (Variables|Default|SetStanceCache "NewEnumerator0" :!label _label_2)))
    (else
      (goto _label_2))))

(fn FilterOutInvalid
  (params (In :type Array%20of%20Primary%20Asset%20Id%20Structures))
  (for _array_element In
    (if (AssetManager|IsValidPrimaryAssetId _array_element)
      (Utilities|Array|Add (LocalVariables|GetRet) _array_element)))
  (return (LocalVariables|GetRet)))

(fn SwapSpecies
  (bind _output_get (Variables|Default|SetFullAppearance (Utilities|Struct|MakeFAppearanceFull (select (== (.Appearance (Utilities|Struct|BreakFAppearanceFull (Variables|Default|GetFullAppearance))) "/Game/MMOKit/MMO_Content/CreatureAppearances/Human.Human") "/Game/MMOKit/MMO_Content/CreatureAppearances/Mannequin.Mannequin" "/Game/MMOKit/MMO_Content/CreatureAppearances/Human.Human") (.Sex (Utilities|Struct|BreakFAppearanceFull (Variables|Default|GetFullAppearance))) (select (Utilities|Enum|Equal(Enum) (.Race (Utilities|Struct|BreakFAppearanceFull (Variables|Default|GetFullAppearance))) "NewEnumerator1") "NewEnumerator0" "NewEnumerator1") (.EquippedItems (Utilities|Struct|BreakFAppearanceFull (Variables|Default|GetFullAppearance))))))
  (Utilities|Array|SetArrayElem (Variables|Default|GetAppearancesStack) 0 _output_get))
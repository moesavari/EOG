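; BPFL_Lib is a small general-purpose helper function library in MMOKit's logic layer.
; It offers validity-guarded component destruction and widget removal, plus integer formatting as comma-separated lists or zero-padded two-digit time strings.
; FindDiff copies two collections into sets and returns, as an array, the items in the old collection that are missing from the new one.
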(fn DestroyComponentifValid
  (params (Component :type Actor%20Component%20Object%20Reference))
  (Utilities|IsValid Component
    (:Is%20Valid
      (Components|DestroyComponent Component))))

(fn RemoveifValid
  (params (Widget :type Widget%20Object%20Reference))
  (Utilities|IsValid Widget
    (:Is%20Valid
      (Widget|RemovefromParent Widget))))

(fn FindDiff
  (params (OldCollection :type Array%20of%20Primary%20Asset%20Id%20Structures) (NewCollection :type Array%20of%20Primary%20Asset%20Id%20Structures))
  (Utilities|Set|AddItems (LocalVariables|GetOldCollectionAsSet) OldCollection)
  (Utilities|Set|AddItems (LocalVariables|GetNewCollectionAsSet) NewCollection)
  (bind _result (Utilities|Set|Difference (LocalVariables|GetOldCollectionAsSet) (LocalVariables|GetNewCollectionAsSet)))
  (bind _result_2 (Utilities|Set|ToArray _result))
  (return _result_2))

(fn IntArraytoString
  (params (IntArr :type Array%20of%20Integers))
  (for (_array_element _array_index) IntArr
    (LocalVariables|SetResult (Utilities|String|SelectString (Utilities|String|Append (LocalVariables|GetResult) (Utilities|String|ToString(Integer) _array_element)) (Utilities|String|Append (LocalVariables|GetResult) (Utilities|String|ToString(Integer) _array_element) ", ") (== _array_index (- (Utilities|Array|Length IntArr) 1)))))
  (return (LocalVariables|GetResult)))

(fn FormatInttoTwoDigits
  (params (Int :type Integer))
  ;[1 0.312 0.302] Turns "1" into "01" for the purpose of time display, e.g. 01:30
  (LocalVariables|SetResult (Utilities|String|ToString(Integer) Int))
  (if (== (Utilities|String|Len (LocalVariables|GetResult)) 1)
    (return (Utilities|String|Append "0" (LocalVariables|GetResult)))
    (else
      (return (LocalVariables|GetResult)))))
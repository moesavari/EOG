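; BuffAsset is a data asset defining a buff for the MMOKit, exposing its effects and duration for a given instigator.
; GetEffects merges effects computed by an optional BuffDynamics object with the static effects list, logging a mistake if that object only derives from BuffDynamicsCpp.
; GetDuration prefers a successful dynamic duration and falls back to the static one, where negative means permanent and zero means apply then immediately end.
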(fn GetEffects
  (params (Instigator :type Character%20Object%20Reference))
  ;[0.7865 0.1065 0.7201] Combine static effects from the BuffAsset with dynamic effects from BuffDynamics
  (Utilities|FlowControl|Sequence
    (:then_0
      (Utilities|IsValid (Variables|Default|GetBuffDynamics)
        (:Is%20Valid
          (bind _asbuff_dynamics (Utilities|Casting|CastToBuffDynamics (Variables|Default|GetBuffDynamics))
            (:then
              (bind _effects (Default|GetDynamicEffects _asbuff_dynamics Instigator))
              (for _array_element _effects
                (Utilities|Array|Add (LocalVariables|GetResult) _array_element)))
            (:CastFailed
              (Class|MmoUtilities|LogString (Variables|Default|GetBuffDynamics) (Utilities|String|ToString(Text) (Utilities|Text|FormatText "BuffDynamics in {name}(BuffAsset) wasn't inherited from BuffDynamics, but probably from BuffDynamicsCpp. This is a mistake." (Variables|Other|GetBuffName))) "Verbosity_Normal" true true "(R=1.000000,G=0.000000,B=0.058691,A=1.000000)" 5.0))))))
    (:then_1
      (for _array_element_2 (Variables|Statics|GetStaticEffects)
        (Utilities|Array|Add (LocalVariables|GetResult) _array_element_2)))
    (:then_2
      (return (LocalVariables|GetResult)))))

(fn GetDuration
  (params (Instigator :type Character%20Object%20Reference))
  ;[0.7865 0.1065 0.7201] Returns Dynamic Duration if it's defined
  ; If dynamic is not found/defined, use static duration
  ; Negative duration means it's a permanent duration, be careful with it
  ; Duration zero means the buff is applied and immediately removed, triggering both OnBuffApply and OnBuffEnd
  (Utilities|IsValid (Variables|Default|GetBuffDynamics)
    (:Is%20Valid
      (bind _asbuff_dynamics (Utilities|Casting|CastToBuffDynamics (Variables|Default|GetBuffDynamics))
        (:then
          (bind (_duration _success) (Default|GetDynamicDuration _asbuff_dynamics Instigator))
          (return (Math|Float|SelectFloat _duration (Variables|Statics|GetStaticDuration) _success)))
        (:CastFailed
          _)))
    (:Is%20Not%20Valid
      _))
  (return (Variables|Statics|GetStaticDuration)))
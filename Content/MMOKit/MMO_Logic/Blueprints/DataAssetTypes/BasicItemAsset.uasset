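; BasicItemAsset is an MMOKit item data asset Blueprint that answers queries about an item's price, sellability and meshes.
; GetPrice and IsSellable search the Properties array for a Sellable entry, so selling is a composable property, with zero or false when none is found.
; The mesh getters report no skeletal mesh and supply SM_Bag as the static mesh.
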(fn GetPrice
  (for _array_element (Variables|Default|GetProperties)
    (bind _assellable (Utilities|Casting|CastToSellable _array_element))
    (return (Variables|/Game/MMOKit/MMO_Logic/Blueprints/DataAssetTypes/ItemProperties/Sellable.Sellable_C|GetPrice _assellable)))
  (return 0))

(fn IsSellable
  (for _array_element (Variables|Default|GetProperties)
    (Utilities|Casting|CastToSellable _array_element)
    (return true))
  (return false))

(fn GetSkelMesh
  (return 0 false))

(fn GetStatMesh
  (return "/Game/MMOKit/MMO_Assets/Bag/SM_Bag.SM_Bag" true))
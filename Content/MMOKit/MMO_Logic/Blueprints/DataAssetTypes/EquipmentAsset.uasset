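; EquipmentAsset is a data asset type that describes a piece of equipment in the MMOKit game, exposing its meshes and gameplay properties.
; GetWeaponStats scans the Properties array for a WeaponProperty, using casts to pick out weapon data, and reports whether one was found.
; GetSkelMesh and GetStatMesh return soft references to the skeletal and static meshes, each with a flag showing whether the reference is valid.
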(fn GetWeaponStats
  (for _array_element (Variables|Default|GetProperties)
    (bind _asweapon_property (Utilities|Casting|CastToWeaponProperty _array_element))
    (return _asweapon_property true))
  (return 0 false))

(fn GetSkelMesh
  (bind _skelmesh (Variables|Equipment|GetSkelMesh))
  (return _skelmesh (Utilities|IsValidSoftObjectReference _skelmesh)))

(fn GetStatMesh
  (bind _statmesh (Variables|Equipment|GetStatMesh))
  (return _statmesh (Utilities|IsValidSoftObjectReference _statmesh)))
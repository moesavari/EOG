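; Server-only actor component that persists its owning actor to the database through the GameMode's persistency manager.
; On BeginPlay in a Ready world it requests a unique ID and saves; world-restore spawns stay passive, and destruction removes the record.
; It caches class, transform, update policy and serialized SaveGame properties, comparing rebuilds to detect changes.
; Update policy controls registration for automatic updates; restoring deserializes into the owner and notifies it.
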(event EventBeginPlay
  ;[0.4452 0.6332 1] At BeginPlay, the component will:
  ; - add itself to the list in gamemode, so we can iterate over all PersistencyComponents easily
  ; - if id <0, request a new id (if we're in an Initialized world, the gamemode will give you a new id. otherwise, it won't, because this Component was created by the GameMode spawner and the component's data will be populated)
  ; - request to be saved in DB (if we're in an Initialized world, that is. If we're in pre-initialized world, it means we just got spawned by GameMode from DB, so we're already in DB).
  ; So to sum it up, there's two behaviors here. One is when the object just got added during gameplay and needs to be saved, and the other is when the object just got added during the Initialization of the world,
  ; which means it comes from the DB and must act in a passive way, because it's being initialized externally.
  (Networking|CanExecuteCosmeticEvents
    (:True
      ;;[1 0.312 0.302] don't need it on clients
      (Components|DestroyComponent))
    (:False
      (if (> (Utilities|Array|Length (Actor|GetComponentsByClass (Components|GetOwner) "BP_PersistencyComponent_C")) 1)
        (Class|MmoUtilities|LogString "Error in your code! More than one Persistency Component on an object. Deleting redundant component. Fix your code." "Verbosity_Normal" true true "(R=1.000000,G=0.000000,B=0.026156,A=1.000000)" 1e+01)
        (Components|DestroyComponent)
        (else
          (Utilities|FlowControl|Sequence
            (:then_0
              (switch Utilities|FlowControl|Switch|SwitchonEPersistentObjUpdatePolicy (Variables|Default|GetUpdatePolicy)
                (:NewEnumerator1
                  (bind _manager (Class|BPIGameMode|GetPersistencyManager(Message) (Game|GetGameMode)))
                  (Default|RegisterPersistentObjectforUpdates _manager self))))
            (:then_1
              (bind _state (Class|BPIGameMode|GetServerState(Message) (Game|GetGameMode)))
              (if (and (< (Variables|Default|GetUniqueId) 0) (Utilities|Enum|Equal(Enum) _state "NewEnumerator1")) ; - if we're in Ready server state, request the new unique ID, because this is a new object that just got spawned by gameplay\n- if we're in pre-Initialized server state, we don't need to request anything, because this object is being spawned\nby game mode from DB and will initialize its ID itself\n- if we have a valid id (>= 0), then we don't need to request anything anyway
                (bind _manager_2 (Class|BPIGameMode|GetPersistencyManager(Message) (Game|GetGameMode)))
                (bind _id (Default|RequestPersistencyId _manager_2))
                (Variables|Default|SetUniqueId _id)))
            (:then_2
              (bind _state_2 (Class|BPIGameMode|GetServerState(Message) (Game|GetGameMode)))
              (if (Utilities|Enum|Equal(Enum) _state_2 "NewEnumerator1") ; Request to serialize and save the object in DB,\nbut only if we've finished initializing the world,\nbecause otherwise it means the object is currently being \nRESTORED from db, and therefore doesn't need to be saved in it
                (bind _manager_3 (Class|BPIGameMode|GetPersistencyManager(Message) (Game|GetGameMode)))
                (Default|AddorUpdatePersistentObjectinDB _manager_3 self)))))))))

(event EventEndPlay
  (params (EndPlayReason :type EEndPlayReason%20Enum :default "Destroyed"))
  ;[0.4452 0.6332 1] OnDestroy, ask the item to be removed from DB
  (Networking|CanExecuteCosmeticEvents
    (:False
      (switch Utilities|FlowControl|Switch|SwitchonEEndPlayReason EndPlayReason
        (:Destroyed
          (bind _state (Class|BPIGameMode|GetServerState(Message) (Game|GetGameMode)))
          (switch Utilities|FlowControl|Switch|SwitchonEServerState _state
            (:NewEnumerator1
              (if (>= (Variables|Default|GetUniqueId) 0)
                (bind _manager (Class|BPIGameMode|GetPersistencyManager(Message) (Game|GetGameMode)))
                (Default|RemovePersistentObjectinDB _manager self)))))))))

(fn GetSerializedParent
  (bind _uniqueid (Variables|Default|GetUniqueId))
  ;[0.4452 0.6332 1] Returns a serialized parent of this component, ready to be saved to DB
  (if (Utilities|Array|IsEmpty (Utilities|Struct|BreakFPersistentObject (Variables|Default|GetCachedParent))) ; If there's no serialized and cached parent, rebuild the cache now
    (bind _success (CallFunction|SerializeParent))
    (if _success
      _
      (else
        (return false 0 ""))))
  (return (>= _uniqueid 0) _uniqueid (Variables|Default|GetCachedParent)))

(fn DeserializeIntoParent
  (params (Id :type Integer) (Bytes :type Array%20of%20Bytes))
  (bind _returnvalue (Components|GetOwner))
  ;[0.4452 0.6332 1] Takes bytes from the DB and populates the parent with its properties that are marked as "SaveGame"
  (Variables|Default|SetUniqueId Id)
  (Class|MmoUtilities|DeserializeObject _returnvalue Bytes)
  (Class|BPIPersistentActor|OnPropertiesRestored(Message) _returnvalue))

(fn InitializeUpdatePolicy
  (params (UpdatePolicy :type EPersistentObjUpdatePolicy%20Enum :default "NewEnumerator0"))
  ;[0.4452 0.6332 1] Initialize Update Policy
  ; It's used when we spawned an actor with an attached Persistency component
  ; The attached persistency component doesn't have policy exposed on spawn, so
  ; we update it right after spawning it.
  ; The function "ChangeUpdatePolicy" is different, because changing the policy during gameplay may require an immediate db update (if we're turning off auto-updates for the component)
  (bind _output_get (Variables|Default|SetUpdatePolicy UpdatePolicy))
  (bind _manager (Class|BPIGameMode|GetPersistencyManager(Message) (Game|GetGameMode)))
  (switch Utilities|FlowControl|Switch|SwitchonEPersistentObjUpdatePolicy _output_get
    (:NewEnumerator0
      (Default|UnregisterPersistentObjectforUpdates _manager self))
    (:NewEnumerator1
      (Default|RegisterPersistentObjectforUpdates _manager self))))

(fn HasChanged
  (bind _cachedparent (Variables|Default|GetCachedParent))
  (bind (_transform _updatepolicy _properties) (Utilities|Struct|BreakFPersistentObject _cachedparent))
  ;[0.4452 0.6332 1] Rebuilds cache and checks against the previous version
  ; If there are differences, returns true.
  ; We skip ClassName in the struct, because it can't change.
  (if (Utilities|Array|IsEmpty (Utilities|Struct|BreakFPersistentObject (Variables|Default|GetCachedParent)))
    (CallFunction|SerializeParent) ; If we're serializing for the first time and have no previous version, simply serialize and report no changes
    (return false)
    (else
      (bind _output_get (LocalVariables|SetCacheBeforeRebuild (Variables|Default|GetCachedParent)))
      (bind _success (CallFunction|SerializeParent)) ; Rebuilds "CachedParent", so now we can comare\nthe previous version with the current one
      (if _success
        (if (Math|Boolean|ANDBoolean (== (.Transform (Utilities|Struct|BreakFPersistentObject _output_get)) _transform) (Utilities|Enum|Equal(Enum) (.UpdatePolicy (Utilities|Struct|BreakFPersistentObject _output_get)) _updatepolicy) (== (Utilities|Array|Length (.Properties (Utilities|Struct|BreakFPersistentObject _output_get))) (Utilities|Array|Length _properties)))
          (for (_array_element _array_index) (.Properties (Utilities|Struct|BreakFPersistentObject _output_get))
            (if (!= _array_element (Utilities|Array|Get(acopy) _properties _array_index))
              (return true)))
          (return false)
          (else
            (return true)))
        (else
          (return false))))))

(fn SerializeParent
  (bind _returnvalue (Components|GetOwner))
  ;[0.4452 0.6332 1] This serializes the parent and stores it in a cached variable
  ; The first time it's serialized, we'll send it to DB
  ; Afterwards, we'll re-serialize it and compare it to the previous version, to see if changes occured
  (Utilities|IsValid _returnvalue
    (:Is%20Valid
      (bind _returnvalue_2 (Class|MmoUtilities|SerializeObject (Components|GetOwner)))
      (Variables|Default|SetCachedParent (Utilities|Struct|MakeFPersistentObject (Utilities|BreakSoftClassPath (Class|KismetSystemLibrary|GetSoftClassPath (Utilities|GetClass _returnvalue))) (Transformation|GetActorTransform _returnvalue) (Variables|Default|GetUpdatePolicy) _returnvalue_2))
      (return true))
    (:Is%20Not%20Valid
      (Class|MmoUtilities|LogString "Rebuild cache failed: no owner?" "Verbosity_Normal" true true "(R=1.000000,G=0.000000,B=0.008162,A=1.000000)" 5.0)
      (return false))))

(fn ShouldUpdateAutomatically
  (if (< (Variables|Default|GetUniqueId) 0)
    (return false)
    (else
      (return (Utilities|Enum|Equal(Enum) (Variables|Default|GetUpdatePolicy) "NewEnumerator1")))))

(fn ChangeUpdatePolicy
  (params (UpdatePolicy :type EPersistentObjUpdatePolicy%20Enum :default "NewEnumerator0"))
  ;[0.4452 0.6332 1] Change Update Policy during gameplay
  (bind _output_get (Variables|Default|SetUpdatePolicy UpdatePolicy))
  (bind _manager (Class|BPIGameMode|GetPersistencyManager(Message) (Game|GetGameMode)))
  (switch Utilities|FlowControl|Switch|SwitchonEPersistentObjUpdatePolicy _output_get
    (:NewEnumerator0
      (Default|UnregisterPersistentObjectforUpdates _manager self)
      (Default|AddorUpdatePersistentObjectinDB _manager self))
    (:NewEnumerator1
      (Default|RegisterPersistentObjectforUpdates _manager self))))
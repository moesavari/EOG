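; Server-side persistency manager component that spawns saved objects from the database and writes changes back.
; Async-loads and spawns objects from JSON, restores their BP_PersistencyComponent, and updates server readiness once the expected count is spawned.
; Tick checks one component per frame from a snapshot of auto-updated objects, saving only changed ones and sleeping while none are registered.
; Also issues new object IDs and deletes records by saving empty objects.
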(event Custom|ResetPassThroughArray
  ;[0.4452 0.6332 1] Reset passthrough
  (if (> (Utilities|Set|Length (Variables|Default|GetAutoUpdatedObjects)) 0)
    (Components|Tick|SetComponentTickEnabled true)
    (bind _result (Utilities|Set|ToArray (Variables|Default|GetAutoUpdatedObjects)))
    (Variables|Default|SetPassThroughObjects _result)
    (Variables|Default|SetPassThroughIterator 0)
    (else
      (Components|Tick|SetComponentTickEnabled false)
      (Utilities|FlowControl|Delay 1e+01)
      (CallFunction|ResetPassThroughArray))))

(event EventTick
  (params (DeltaSeconds :type Float%20%28single-precision%29))
  ;[0.4452 0.6332 1] Tick is turned off by default in this class.
  ; Only ticks when there are objects to treat.
  (CallFunction|TickPassThrough))

(event EventRegisterPersistentObjectforUpdates
  (params (ComponentRef :type BP%20Persistency%20Component%20Object%20Reference))
  ;[0.4452 0.6332 1] Register Persistent Object for Updates
  (Utilities|Set|Add (Variables|Default|GetAutoUpdatedObjects) ComponentRef))

(event EventUnregisterPersistentObjectforUpdates
  (params (ComponentRef :type BP%20Persistency%20Component%20Object%20Reference))
  ;[0.4452 0.6332 1] Unregister Persistent Object from Updates
  (Utilities|Set|Remove (Variables|Default|GetAutoUpdatedObjects) ComponentRef))

(event EventRemovePersistentObjectinDB
  (params (ComponentRef :type BP%20Persistency%20Component%20Object%20Reference))
  ;[0.4452 0.6332 1] Delete Persistent Object from DB
  (CallFunction|UnregisterPersistentObjectforUpdates ComponentRef)
  (bind _tcpconn (Class|BPIGameState|GetTcpConnection(Message) (Game|GetGameState)))
  (Default|SavePersistentObject _tcpconn (Variables|/Game/MMOKit/MMO_Logic/Blueprints/Persistency/BP_PersistencyComponent.BP_PersistencyComponent_C|GetUniqueId ComponentRef) (Utilities|Struct|MakeFPersistentObject)))

(event EventSetPersistentObjectstoSpawn
  (params (ObjCount :type Integer))
  ;[0.4452 0.6332 1] Set Persistent Objects to Spawn
  ; (received from ServerLogin response)
  (bind _output_get (Variables|Default|SetObjectsToSpawn ObjCount))
  (if (== _output_get 0)
    (Class|BPIGameMode|UpdateServerReadiness(Message) (Game|GetGameMode)) ; if we're going to spawn 0 persistent objects, \nwe won't receive any persistent objects and won't have an opportunity to trigger a check,\nso check if we're ready now
    (CallFunction|ResetPassThroughArray)))

(event EventAddorUpdatePersistentObjectinDB
  (params (ComponentRef :type BP%20Persistency%20Component%20Object%20Reference))
  ;[0.4452 0.6332 1] Add Or Update Persistent object in DB
  (bind (_success _uniqueid _persistentobject) (Default|GetSerializedParent ComponentRef))
  (if _success
    (bind _tcpconn (Class|BPIGameState|GetTcpConnection(Message) (Game|GetGameState)))
    (Default|SavePersistentObject _tcpconn _uniqueid _persistentobject)))

(event EventSpawnPersistentObject
  (params (ObjId :type Integer) (JsonString :type String))
  ;[0.4452 0.6332 1] Spawn Persistent Object from DB
  ; If Persistence Server has restarted during gameplay, we don't spawn persistent objects again.
  (bind _serverstate (Class|BPIGameMode|GetServerReadiness(Message) (Game|GetGameMode)))
  (if (Utilities|Enum|Equal(Enum) _serverstate "NewEnumerator0")
    (bind _outjsonobject (Class|JsonBlueprintFunctionLibrary|FromString JsonString))
    (bind _outvalue (|GetJsonField _outjsonobject "Obj"))
    (if (Utilities|IsValidSoftClassReference (Class|KismetSystemLibrary|ToSoftClassRef(SoftClassPath) (Class|KismetSystemLibrary|MakeSoftClassPath (Utilities|Struct|BreakFPersistentObject _outvalue))))
      (bind (_class _objectid _jsonobject) (|AsyncLoadPersistentClass (Class|KismetSystemLibrary|ToSoftClassRef(SoftClassPath) (Class|KismetSystemLibrary|MakeSoftClassPath (Utilities|Struct|BreakFPersistentObject _outvalue))) ObjId _outjsonobject)
        (:Completed
          (bind _outvalue_2 (|GetJsonField _jsonobject "Obj"))
          (bind _asactor (Utilities|Casting|CastToActorClass _class))
          (bind _returnvalue (Game|SpawnActorfromClass _asactor (.Transform (Utilities|Struct|BreakFPersistentObject _outvalue_2)) "AdjustIfPossibleButAlwaysSpawn" "SelectDefaultAtRuntime" 0 0))
          (Utilities|IsValid (Actor|GetComponentbyClass _returnvalue "/Game/MMOKit/MMO_Logic/Blueprints/Persistency/BP_PersistencyComponent.BP_PersistencyComponent_C")
            (:Is%20Valid
              (Default|InitializeUpdatePolicy (Actor|GetComponentbyClass _returnvalue "/Game/MMOKit/MMO_Logic/Blueprints/Persistency/BP_PersistencyComponent.BP_PersistencyComponent_C") (.UpdatePolicy (Utilities|Struct|BreakFPersistentObject _outvalue_2)))
              (Default|DeserializeIntoParent (Actor|GetComponentbyClass _returnvalue "/Game/MMOKit/MMO_Logic/Blueprints/Persistency/BP_PersistencyComponent.BP_PersistencyComponent_C") _objectid (.Properties (Utilities|Struct|BreakFPersistentObject _outvalue_2))))
            (:Is%20Not%20Valid
              (bind _returnvalue_2 (Game|AddComponentbyClass _returnvalue "/Game/MMOKit/MMO_Logic/Blueprints/Persistency/BP_PersistencyComponent.BP_PersistencyComponent_C" (.UpdatePolicy (Utilities|Struct|BreakFPersistentObject _outvalue_2))))
              (Default|DeserializeIntoParent _returnvalue_2 _objectid (.Properties (Utilities|Struct|BreakFPersistentObject _outvalue_2)))))
          (Math|Integer|IncrementInt (Variables|Default|GetObjectsSpanwedFromDb)
            (:%20%20
              (if (>= _objectid (Variables|Default|GetNextIdForNewObject))
                (Variables|Default|SetNextIdForNewObject (+ _objectid 1)))
              (bind _finished (CallFunction|IsFinishedSpawningObjects))
              (if _finished
                (Class|BPIGameMode|UpdateServerReadiness(Message) (Game|GetGameMode))
                (CallFunction|ResetPassThroughArray))))))
      (else
        (Class|MmoUtilities|LogString (Utilities|String|Append "Async load class failed: " (Utilities|Struct|BreakFPersistentObject _outvalue)) "Verbosity_Normal" true true "(R=1.000000,G=0.000000,B=0.000000,A=1.000000)" 5.0)))))

(fn TickPassThrough
  (Utilities|FlowControl|Sequence
    (:then_0
      (bind _output_get (LocalVariables|SetPersistentComp (Utilities|Array|Get(acopy) (Variables|Default|GetPassThroughObjects) (Variables|Default|GetPassThroughIterator))))
      (Utilities|IsValid _output_get
        (:Is%20Valid
          (bind _should (Default|ShouldUpdateAutomatically (LocalVariables|GetPersistentComp))) ; it's possible the component has been removed from\nauto-updates while we were getting to it,\nso we skip it
          (if _should
            (bind _changed (Default|HasChanged (LocalVariables|GetPersistentComp))) ; reserialize the component and check\nagainst the cached version
            (if _changed
              (CallFunction|AddorUpdatePersistentObjectinDB (LocalVariables|GetPersistentComp)) ; if it has changed, send the latest serialized version to DB
              (Class|MmoUtilities|LogString "Persistency Object changed: updating in db" "Verbosity_SuperVerbose"))))))
    (:then_1
      (Math|Integer|IncrementInt (Variables|Default|GetPassThroughIterator)
        (:%20%20
          (if (>= (Variables|Default|GetPassThroughIterator) (Utilities|Array|Length (Variables|Default|GetPassThroughObjects)))
            (Utilities|Array|Clear (Variables|Default|GetPassThroughObjects))
            (CallFunction|ResetPassThroughArray)))))))

(fn IsFinishedSpawningObjects
  ;[0.4452 0.6332 1] by default, persistent objects to spawn is equal to -1
  ; when we connect to PS, we receive its true number and it'll be 0 or higher
  ; when the two ints are equal, we have spawned all we needed to spawn
  (return (== (Variables|Default|GetObjectsToSpawn) (Variables|Default|GetObjectsSpanwedFromDb))))

(fn RequestPersistencyId
  (bind _nextidfornewobject (Variables|Default|GetNextIdForNewObject))
  (LocalVariables|SetResult _nextidfornewobject)
  (Math|Integer|IncrementInt _nextidfornewobject
    (:%20%20
      (return (LocalVariables|GetResult)))))
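; Server game mode for the MMO kit that bridges players and the Persistence Server over a TCP connection held by GameState.
; It preloads primary assets into memory, becoming Ready once those, the connection and persistent-object respawning finish.
; Queued controllers receive DB characters in request order, and online maps support lookup, save and kick.
; It also spawns delayed mob spawners, diffs party updates for members, and syncs party health on a timer.
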(event Custom|SaveAllCharacters
  ;[0.4452 0.6332 1] Save All Characters
  (Class|MmoUtilities|LogString "Saving All Characters" "Verbosity_SuperVerbose")
  (for _index (range 0 (- (Class|GameplayStatics|GetNumPlayerControllers) 1))
    (Class|BPIPlayerController|ForceSaveCharacter(Message) (Game|GetPlayerController _index))))

(event EventBeginPlay
  ;[0.4452 0.6332 1] Server-side: Load assets and keep them in memory by referencing them in the game mode
  (Utilities|FlowControl|Sequence
    (:then_0
      (Class|MmoUtilities|LogString "BeginPlay: GameMode" "Verbosity_SuperVerbose")
      (for _array_element (Variables|Default|GetPrimaryTypesToLoad) ; loads items/equipment into server memory on start\nloads AbilityAssets\nloads CreatureAppearances
        (bind _outprimaryassetidlist (Class|KismetSystemLibrary|GetPrimaryAssetIdList _array_element))
        (bind _loaded (|AsyncLoadPrimaryAssetList _outprimaryassetidlist)
          (:Completed
            (for _array_element_2 _loaded
              (bind _asitem_asset (Utilities|Casting|CastToItemAsset _array_element_2)
                (:then
                  (Utilities|Array|Add (Variables|Default|GetLoadedItems) _asitem_asset)
                  (Class|MmoUtilities|LogString (Utilities|String|Append "Server Loaded Item: " (Utilities|String|ToString(Text) (Variables|/Script/MMOKitCode.ItemAsset|GetItemName _asitem_asset))) "Verbosity_SuperVerbose"))
                (:CastFailed
                  (bind _asability_asset (Utilities|Casting|CastToAbilityAsset _array_element_2)
                    (:then
                      (Utilities|Array|Add (Variables|Default|GetLoadedAbilities) _asability_asset)
                      (Class|MmoUtilities|LogString (Utilities|String|Append "Server Loaded Ability: " (Utilities|GetObjectName _asability_asset)) "Verbosity_SuperVerbose"))
                    (:CastFailed
                      (bind _ascreature_appearance (Utilities|Casting|CastToCreatureAppearance _array_element_2)
                        (:then
                          (Utilities|Array|Add (Variables|Default|GetLoadedAppearances) _ascreature_appearance)
                          (Class|MmoUtilities|LogString (Utilities|String|Append "Server Loaded Appearance: " (Utilities|GetObjectName _ascreature_appearance)) "Verbosity_SuperVerbose"))
                        (:CastFailed
                          (bind _asbuff_asset (Utilities|Casting|CastToBuffAsset _array_element_2))
                          (Utilities|Array|Add (Variables|Default|GetLoadedBuffs) _asbuff_asset)
                          (Class|MmoUtilities|LogString (Utilities|String|Append "Server Loaded Buff: " (Utilities|GetObjectName _asbuff_asset)) "Verbosity_SuperVerbose"))))))))
            (Math|Integer|IncrementInt (Variables|ServerReadiness|GetPrimaryAssetTypesLoaded)
              (:%20%20
                (CallFunction|UpdateServerReadiness)))))))
    (:then_1
      ;;[1 0.312 0.302] If launching the project in an incorrect mode (standalone or listen server), display a warning for user
      (if (and (Networking|IsServer) (not (Networking|IsDedicatedServer)))
        (Utilities|FlowControl|Delay 1.0)
        (Class|BPIPlayerController|DisplayEditorWarning3(Message) (Game|GetPlayerController 0))))
    (:then_2
      ;;[0.4452 0.6332 1] Send Party Members Info to PS every 2 seconds
      (Utilities|Time|SetTimerbyEvent (EventDispatchers|CreateEvent :!event SyncPartyMembersInfo) 2.0 true))))

(event EventSaveCharacter
  (params (ChId :type Integer) (Json :type Json%20Object%20Wrapper%20Structure))
  ;[0.4452 0.6332 1] Save Character - gets called from PlayerController
  (bind _tcpconn (Class|BPIGameState|GetTcpConnection(Message) (Game|GetGameState)))
  (Default|SaveCharacter _tcpconn ChId Json))

(event EventUpdateServerReadiness
  ;[0.4452 0.6332 1] Try to update server readiness. It's ready when:
  ; - all assets are loaded
  ; - a websocket connection with Persistence Server is established
  ; - all persistent objects (acquired from DB) have been respawned
  (switch Utilities|FlowControl|Switch|SwitchonEServerState (Variables|ServerReadiness|GetServerState)
    (:NewEnumerator0
      (bind _tcpconn (Class|BPIGameState|GetTcpConnection(Message) (Game|GetGameState)))
      (Utilities|IsValid _tcpconn
        (:Is%20Valid
          (bind _manager (CallFunction|GetPersistencyManager))
          (bind _finished (Default|IsFinishedSpawningObjects _manager))
          (switch Utilities|FlowControl|Switch|SwitchonEServerState (select (Math|Boolean|ANDBoolean (Class|WebSocketConn|IsConnected _tcpconn) (== (Variables|ServerReadiness|GetPrimaryAssetTypesLoaded) (Utilities|Array|Length (Variables|Default|GetPrimaryTypesToLoad))) _finished) "NewEnumerator1" "NewEnumerator0")
            (:NewEnumerator1
              (Variables|ServerReadiness|SetServerState (select (Math|Boolean|ANDBoolean (Class|WebSocketConn|IsConnected _tcpconn) (== (Variables|ServerReadiness|GetPrimaryAssetTypesLoaded) (Utilities|Array|Length (Variables|Default|GetPrimaryTypesToLoad))) _finished) "NewEnumerator1" "NewEnumerator0"))
              (Class|MmoUtilities|LogString "Server is ready to accept players" "Verbosity_Normal" false true "(R=0.000000,G=1.000000,B=0.008096,A=1.000000)"))))))))

(event EventDisconnectCharId
  (params (CharId :type Integer))
  (bind _characteridsonline (Variables|Default|GetCharacterIdsOnline))
  (bind (_value _returnvalue) (Utilities|Map|Find _characteridsonline CharId))
  (bind _returnvalue_2 (Pawn|GetController _value))
  ;[0.4452 0.6332 1] Disconnect Char Id
  (if _returnvalue
    (Class|BPIPlayerController|ForceSaveCharacter(Message) _returnvalue_2)
    (Class|GameModeBaseCpp|KickPlayer (.AsPlayer%20Controller (Utilities|Casting|CastToPlayerController _returnvalue_2)))))

(event EventUpdateFullPartyInfo
  (params (PartyInfo :type F%20Party%20Structure))
  (CallFunction|ProcessPartyInfoUpdate PartyInfo))

(event EventSetServerInfofromJson
  (params (JsonString :type String))
  ;[0.4452 0.6332 1] Set Server Info from Json
  ; (received from ServerLogin response)
  (bind _outjsonobject (Class|JsonBlueprintFunctionLibrary|FromString JsonString))
  (CallFunction|OnServerInfoReceived _outjsonobject))

(event EventOnEndPIE
  ;[0.4452 0.6332 1] OnEndPIE gets fired only in Editor
  ; In a regular game, PlayerController::OnUnPossess will save the exiting character
  ; But in Editor, UnPossess will fire so late,  that our WebSocket connection will already be closed
  ; So we attempt to save characters as soon as End PIE is detected
  (Variables|ServerReadiness|SetServerState "NewEnumerator2")
  (CallFunction|SaveAllCharacters))

(event EventSpawnMobAfterDelay
  (params (RespawnPoint :type Transform) (MobClass :type BP%20Mob%20Character%20Class%20Reference) (Stats :type F%20Stats%20Mob%20Structure) (Delay :type Float%20%28double-precision%29) (Loot :type F%20Mob%20Loot%20Structure) (BT :type Behavior%20Tree%20Object%20Reference))
  ;[0.4452 0.6332 1] Spawn mob after a delay
  (Game|SpawnActorfromClass "/Game/MMOKit/MMO_Logic/Blueprints/Misc/BP_MobSpawner.BP_MobSpawner_C" RespawnPoint "AlwaysSpawn" "OverrideRootScale" 0 MobClass Stats Delay Loot BT 0))

(event EventGetCharacterforController
  (params (PlayerController :type Player%20Controller%20Object%20Reference) (Cookie :type String) (CharID :type Integer))
  ;[0.4452 0.6332 1] This all has to do with when we GetCharacter from Persistence server
  (Utilities|Array|Add (Variables|Default|GetGetCharacterQueue) PlayerController)
  (bind _tcpconn (Class|BPIGameState|GetTcpConnection(Message) (Game|GetGameState)))
  (Default|GetCharacter _tcpconn Cookie CharID)
  ;[1 1 1] Editor only: display warning if user hasn't launched the persistence server
  (bind _returnvalue (Class|MmoUtilities|InPieWorld))
  (if _returnvalue
    (if (not (Class|WebSocketConn|IsConnected _tcpconn))
      (Class|BPIPlayerController|DisplayEditorWarning1(Message) PlayerController))))

(event EventFailedGettingCharacterforController
  (bind _getcharacterqueue (Variables|Default|GetGetCharacterQueue))
  (bind _getcharacterqueue_2 (Variables|Default|GetGetCharacterQueue))
  ;[0.4452 0.6332 1] This all has to do with when we GetCharacter from Persistence server
  (bind _returnvalue (Class|MmoUtilities|InPieWorld))
  (if _returnvalue
    ;;[1 1 1] in editor, display a warning that there's not enough characters in DB
    (Class|BPIPlayerController|DisplayEditorWarning2(Message) (Utilities|Array|Get(acopy) _getcharacterqueue))
    (Utilities|Array|RemoveIndex _getcharacterqueue)
    (else
      ;;[0.4452 0.6332 1] in prod, disconnect player
      (Actor|DestroyActor (Utilities|Array|Get(acopy) _getcharacterqueue_2))
      (Utilities|Array|RemoveIndex _getcharacterqueue_2))))

(event EventGotCharacterforController
  (params (AccountID :type Integer) (CharID :type Integer) (CharName :type String) (Permissions :type Integer) (Serialized :type String) (GuildId :type Integer) (GuildRank :type Integer))
  (bind _getcharacterqueue (Variables|Default|GetGetCharacterQueue))
  ;[0.4452 0.6332 1] This all has to do with when we GetCharacter from Persistence server
  (bind _eventbus (Class|BPIPlayerController|GetPlayerControllerEventBus(Message) (Utilities|Array|Get(acopy) _getcharacterqueue)))
  (Default|CallOnGotCharacterfromDB _eventbus AccountID CharID CharName Permissions Serialized GuildId GuildRank)
  (Utilities|Array|RemoveIndex _getcharacterqueue))

(event EventContinuePlayerSpawn
  (params (PlayerController :type BP%20Player%20Controller%20Object%20Reference) (PlayerPawn :type Pawn%20Object%20Reference) (SpawnRotator :type Rotator :default "0, 0, 0"))
  ;[0.4452 0.6332 1] This all has to do with when we GetCharacter from Persistence server
  (Class|GameModeBaseCpp|ContinuePlayerStart PlayerController PlayerPawn SpawnRotator))

(event EventCharacterEnteredWorld
  (params (Name :type String) (Character :type Character%20Object%20Reference) (Id :type Integer))
  ;[0.4452 0.6332 1] On character entered/left world
  (Utilities|Map|Add (Variables|Default|GetCharactersOnline) Name Character)
  (Utilities|Map|Add (Variables|Default|GetCharacterIdsOnline) Id Character))

(event EventCharacterLeftWorld
  (params (Name :type String) (Id :type Integer))
  ;[0.4452 0.6332 1] On character entered/left world
  (Utilities|Map|Remove (Variables|Default|GetCharactersOnline) Name)
  (Utilities|Map|Remove (Variables|Default|GetCharacterIdsOnline) Id))

(fn ConstructionScript)

(fn SaveServerInfoinDB
  (LocalVariables|SetJsonObj (Utilities|Struct|MakeJsonObjectWrapper))
  (|SetJsonField (LocalVariables|GetJsonObj) "Info1" (Utilities|Struct|MakeFServerInfo 1))
  (bind _tcpconn (Class|BPIGameState|GetTcpConnection(Message) (Game|GetGameState)))
  (Default|SaveServerInfo _tcpconn (LocalVariables|GetJsonObj)))

(fn OnServerInfoReceived
  (params (JsonObj :type Json%20Object%20Wrapper%20Structure))
  (bind _returnvalue (Class|JsonBlueprintFunctionLibrary|HasField JsonObj "Info1"))
  (if _returnvalue
    (bind _outvalue (|GetJsonField JsonObj "Info1"))))

(fn ProcessPartyInfoUpdate
  (params (NewPartyInfo :type F%20Party%20Structure))
  (bind _parties (Variables|Default|GetParties))
  (bind _parties_2 (Variables|Default|GetParties))
  (bind _partyid (Utilities|Struct|BreakFParty NewPartyInfo))
  (bind (_partyid_2 _memberids) (Utilities|Struct|BreakFParty NewPartyInfo))
  (bind (_value _returnvalue) (Utilities|Map|Find _parties _partyid))
  ;[0.4452 0.6332 1] Does a diff between old members of this party and new ones.
  ; The ones who are no longer party members are leavers and we pass the info to their Controller and Character, so it's replicated down to Clients
  ; For others (who haven't left), we update the info and it too will be replicated to Clients
  ; Then we update the Parties map
  ; If there are no members in the party, remove it from Parties map
  (Utilities|FlowControl|Sequence
    (:then_0
      (if _returnvalue
        (LocalVariables|SetOldPartyInfo _value)
        (Utilities|Set|AddItems (LocalVariables|GetOldMemberIds) (Utilities|Struct|BreakFParty (LocalVariables|GetOldPartyInfo)))))
    (:then_1
      (Utilities|Set|AddItems (LocalVariables|GetNewMemberIds) (Utilities|Struct|BreakFParty NewPartyInfo)))
    (:then_2
      (bind _result (Utilities|Set|Difference (LocalVariables|GetOldMemberIds) (LocalVariables|GetNewMemberIds)))
      (bind _result_2 (Utilities|Set|ToArray _result))
      (for _array_element _result_2
        (if (.ReturnValue (Utilities|Map|Find (Variables|Default|GetCharacterIdsOnline) _array_element))
          (Class|BPIPlayerCharacterSpecific|SetinParty(Message) (.Value (Utilities|Map|Find (Variables|Default|GetCharacterIdsOnline) _array_element)) false)
          (Class|BPIPlayerController|SetPartyInfo(Message) (Pawn|GetController (.Value (Utilities|Map|Find (Variables|Default|GetCharacterIdsOnline) _array_element))) (Utilities|Struct|MakeFParty)))))
    (:then_3
      (for _array_element_2 (Utilities|Struct|BreakFParty NewPartyInfo)
        (if (.ReturnValue (Utilities|Map|Find (Variables|Default|GetCharacterIdsOnline) _array_element_2))
          (Class|BPIPlayerCharacterSpecific|SetinParty(Message) (.Value (Utilities|Map|Find (Variables|Default|GetCharacterIdsOnline) _array_element_2)) true)
          (Class|BPIPlayerController|SetPartyInfo(Message) (Pawn|GetController (.Value (Utilities|Map|Find (Variables|Default|GetCharacterIdsOnline) _array_element_2))) NewPartyInfo))))
    (:then_4
      (Utilities|Map|Remove _parties_2 _partyid_2)
      (if (> (Utilities|Array|Length _memberids) 0)
        (Utilities|Map|Add _parties_2 _partyid_2 NewPartyInfo)))))

(fn SyncPartyMembersInfo
  (bind _keys (Utilities|Map|Keys (Variables|Default|GetParties)))
  (for _array_element _keys
    (LocalVariables|SetPartyId _array_element)
    (Utilities|Array|Clear (LocalVariables|GetPartyMembers))
    (for _array_element_2 (Utilities|Struct|BreakFParty (.Value (Utilities|Map|Find (Variables|Default|GetParties) (LocalVariables|GetPartyId))))
      (bind _output_get (LocalVariables|SetCharId _array_element_2))
      (if (.ReturnValue (Utilities|Map|Find (Variables|Default|GetCharacterIdsOnline) _output_get))
        (bind _playerstats (Class|BPIPlayerCharacterSpecific|GetPlayerStats(Message) (.Value (Utilities|Map|Find (Variables|Default|GetCharacterIdsOnline) _output_get))))
        (Utilities|Array|Add (LocalVariables|GetPartyMembers) (Utilities|Struct|MakeFPartySyncOneMember (LocalVariables|GetCharId) (Variables|/Game/MMOKit/MMO_Logic/Blueprints/Stats/BP_BaseStatsComponent.BP_BaseStatsComponent_C|GetCurHp _playerstats) (Variables|/Game/MMOKit/MMO_Logic/Blueprints/Stats/BP_BaseStatsComponent.BP_BaseStatsComponent_C|GetMaxHp _playerstats)))))
    (if (> (Utilities|Array|Length (LocalVariables|GetPartyMembers)) 0)
      (Utilities|Array|Add (LocalVariables|GetPartiesInfo) (Utilities|Struct|MakeFPartySyncOneParty (LocalVariables|GetPartyId) (LocalVariables|GetPartyMembers)))))
  (bind _outjsonstring (|StructtoJsonString (Utilities|Struct|MakeFPartySyncFull (LocalVariables|GetPartiesInfo))))
  (bind _tcpconn (Class|BPIGameState|GetTcpConnection(Message) (Game|GetGameState)))
  (Default|SendPartyMembersUpdate _tcpconn _outjsonstring))

(fn GetPersistencyManager
  (return (Variables|Default|GetBP_PersistencyManager)))

(fn GetPlayerCharbyId
  (params (Id :type Integer))
  (bind _characteridsonline (Variables|Default|GetCharacterIdsOnline))
  (bind (_value _returnvalue) (Utilities|Map|Find _characteridsonline Id))
  (return _value _returnvalue))

(fn GetPlayerCharbyName
  (params (Charname :type String))
  (bind _charactersonline (Variables|Default|GetCharactersOnline))
  (bind (_value _returnvalue) (Utilities|Map|Find _charactersonline Charname))
  (return _value _returnvalue))

(fn GetServerPassword
  (return (Class|GameModeBaseCpp|ServerPassword)))

(fn GetServerReadiness
  (return (Variables|ServerReadiness|GetServerState)))

(fn GetServerState
  (return (Variables|ServerReadiness|GetServerState)))
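; BP_BaseStorageComponent is the base Blueprint component for slot-based item storage in the MMO inventory logic.
; It declares stub functions for accepting, finding, getting and removing items and for querying slots, all returning failure or empty defaults.
; The MaxSlots RepNotify calls EmitMaxSlotsChanged, which broadcasts the new slot count through OnMaxSlotsChanged.
; EmitContentUpdated is an empty event left for child classes to override.
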(event Custom|EmitMaxSlotsChanged
  (Default|CallOnMaxSlotsChanged (Variables|Default|GetMaxSlots)))

(event Custom|EmitContentUpdated)

(fn OnRepMaxSlots
  (CallFunction|EmitMaxSlotsChanged))

(fn AcceptsItem
  (params (Item :type Primary%20Asset%20Id%20Structure) (Slot :type Integer))
  (return false))

(fn FindItem
  (params (ItemId :type Primary%20Asset%20Id%20Structure))
  (return false 0 0))

(fn GetFirstAvailableSlot
  (return -1 false))

(fn GetItem
  (params (Slot :type Integer))
  (return "" 0))

(fn GetValidSlots
  (return 0))

(fn HasItematIndex
  (params (Slot :type Integer))
  (return false))

(fn IsSlotIdValid
  (params (Slot :type Integer))
  (return false))

(fn RemoveItem
  (params (AtIndex :type Integer) (Silent :type Boolean))
  (return false "" 0))
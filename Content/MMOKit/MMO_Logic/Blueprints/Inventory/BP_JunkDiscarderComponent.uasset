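; Player controller component that acts as an inventory sink for discarded items, accepting any item and storing none.
; PutItem spawns a pickable item in front of the pawn, line-traced down to the ground without physics.
; OnItemDropped keeps the last five drops and destroys the oldest beyond that, as basic spam protection.
; Alternative physics drop, loot bag and destroy-only options are present but unwired.
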(event Custom|OnItemDropped
  (params (ItemDropped :type Actor%20Object%20Reference))
  (bind _lastdroppeditems (Variables|Default|GetLastDroppedItems))
  (bind _lastdroppeditems_2 (Variables|Default|GetLastDroppedItems))
  (bind _output (Utilities|Array|Get(acopy) _lastdroppeditems))
  ;[0.4452 0.6332 1] Prevent spam of dropped items
  ; Keeps the last 5 dropped items in memory and if a user drops 6th item, the 1st item gets destroyed
  ; If a player relogs, he can spawn 5 more, so it's not a waterproof protection, just an example. It's up to you to think of a system that suits you.
  (Utilities|IsValid ItemDropped
    (:Is%20Valid
      (Utilities|FlowControl|Sequence
        (:then_0
          (bind (_arrayindex _arrayelement) (Utilities|Array|ReverseforEachLoop (Variables|Default|GetLastDroppedItems))
            (:LoopBody
              (Utilities|IsValid _arrayelement
                (:Is%20Not%20Valid
                  (Utilities|Array|RemoveIndex (Variables|Default|GetLastDroppedItems) _arrayindex))))))
        (:then_1
          (Utilities|Array|Add _lastdroppeditems_2 ItemDropped)
          (if (> (Utilities|Array|Length _lastdroppeditems_2) 5)
            (Utilities|FlowControl|Sequence
              (:then_0
                (Utilities|IsValid _output
                  (:Is%20Valid
                    (Actor|DestroyActor _output))))
              (:then_1
                (Utilities|Array|RemoveIndex _lastdroppeditems)))))))))

(event EventPutItem
  (params (Slot :type Integer) (Item :type Primary%20Asset%20Id%20Structure) (Amount :type Integer))
  ;[0.4452 0.6332 1] The function that drops items from inventory (server)
  ;;[0.4452 0.6332 1] Option 3: drop item as a mesh, no physics
  (bind _dropped (CallFunction|DropPickableItem Item Amount))
  (CallFunction|OnItemDropped _dropped))

(fn SpawnPickableIteminAir
  (params (Item :type Primary%20Asset%20Id%20Structure) (Amount :type Integer))
  ;[0.4452 0.6332 1] Drops pickable item (server)
  (bind _ascontroller (Utilities|Casting|CastToController (Components|GetOwner))
    (:then
      (bind _returnvalue (Game|SpawnActorfromClass "/Game/MMOKit/MMO_Logic/Blueprints/Interaction/BP_PickableItem.BP_PickableItem_C" (Math|Transform|MakeTransform (+ (* (Transformation|GetActorForwardVector (Pawn|GetControlledPawn _ascontroller)) 1.5e+02) (Transformation|GetActorLocation (Pawn|GetControlledPawn _ascontroller)) "0.000000,0.000000,75.000000") (Math|Random|RandomRotator true)) "Undefined" "MultiplyWithRoot" 0 Item Amount true 0))
      (return _returnvalue))
    (:CastFailed
      (return 0))))

(fn DropPickableItem
  (params (Item :type Primary%20Asset%20Id%20Structure) (Amount :type Integer))
  ;[0.4452 0.6332 1] Drops pickable item (server)
  (bind _ascontroller (Utilities|Casting|CastToController (Components|GetOwner))
    (:then
      (LocalVariables|SetSpawnLocation (+ (* (Transformation|GetActorForwardVector (Pawn|GetControlledPawn _ascontroller)) 1.5e+02) (Transformation|GetActorLocation (Pawn|GetControlledPawn _ascontroller)) "0.000000,0.000000,75.000000")) ; first tentative location is in front of a character, in the air
      (Utilities|FlowControl|Sequence
        (:then_0
          (bind _outhit (Collision|LineTraceForObjects (LocalVariables|GetSpawnLocation) (- (LocalVariables|GetSpawnLocation) "0.000000,0.000000,5000.000000") (Utilities|Array|MakeArray "ObjectTypeQuery1" "ObjectTypeQuery2") false 0 "None"))
          (if (.bBlockingHit (Collision|BreakHitResult _outhit))
            (LocalVariables|SetSpawnLocation (.Location (Collision|BreakHitResult _outhit)))))
        (:then_1
          (bind _returnvalue (Game|SpawnActorfromClass "/Game/MMOKit/MMO_Logic/Blueprints/Interaction/BP_PickableItem.BP_PickableItem_C" (Math|Transform|MakeTransform (LocalVariables|GetSpawnLocation) (Math|Rotator|MakeRotator (Math|Float|SelectFloat 9e+01 0.0 (== (.PrimaryAssetType (Utilities|Struct|BreakPrimaryAssetId Item)) "Equipment")) 0.0 (Math|Random|RandomFloatinRange 0.0 3.6e+02))) "Undefined" "MultiplyWithRoot" 0 Item Amount false 0))
          (return _returnvalue))))
    (:CastFailed
      (return 0))))

(fn DropLootableBag
  (params (Item :type Primary%20Asset%20Id%20Structure) (Amount :type Integer))
  ;[0.4452 0.6332 1] Drops pickable item (server)
  (bind _ascontroller (Utilities|Casting|CastToController (Components|GetOwner))
    (:then
      (LocalVariables|SetSpawnLocation (+ (* (Transformation|GetActorForwardVector (Pawn|GetControlledPawn _ascontroller)) 1.5e+02) (Transformation|GetActorLocation (Pawn|GetControlledPawn _ascontroller)))) ; first tentative location is in front of a character, in the air
      (Utilities|FlowControl|Sequence
        (:then_0
          (bind _outhit (Collision|LineTraceForObjects (LocalVariables|GetSpawnLocation) (- (LocalVariables|GetSpawnLocation) "0.000000,0.000000,5000.000000") (Utilities|Array|MakeArray "ObjectTypeQuery1" "ObjectTypeQuery2") false 0 "None"))
          (if (.bBlockingHit (Collision|BreakHitResult _outhit))
            (LocalVariables|SetSpawnLocation (.Location (Collision|BreakHitResult _outhit)))))
        (:then_1
          (bind _returnvalue (Game|SpawnActorfromClass "/Game/MMOKit/MMO_Logic/Blueprints/Interaction/BP_LootBag.BP_LootBag_C" (Math|Transform|MakeTransform (LocalVariables|GetSpawnLocation)) "Undefined" "MultiplyWithRoot" 0 (Utilities|Array|MakeArray Item) (Utilities|Array|MakeArray Amount) 0))
          (return _returnvalue))))
    (:CastFailed
      (return 0))))

(fn AcceptsItem
  (params (Item :type Primary%20Asset%20Id%20Structure) (Slot :type Integer))
  (return true))

(fn FindItem
  (params (ItemId :type Primary%20Asset%20Id%20Structure))
  (return false 0 0))

(fn GetFirstAvailableSlot
  (return 0 true))

(fn GetItem
  (params (Slot :type Integer))
  (return "" 0))

(fn GetValidSlots
  (return (Utilities|Array|MakeArray 0)))

(fn HasItematIndex
  (params (Slot :type Integer))
  (return false))

(fn IsSlotIdValid
  (params (Slot :type Integer))
  (return true))

(fn RemoveItem
  (params (AtIndex :type Integer) (Silent :type Boolean))
  (return false "" 0))
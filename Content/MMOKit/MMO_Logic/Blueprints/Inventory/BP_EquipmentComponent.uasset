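; Player equipment component storing item asset IDs and amounts for Head, Right Hand and Left Hand slots, with slot-type checks.
; Inventory-interface edits are meant for the server, which pushes changes to the client and notifies appearance and right-hand weapon listeners.
; SendToClient copies the arrays and broadcasts a content-updated payload.
; Initialize loads database equipment, resizing it to three slots and blanking missing assets, while GetSerializedEquipment packs it back into a struct.
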(event Custom|SendToClient
  (params (Equipment :type Array%20of%20Primary%20Asset%20Id%20Structures) (Amounts :type Array%20of%20Integers))
  ;[1 1 1] Replicate equipment to client
  (Variables|Default|SetEquipment Equipment)
  (Variables|Default|SetAmounts Amounts)
  (CallFunction|EmitContentUpdated))

(event Custom|OnEquipmentChanged
  ;[1 1 1] Replicate equipment to client
  (CallFunction|SendtoClient (Variables|Default|GetEquipment) (Variables|Default|GetAmounts))
  (Default|CallOnAppearanceUpdated (Variables|Default|GetEquipment)) ; Bp_AppearanceComponent watches this event
  (Default|CallOnRhandUpdated (Utilities|Array|Get(acopy) (Variables|Default|GetAmounts) 1) (Utilities|Array|Get(acopy) (Variables|Default|GetEquipment) 1)) ; RHand slot will update our Autoattack/LMB ability based on weapon
)

(event Custom|Initialize
  (params (InEquipment :type F%20Equipment%20Structure))
  ;[0.4452 0.6332 1] Initialize is called from BP_PlayerController::SpawnCharacter which happens when we receive the character from DB
  (bind _equipmentout (CallFunction|AdjustSlotstoDesired InEquipment 3))
  (bind _output_get (Variables|Default|SetMaxSlots (.MaxSlots (Utilities|Struct|BreakFEquipment _equipmentout))))
  (Variables|Default|SetAmounts (.Amounts (Utilities|Struct|BreakFEquipment _equipmentout)))
  (for _index (range 0 (- _output_get 1))
    (Utilities|Array|Add (Variables|Default|GetEquipment) (select (CallFunction|DoesPrimaryAssetExist (Utilities|Array|Get(acopy) (.Equipment (Utilities|Struct|BreakFEquipment _equipmentout)) _index)) (Utilities|Array|Get(acopy) (.Equipment (Utilities|Struct|BreakFEquipment _equipmentout)) _index) (Utilities|Struct|MakePrimaryAssetId))))
  (CallFunction|OnEquipmentChanged))

(event EventEmitContentUpdated
  ;[1 1 1] Emit content updated
  (bind _returnvalue (Game|ConstructObjectfromClass "/Game/MMOKit/MMO_Logic/Blueprints/Inventory/BP_Equipment_UpdateData.BP_Equipment_UpdateData_C" (Variables|Default|GetAmounts) (Variables|Default|GetEquipment)))
  (Default|CallOnContentUpdated _returnvalue))

(event EventPutItem
  (params (Slot :type Integer) (Item :type Primary%20Asset%20Id%20Structure) (Amount :type Integer))
  ;[1 1 1] Interface implementations
  (Networking|CanExecuteCosmeticEvents
    (:True
      (Class|MmoUtilities|LogString "You're trying to PUT ITEM on the Client's Equipment. Only do it on the server!" "Verbosity_Normal" true true "(R=1.000000,G=0.000000,B=0.024480,A=1.000000)" 5.0))
    (:False
      (CallFunction|PutItemonServer Slot Item Amount true))))

(event EventChangeAmount
  (params (AtIndex :type Integer) (NewAmount :type Integer))
  ;[1 1 1] Interface implementations
  (Networking|CanExecuteCosmeticEvents
    (:True
      (Class|MmoUtilities|LogString "You're trying to CHANGE AMOUNT on the Client's Equipment. Only do it on the server!" "Verbosity_Normal" true true "(R=1.000000,G=0.000000,B=0.024480,A=1.000000)" 5.0))
    (:False
      (CallFunction|ChangeAmountonServer AtIndex NewAmount true))))

(event EventAddItem
  (params (Item :type Primary%20Asset%20Id%20Structure) (Amount :type Integer))
  ;[1 1 1] Interface implementations
  (Class|MmoUtilities|LogString "Add Item is NOT a valid function for Equipment!" "Verbosity_Normal" true true "(R=1.000000,G=0.000000,B=0.024480,A=1.000000)" 5.0))

(fn IsSlotIdValid
  (params (Slot :type Integer))
  ;[1 1 1] For slot ID to be valid, it must be above or equal to 0, and less than MaxSlots
  (return (and (>= Slot 0) (< Slot (Variables|Default|GetMaxSlots)))))

(fn AcceptsItem
  (params (Item :type Primary%20Asset%20Id%20Structure) (Slot :type Integer))
  (bind _returnvalue (Class|KismetSystemLibrary|GetObjectfromPrimaryAssetId Item))
  (Utilities|IsValid _returnvalue
    (:Is%20Valid
      (bind _asequipment_asset (Utilities|Casting|CastToEquipmentAsset _returnvalue)
        (:then
          (bind _fits (CallFunction|DoesEquipslotFit (Variables|/Game/MMOKit/MMO_Logic/Blueprints/DataAssetTypes/EquipmentAsset.EquipmentAsset_C|GetEquip%20Slot _asequipment_asset) Slot))
          (return _fits))
        (:CastFailed
          _)))
    (:Is%20Not%20Valid
      _))
  (Class|MmoUtilities|LogString "EquipmentComponent: Accepts Item: problem" "Verbosity_Normal" true true "(R=1.000000,G=0.000000,B=0.024480,A=1.000000)")
  (return false))

(fn DoesEquipslotFit
  (params (EquipType :type EEquipSlot%20Enum :default "NewEnumerator0") (DesiredSlot :type Integer))
  ;[0.4452 0.6332 1] EquipType is a type of equipment.
  ; Desired slot is where the player is trying to put the item.
  ; 0 = Head
  ; 1 = RightHand
  ; 2 = LeftHand
  ;
  ; If you have two ring slots next, you could allow Desired Slot == 3 or Desired Slot == 4 for equip type Ring
  (bind _valid (CallFunction|IsSlotIdValid DesiredSlot))
  (if _valid
    (switch Utilities|FlowControl|Switch|SwitchonEEquipSlot EquipType
      (:NewEnumerator1
        (return (== DesiredSlot 0)))
      (:NewEnumerator0
        (return (== DesiredSlot 1)))
      (:NewEnumerator2
        (return (== DesiredSlot 2))))
    (else
      (return false))))

(fn PutItemonServer
  (params (SlotId :type Integer) (Item :type Primary%20Asset%20Id%20Structure) (Amount :type Integer) (SendToClient :type Boolean))
  (Utilities|FlowControl|Sequence
    (:then_0
      (bind _valid (CallFunction|IsSlotIdValid SlotId))
      (if _valid
        (|SetBy-RefVar (Utilities|Array|Get(acopy) (Variables|Default|GetEquipment) SlotId) Item)
        (|SetBy-RefVar (Utilities|Array|Get(acopy) (Variables|Default|GetAmounts) SlotId) Amount)
        (else
          (Class|MmoUtilities|LogString "Item's slot exceeds max equipment slot" "Verbosity_Normal" true true "(R=1.000000,G=0.000000,B=0.012190,A=1.000000)" 3.0))))
    (:then_1
      (if SendToClient
        (CallFunction|OnEquipmentChanged)))))

(fn GetItem
  (params (Slot :type Integer))
  (if (and (Utilities|Array|IsValidIndex (Variables|Default|GetAmounts) Slot) (Utilities|Array|IsValidIndex (Variables|Default|GetEquipment) Slot))
    (return (Utilities|Array|Get(acopy) (Variables|Default|GetEquipment) Slot) (Utilities|Array|Get(acopy) (Variables|Default|GetAmounts) Slot))
    (else
      (return (Utilities|Struct|MakePrimaryAssetId) 0))))

(fn HasItematIndex
  (params (Slot :type Integer))
  (if (and (Utilities|Array|IsValidIndex (Variables|Default|GetAmounts) Slot) (Utilities|Array|IsValidIndex (Variables|Default|GetEquipment) Slot))
    (return (> (Utilities|Array|Get(acopy) (Variables|Default|GetAmounts) Slot) 0))
    (else
      (return false))))

(fn ChangeAmountonServer
  (params (AtIndex :type Integer) (NewAmount :type Integer) (SendToClient :type Boolean))
  (Utilities|FlowControl|Sequence
    (:then_0
      (bind _valid (CallFunction|IsSlotIdValid AtIndex))
      (if _valid
        (bind _contains (CallFunction|HasItematIndex AtIndex))
        (if _contains
          (|SetBy-RefVar (Utilities|Array|Get(acopy) (Variables|Default|GetAmounts) AtIndex) NewAmount)
          (if (<= NewAmount 0)
            (|SetBy-RefVar (Utilities|Array|Get(acopy) (Variables|Default|GetEquipment) AtIndex) (Utilities|Struct|MakePrimaryAssetId)))
          (else
            (Class|MmoUtilities|LogString "Equipment: Change Amount failed (contains item was false)." "Verbosity_Normal" true true "(R=1.000000,G=0.000000,B=0.024480,A=1.000000)" 5.0)))
        (else
          (Class|MmoUtilities|LogString "Equipment: Change Amount failed (slot invalid)" "Verbosity_Normal" true true "(R=1.000000,G=0.000000,B=0.024480,A=1.000000)" 5.0))))
    (:then_1
      (if SendToClient
        (CallFunction|OnEquipmentChanged)))))

(fn RemoveItem
  (params (AtIndex :type Integer) (Silent :type Boolean))
  (Networking|CanExecuteCosmeticEvents
    (:True
      (Class|MmoUtilities|LogString "Equipment: You're trying to REMOVE ITEM client-side! You must do it server-side!" "Verbosity_Normal" true true "(R=1.000000,G=0.000000,B=0.024480,A=1.000000)" 5.0))
    (:False
      (bind (_item _amount) (CallFunction|GetItem AtIndex))
      (if (> _amount 0)
        (LocalVariables|SetReturnItem _item)
        (LocalVariables|SetReturnAmount _amount)
        (CallFunction|ChangeAmountonServer AtIndex 0 (not Silent))
        (return true (LocalVariables|GetReturnItem) (LocalVariables|GetReturnAmount))
        (else
          (return false (Utilities|Struct|MakePrimaryAssetId) 0))))))

(fn GetValidSlots
  (for _array_element (Variables|Default|GetAmounts)
    (if (>= _array_element 1)
      (Utilities|Array|Add (LocalVariables|GetIdsToReturn) _array_element)))
  (return (LocalVariables|GetIdsToReturn)))

(fn FindItem
  (params (ItemId :type Primary%20Asset%20Id%20Structure))
  (for (_array_element _array_index) (Variables|Default|GetEquipment)
    (if (== ItemId _array_element)
      (Utilities|Array|Add (LocalVariables|GetFoundAtIndices) _array_index)
      (Utilities|Array|Add (LocalVariables|GetFoundAmounts) (Utilities|Array|Get(acopy) (Variables|Default|GetAmounts) _array_index))))
  (return (Utilities|Array|IsNotEmpty (LocalVariables|GetFoundAtIndices)) (LocalVariables|GetFoundAtIndices) (LocalVariables|GetFoundAmounts)))

(fn AdjustSlotstoDesired
  (params (Equipment :type F%20Equipment%20Structure) (ShouldHaveSlots :type Integer))
  ;[0.4452 0.6332 1] This function adjusts the number of equipment slots and amount based on desired amount
  ; So let's say we're increasing the number of slots from 3 to 5
  ; This function will take the existing slots ['', 'sword', ''] and amounts [0,1,0] and turn them into ['', 'sword', '', '', ''] and [0,1,0,0,0]
  ; Or do the opposite and trim the excess slots
  (Utilities|FlowControl|Sequence
    (:then_0
      (bind _output_get (LocalVariables|SetOutEquipmentArray (.Equipment (Utilities|Struct|BreakFEquipment Equipment))))
      (if (!= (- ShouldHaveSlots (Utilities|Array|Length _output_get)) 0)
        (Utilities|Array|Resize (LocalVariables|GetOutEquipmentArray) ShouldHaveSlots)))
    (:then_1
      (bind _output_get_2 (LocalVariables|SetOutAmountArray (.Amounts (Utilities|Struct|BreakFEquipment Equipment))))
      (if (!= (- ShouldHaveSlots (Utilities|Array|Length _output_get_2)) 0)
        (Utilities|Array|Resize (LocalVariables|GetOutAmountArray) ShouldHaveSlots)))
    (:then_2
      (return (Utilities|Struct|MakeFEquipment ShouldHaveSlots (LocalVariables|GetOutEquipmentArray) (LocalVariables|GetOutAmountArray))))))

(fn DoesPrimaryAssetExist
  (params (Asset :type Primary%20Asset%20Id%20Structure))
  (if (AssetManager|IsValidPrimaryAssetId Asset)
    (bind _returnvalue (Class|KismetSystemLibrary|GetCurrentBundleState Asset false)) ; weird way to check for validity of primary data asset\nbut the "is valid primary asset id" doesn't check for the asset's existence
    (return _returnvalue)
    (else
      (return false))))

(fn GetSerializedEquipment
  (return (Utilities|Struct|MakeFEquipment (Variables|Default|GetMaxSlots) (Variables|Default|GetEquipment) (Variables|Default|GetAmounts))))
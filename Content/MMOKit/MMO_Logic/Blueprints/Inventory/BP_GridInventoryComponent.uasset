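; Grid inventory component that stores a player's items as sparse parallel arrays of slot index, primary asset ID and amount.
; Initialize loads saved data from the player controller's spawn flow and purges invalid entries, using bundle state to detect deleted assets.
; Add, put, remove and amount changes are meant for the server, which can resend the whole inventory to the client.
; Receiving it broadcasts OnContentUpdated with an update data object.
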(event Custom|SendInventory
  (params (NewMaxSlots :type Integer) (NewIndices :type Array%20of%20Integers) (NewItems :type Array%20of%20Primary%20Asset%20Id%20Structures) (NewAmounts :type Array%20of%20Integers))
  ;[1 1 1] Send the entire inventory from server to client
  (Variables|Default|SetMaxSlots NewMaxSlots)
  (Variables|Default|SetInventoryIndices NewIndices)
  (Variables|Default|SetInventoryItems NewItems)
  (Variables|Default|SetInventoryAmounts NewAmounts)
  (CallFunction|EmitContentUpdated))

(event Custom|DropItem
  (params (Index :type Integer))
  ;[1 1 1] Drop Item Request from client to server
  (CallFunction|RemoveItemonServer Index true))

(event Custom|ReplicateInventory
  ;[1 1 1] Send the entire inventory from server to client
  (CallFunction|SendInventory (Variables|Default|GetMaxSlots) (Variables|Default|GetInventoryIndices) (Variables|Default|GetInventoryItems) (Variables|Default|GetInventoryAmounts)))

(event EventChangeAmount
  (params (AtIndex :type Integer) (NewAmount :type Integer))
  ;[1 1 1] Interface implementations.
  ; Since only the server authority can add items
  ; or change their amount in the inventory, call these functions only server-side
  (Networking|CanExecuteCosmeticEvents
    (:True
      (Class|MmoUtilities|LogString "You're trying to change item amount from the client-side, you must do it SERVER-SIDE!" "Verbosity_Normal" true true "(R=1.000000,G=0.000000,B=0.024480,A=1.000000)"))
    (:False
      (CallFunction|ChangeAmountonServer AtIndex NewAmount true))))

(event EventInitialize
  (params (InInventory :type F%20Grid%20Inventory%20Structure))
  (bind (_maxslots _inventoryindices _inventoryitems _inventoryamounts) (Utilities|Struct|BreakFGridInventory InInventory))
  ;[1 1 1] Initialize (called from BP_PlayerController's SpawnCharacter function)
  (Variables|Default|SetMaxSlots _maxslots)
  (Variables|Default|SetInventoryIndices _inventoryindices)
  (Variables|Default|SetInventoryAmounts _inventoryamounts)
  (Variables|Default|SetInventoryItems _inventoryitems)
  (CallFunction|PurgeInvalidItems)
  (CallFunction|ReplicateInventory))

(event EventBeginPlay
  ;[1 1 1] BeginPlay
  (Networking|CanExecuteCosmeticEvents))

(event EventPutItem
  (params (Slot :type Integer) (Item :type Primary%20Asset%20Id%20Structure) (Amount :type Integer))
  ;[1 1 1] Interface implementations.
  ; Since only the server authority can add items
  ; or change their amount in the inventory, call these functions only server-side
  (Networking|CanExecuteCosmeticEvents
    (:True
      (Class|MmoUtilities|LogString "You're trying to PUT item into the inventory client-side, you must do it SERVER-SIDE!" "Verbosity_Normal" true true "(R=1.000000,G=0.000000,B=0.024480,A=1.000000)"))
    (:False
      (CallFunction|PutItemonServer Slot Item Amount true))))

(event EventEmitContentUpdated
  (bind _returnvalue (Game|ConstructObjectfromClass "/Game/MMOKit/MMO_Logic/Blueprints/Inventory/BP_GridInventory_UpdateData.BP_GridInventory_UpdateData_C" (Variables|Default|GetInventoryIndices) (Variables|Default|GetInventoryAmounts) (Variables|Default|GetInventoryItems)))
  (Default|CallOnContentUpdated _returnvalue))

(event EventAddItem
  (params (Item :type Primary%20Asset%20Id%20Structure) (Amount :type Integer))
  ;[1 1 1] Interface implementations.
  ; Since only the server authority can add items
  ; or change their amount in the inventory, call these functions only server-side
  (Networking|CanExecuteCosmeticEvents
    (:True
      (Class|MmoUtilities|LogString "You're trying to add item from the client-side, you must do it SERVER-SIDE!" "Verbosity_Normal" true true "(R=1.000000,G=0.000000,B=0.024480,A=1.000000)"))
    (:False
      (CallFunction|AddItemonServer Item Amount true))))

(fn AddItemonServer
  (params (Item :type Primary%20Asset%20Id%20Structure) (Amount :type Integer) (SendToClient :type Boolean))
  (Utilities|FlowControl|Sequence
    (:then_0
      (bind (_slot _hasavailable) (CallFunction|GetFirstAvailableSlot))
      (if _hasavailable
        (Utilities|Array|Add (Variables|Default|GetInventoryIndices) _slot)
        (Utilities|Array|Add (Variables|Default|GetInventoryItems) Item)
        (Utilities|Array|Add (Variables|Default|GetInventoryAmounts) Amount)
        (else
          (Class|MmoUtilities|LogString "Can't add item: no free slots" "Verbosity_Normal"))))
    (:then_1
      (if SendToClient
        (CallFunction|ReplicateInventory)))))

(fn RemoveItemonServer
  (params (Index :type Integer) (SendToClient :type Boolean))
  (LocalVariables|SetIndexToRemove -1)
  (Utilities|FlowControl|Sequence
    (:then_0
      (bind (_array_element _array_index) (Utilities|Array|ForEachLoopwithBreak (Variables|Default|GetInventoryIndices))
        (:LoopBody
          (if (== _array_element Index)
            (bind _output_get (LocalVariables|SetIndexToRemove _array_index))
            (LocalVariables|SetItemRemoved (Utilities|Array|Get(acopy) (Variables|Default|GetInventoryItems) _output_get))
            (LocalVariables|SetAmountRemoved (Utilities|Array|Get(acopy) (Variables|Default|GetInventoryAmounts) _output_get))))))
    (:then_1
      (if (>= (LocalVariables|GetIndexToRemove) 0)
        (Utilities|Array|RemoveIndex (Variables|Default|GetInventoryIndices) (LocalVariables|GetIndexToRemove))
        (Utilities|Array|RemoveIndex (Variables|Default|GetInventoryItems) (LocalVariables|GetIndexToRemove))
        (Utilities|Array|RemoveIndex (Variables|Default|GetInventoryAmounts) (LocalVariables|GetIndexToRemove))))
    (:then_2
      (if (and SendToClient (>= (LocalVariables|GetIndexToRemove) 0))
        (CallFunction|ReplicateInventory)
        (return true (LocalVariables|GetItemRemoved) (LocalVariables|GetAmountRemoved))
        (else
          (return false "" 0))))))

(fn PutItemonServer
  (params (Slot :type Integer) (Item :type Primary%20Asset%20Id%20Structure) (Amount :type Integer) (SendToClient :type Boolean))
  (Utilities|FlowControl|Sequence
    (:then_0
      (Utilities|Array|Add (Variables|Default|GetInventoryIndices) Slot)
      (Utilities|Array|Add (Variables|Default|GetInventoryItems) Item)
      (Utilities|Array|Add (Variables|Default|GetInventoryAmounts) Amount))
    (:then_1
      (if SendToClient
        (CallFunction|ReplicateInventory)))))

(fn ChangeAmountonServer
  (params (Index :type Integer) (NewAmount :type Integer) (SendToClient :type Boolean))
  (Utilities|FlowControl|Sequence
    (:then_0
      (bind (_array_element _array_index) (Utilities|Array|ForEachLoopwithBreak (Variables|Default|GetInventoryIndices) :!label _label)
        (:LoopBody
          (if (== _array_element Index)
            (Utilities|Array|SetArrayElem (Variables|Default|GetInventoryAmounts) _array_index NewAmount)
            (goto _label Break)))))
    (:then_1
      (if SendToClient
        (CallFunction|ReplicateInventory)))))

(fn AcceptsItem
  (params (Item :type Primary%20Asset%20Id%20Structure) (Slot :type Integer))
  ;[1 1 1] only equipment can refuse to accept an item into a slot
  (return true))

(fn GetItem
  (params (Slot :type Integer))
  (for (_array_element _array_index) (Variables|Default|GetInventoryIndices)
    (if (== _array_element Slot)
      (return (Utilities|Array|Get(acopy) (Variables|Default|GetInventoryItems) _array_index) (Utilities|Array|Get(acopy) (Variables|Default|GetInventoryAmounts) _array_index))))
  (return "" 0))

(fn HasItematIndex
  (params (Slot :type Integer))
  (bind _amount (CallFunction|GetItem Slot))
  (return (> _amount 0)))

(fn IsSlotIdValid
  (params (Slot :type Integer))
  (return (and (>= Slot 0) (< Slot (Variables|Default|GetMaxSlots)))))

(fn RemoveItem
  (params (AtIndex :type Integer) (Silent :type Boolean))
  (Networking|CanExecuteCosmeticEvents
    (:True
      (Class|MmoUtilities|LogString "You're trying to remove item from the client-side, you must do it SERVER-SIDE!" "Verbosity_Normal" true true "(R=1.000000,G=0.000000,B=0.024480,A=1.000000)" 5.0)
      (return false "" 0))
    (:False
      (bind (_success _item _amount) (CallFunction|RemoveItemonServer AtIndex (not Silent)))
      (return _success _item _amount))))

(fn GetFirstAvailableSlot
  ;[1 1 1] Iterates through the inventory and finds the first available slot, if there is one
  (Utilities|Set|AddItems (LocalVariables|GetIndicesSet) (Variables|Default|GetInventoryIndices))
  (for _index (range 0 (- (Variables|Default|GetMaxSlots) 1))
    (if (not (Utilities|Set|Contains (LocalVariables|GetIndicesSet) _index))
      (return _index true)))
  (return -1 false))

(fn GetValidSlots
  (return (Variables|Default|GetInventoryIndices)))

(fn FindItem
  (params (ItemId :type Primary%20Asset%20Id%20Structure))
  (for (_array_element _array_index) (Variables|Default|GetInventoryItems)
    (if (== ItemId _array_element)
      (Utilities|Array|Add (LocalVariables|GetFoundAtIndices) (Utilities|Array|Get(acopy) (Variables|Default|GetInventoryIndices) _array_index))
      (Utilities|Array|Add (LocalVariables|GetFoundAmounts) (Utilities|Array|Get(acopy) (Variables|Default|GetInventoryAmounts) _array_index))))
  (return (Utilities|Array|IsNotEmpty (LocalVariables|GetFoundAtIndices)) (LocalVariables|GetFoundAtIndices) (LocalVariables|GetFoundAmounts)))

(fn PurgeInvalidItems
  ;[0.4452 0.6332 1] If we created some items, gave them to player, but then deleted them, we don't need a corrupt inventory.
  (for (_array_element _array_index) (Variables|Default|GetInventoryItems)
    (LocalVariables|SetTestingAssetId _array_element)
    (LocalVariables|SetTestingIndex _array_index)
    (if (AssetManager|IsValidPrimaryAssetId (LocalVariables|GetTestingAssetId))
      (bind _returnvalue (Class|KismetSystemLibrary|GetCurrentBundleState (LocalVariables|GetTestingAssetId) false)) ; weird way to check for validity of primary data asset\nbut the "is valid primary asset id" doesn't check for the asset's existence
      (if (or (>= (LocalVariables|GetTestingIndex) (Variables|Default|GetMaxSlots)) (not _returnvalue))
        (Utilities|Array|Add (LocalVariables|GetInvalidIndices) (LocalVariables|GetTestingIndex) :!label _label)
        (Class|MmoUtilities|LogString (Utilities|String|Append "Purging invalid item from inventory: " (Utilities|String|ToString(Integer) (LocalVariables|GetTestingAssetId))) "Verbosity_Normal" true true "(R=1.000000,G=0.000000,B=0.719426,A=1.000000)" 5.0))
      (else
        (goto _label))))
  (Class|KismetArrayLibrary|SortIntArray (LocalVariables|GetInvalidIndices))
  (bind _arrayelement (Utilities|Array|ReverseforEachLoop (LocalVariables|GetInvalidIndices))
    (:LoopBody
      (Utilities|Array|RemoveIndex (Variables|Default|GetInventoryItems) _arrayelement)
      (Utilities|Array|RemoveIndex (Variables|Default|GetInventoryIndices) _arrayelement)
      (Utilities|Array|RemoveIndex (Variables|Default|GetInventoryAmounts) _arrayelement))))

(fn GetSerializedInventory
  (return (Utilities|Struct|MakeFGridInventory (Variables|Default|GetMaxSlots) (Variables|Default|GetInventoryIndices) (Variables|Default|GetInventoryItems) (Variables|Default|GetInventoryAmounts))))
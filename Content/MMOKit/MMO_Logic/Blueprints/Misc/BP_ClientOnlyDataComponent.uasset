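; Client-side component that tracks player characters currently in the local player's vicinity, keyed by character ID.
; On BeginPlay it retries each tick until player controller 0's event bus is valid, then binds to its vicinity enter and leave events.
; Those events add or remove entries in the SeenPlayers map, which GetSeenPlayerById exposes for lookup.
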(event Custom|OnNoSeePlayer
  (params (PlayerChar :type Character%20Object%20Reference))
  (bind _id (Class|BPICharacter|GetCharId(Message) PlayerChar))
  (Utilities|Map|Remove (Variables|Default|GetSeenPlayers) _id))

(event Custom|OnSeePlayer
  (params (PlayerChar :type Character%20Object%20Reference))
  (bind _id (Class|BPICharacter|GetCharId(Message) PlayerChar))
  (Utilities|Map|Add (Variables|Default|GetSeenPlayers) _id PlayerChar))

(event EventBeginPlay
  (bind _eventbus (Class|BPIPlayerController|GetPlayerControllerEventBus(Message) (Game|GetPlayerController 0) :!label _label))
  (Utilities|IsValid _eventbus
    (:Is%20Valid
      (EventDispatchers|AssignOnPlayerEnteredVicinity _eventbus (delegate Custom|OnSeePlayer))
      (EventDispatchers|BindEventtoOnPlayerLeftVicinity _eventbus (delegate Custom|OnNoSeePlayer)))
    (:Is%20Not%20Valid
      (Utilities|FlowControl|DelayUntilNextTick)
      (goto _label))))

(fn GetSeenPlayerbyId
  (params (Id :type Integer))
  (return (.Value (Utilities|Map|Find (Variables|Default|GetSeenPlayers) Id))))
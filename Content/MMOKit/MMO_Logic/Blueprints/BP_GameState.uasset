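; BP_GameState is the MMOKit game state that holds the connection to the persistence server and the HTTP manager.
; On BeginPlay it spawns a BP_WebSockets actor and tells it to connect to the persistence server, then spawns a BP_HttpManager, with no authority check.
; Getters expose both actors, and a getter and setter pair stores the server GUID for other code.
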(event EventBeginPlay
  ;[0.7865 0.1065 0.7201] BeginPlay: connect to Persistence Server
  (Utilities|FlowControl|Sequence
    (:then_0
      (bind _returnvalue (Game|SpawnActorfromClass "/Game/MMOKit/MMO_Logic/Blueprints/WebSockets/BP_WebSockets.BP_WebSockets_C" (Math|Transform|MakeTransform "0, 0, 0" "0, 0, 0" "1.000000,1.000000,1.000000") "Undefined" "OverrideRootScale" 0 0))
      (Variables|Default|SetTcpConnectionServer _returnvalue)
      (Default|ConnecttoPersistenceServer (Variables|Default|GetTcpConnectionServer)))
    (:then_1
      ;[0.7865 0.1065 0.7201] Spawn Http Manager
      (bind _returnvalue_2 (Game|SpawnActorfromClass "/Game/MMOKit/MMO_Logic/Blueprints/WebSockets/BP_HttpManager.BP_HttpManager_C" (Math|Transform|MakeTransform "0, 0, 0" "0, 0, 0" "1.000000,1.000000,1.000000") "Undefined" "MultiplyWithRoot" 0 0))
      (Variables|Default|SetHttpManager _returnvalue_2))))

(fn ConstructionScript)

(fn GetHttpManager
  (return (Variables|Default|GetHttpManager)))

(fn GetServerGuid
  (return (Variables|Default|GetServerGuid)))

(fn GetTcpConnection
  (return (Variables|Default|GetTcpConnectionServer)))

(fn SetServerGuid
  (params (ServerGuid :type String))
  (Variables|Default|SetServerGuid ServerGuid)
  (return))